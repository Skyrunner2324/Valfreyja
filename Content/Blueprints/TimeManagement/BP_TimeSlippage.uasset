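; BP_TimeSlippage is an actor in the time management folder that acts as a debug control for global time scale.
; When its Debug flag is set, it enables input from the first player controller on BeginPlay.
; Number keys, Backspace and Enter call SetGlobalTimeScale in fixed steps from full stop to normal speed.
; The F key posts a Wwise test beep event.
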(event EventBeginPlay
  (if (Variables|Default|GetbDebug)
    (Input|EnableInput (Game|GetPlayerController 0))))

(event Input|KeyboardEvents|DebugKey1
  (params (Key :type Key%20Structure :default "None") (ActionValue :type Input%20Action%20Value%20Structure))
  (:Pressed
    (Class|TimeSlippage|SetGlobalTimeScale 0.1)))

(event Input|KeyboardEvents|DebugKey2
  (params (Key :type Key%20Structure :default "None") (ActionValue :type Input%20Action%20Value%20Structure))
  (:Pressed
    (Class|TimeSlippage|SetGlobalTimeScale 0.2)))

(event Input|KeyboardEvents|DebugKeyBackspace
  (params (Key :type Key%20Structure :default "None") (ActionValue :type Input%20Action%20Value%20Structure))
  (:Pressed
    (Class|TimeSlippage|SetGlobalTimeScale 0.0)))

(event Input|KeyboardEvents|DebugKeyF
  (params (Key :type Key%20Structure :default "None") (ActionValue :type Input%20Action%20Value%20Structure))
  (:Pressed
    (Class|AkGameplayStatics|PostEvent "/Game/WwiseAudio/Events/TestEvents/Play_TestBeep.Play_TestBeep")))

(event Input|KeyboardEvents|DebugKey3
  (params (Key :type Key%20Structure :default "None") (ActionValue :type Input%20Action%20Value%20Structure))
  (:Pressed
    (Class|TimeSlippage|SetGlobalTimeScale 0.3)))

(event Input|KeyboardEvents|DebugKey4
  (params (Key :type Key%20Structure :default "None") (ActionValue :type Input%20Action%20Value%20Structure))
  (:Pressed
    (Class|TimeSlippage|SetGlobalTimeScale 0.4)))

(event Input|KeyboardEvents|DebugKey5
  (params (Key :type Key%20Structure :default "None") (ActionValue :type Input%20Action%20Value%20Structure))
  (:Pressed
    (Class|TimeSlippage|SetGlobalTimeScale 0.5)))

(event Input|KeyboardEvents|DebugKey6
  (params (Key :type Key%20Structure :default "None") (ActionValue :type Input%20Action%20Value%20Structure))
  (:Pressed
    (Class|TimeSlippage|SetGlobalTimeScale 0.6)))

(event Input|KeyboardEvents|DebugKey7
  (params (Key :type Key%20Structure :default "None") (ActionValue :type Input%20Action%20Value%20Structure))
  (:Pressed
    (Class|TimeSlippage|SetGlobalTimeScale 0.7)))

(event Input|KeyboardEvents|DebugKey8
  (params (Key :type Key%20Structure :default "None") (ActionValue :type Input%20Action%20Value%20Structure))
  (:Pressed
    (Class|TimeSlippage|SetGlobalTimeScale 0.8)))

(event Input|KeyboardEvents|DebugKey9
  (params (Key :type Key%20Structure :default "None") (ActionValue :type Input%20Action%20Value%20Structure))
  (:Pressed
    (Class|TimeSlippage|SetGlobalTimeScale 0.9)))

(event Input|KeyboardEvents|DebugKeyEnter
  (params (Key :type Key%20Structure :default "None") (ActionValue :type Input%20Action%20Value%20Structure))
  (:Pressed
    (Class|TimeSlippage|SetGlobalTimeScale 1.0)))

(fn ConstructionScript)