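; Power-up that gradually refills the player's dilation meter when picked up.
; On power-up it plays a timeline that ignores time dilation, with play rate derived from the configured duration.
; Each update adds dilation through BP_PlayerController and stops the timeline once the meter is full.
; If the timeline finishes, the actor is destroyed when flagged to do so on pickup.
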(event `self.ReceiveBeginPlay`
  (`parent.ReceiveBeginPlay`)
  (`TimelineComponent.SetIgnoreTimeDilation` (`self.AddDilationTimeline`) true))

(event `Stop`
  (`Timeline|AddDilationTimeline` :!via `Stop`
    (:`Update`
      (`TimelineComponent.SetPlayRate` (`self.AddDilationTimeline`) (/ 1.0 (`self.AddDuration`)))
      (bind _asbp_player_controller (cast `/Game/Blueprints/Controller/BP_PlayerController` (`GameplayStatics.GetPlayerController` 0)))
      (`/Game/Blueprints/Controller/BP_PlayerController.AddDilation` _asbp_player_controller (`self.AddDilationRate`))
      (if (`/Game/Blueprints/Controller/BP_PlayerController.IsDilationFull` _asbp_player_controller)
        (`self.Stop`)))
    (:`Finished`
      (if (`self.bDestroyWhenPickedUp`)
        (`self.K2_DestroyActor`)))))

(fn `OnPowerUpImpl`
  (params (player :type "/Game/Blueprints/Characters/BP_PlayerCharacter Object Reference"))
  (`parent.OnPowerUpImpl` player)
  (`TimelineComponent.PlayFromStart` (`self.AddDilationTimeline`)))

(fn `UserConstructionScript`)