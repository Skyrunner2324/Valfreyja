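; Power-up Blueprint that turns on a weak time dilation effect through BP_PlayerController when triggered.
; On activation it calls StartWeakDilation with 1, scales WeakDilationTimeline's play rate by the inverse of the effect duration and plays it from the start.
; The timeline serves as a timer that ignores time dilation, with its Finished handler calling StartWeakDilation with 0.
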(event `self.ReceiveBeginPlay`
  (`parent.ReceiveBeginPlay`)
  (`TimelineComponent.SetIgnoreTimeDilation` (`self.WeakDilationTimeline`) true))

(fn `OnPowerUpImpl`
  (params (player :type "/Game/Blueprints/Characters/BP_PlayerCharacter Object Reference"))
  (`parent.OnPowerUpImpl` player)
  (`KismetSystemLibrary.PrintString` "dilation" false false)
  (bind _asbp_player_controller (cast `/Game/Blueprints/Controller/BP_PlayerController` (`GameplayStatics.GetPlayerController` 0)))
  (`|ExecutionSequence`
    (:`then_0`
      (`/Game/Blueprints/Controller/BP_PlayerController.StartWeakDilation` _asbp_player_controller 1.0))
    (:`then_1`
      ;[1 1 1] timeline settings
      (`TimelineComponent.SetPlayRate` (`self.WeakDilationTimeline`) (/ 1.0 (`self.WeakDilationDuration`))))
    (:`then_2`
      (`TimelineComponent.PlayFromStart` (`self.WeakDilationTimeline`)))))

(fn `UserConstructionScript`)