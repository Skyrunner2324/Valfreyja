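; BP_RegenShield is a power-up that gradually restores the player's health.
; On pickup it caches the player's health component and plays a timeline that ignores time dilation, adding health each update with play rate scaled by AddDuration.
; The timeline stops early at full health, and the actor is destroyed on Finished if DestroyWhenPickedUp is set.
; Activation always passes, as the full-health check is disconnected.
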(event `self.ReceiveBeginPlay`
  (`parent.ReceiveBeginPlay`)
  (`TimelineComponent.SetIgnoreTimeDilation` (`self.AddHealthTimeline`) true))

(event `Stop`
  (`Timeline|AddHealthTimeline` :!via `Stop`
    (:`Update`
      (`TimelineComponent.SetPlayRate` (`self.AddHealthTimeline`) (/ 1.0 (`self.AddDuration`)))
      (`/Game/Blueprints/Component/ActorComponent/Damage/AC_TakeDamage.AddHealth` (`self.PlayerHealthComponent`) (`self.AddHealthRate`))
      (if (`/Game/Blueprints/Component/ActorComponent/Damage/AC_TakeDamage.IsHealthFull` (`self.PlayerHealthComponent`))
        (`self.Stop`)))
    (:`Finished`
      (if (`self.bDestroyWhenPickedUp`)
        (`self.K2_DestroyActor`)))))

(fn `ActivationCondidtion`
  (returns (bShouldActivate :type Boolean))
  (return true))

(fn `OnPowerUpImpl`
  (params (player :type "/Game/Blueprints/Characters/BP_PlayerCharacter Object Reference"))
  (`parent.OnPowerUpImpl` player)
  (set `self.PlayerHealthComponent` (`/Game/Blueprints/Characters/BP_PlayerCharacter.TakeDamage` player))
  (`TimelineComponent.PlayFromStart` (`self.AddHealthTimeline`)))

(fn `UserConstructionScript`)