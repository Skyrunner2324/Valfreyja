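; CustomRails is a spline rail that builds its own mesh and supplies functions for moving another actor along it.
; The construction script tiles colliding spline meshes by SectionLength with clamped tangents and a selectable forward axis; FullLengthMesh omits the final partial section.
; At runtime it converts a world location to spline distance and picks travel direction from the actor's forward vector.
; GetNextStepOnRail advances that stored distance, returning world position and whether an end is reached.
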(fn `GetClosestPoint`
  (returns (Location :type "Vector Structure"))
  (return (`SplineComponent.GetLocationAtDistanceAlongSpline` (`self.Spline`) (`self.CurrendPositionOnSpline`) "World")))

(fn `GetEndPos/Tangent`
  (params (LoopIndex :type Integer))
  (returns (Pos :type "Vector Structure") (Tan :type "Vector Structure"))
  (bind _spline (`self.Spline`))
  (bind _returnvalue (* (+ LoopIndex 1) (`self.SectionLength`)))
  (return (`SplineComponent.GetLocationAtDistanceAlongSpline` _spline _returnvalue "Local") (`KismetMathLibrary.ClampVectorSize` (`SplineComponent.GetTangentAtDistanceAlongSpline` _spline _returnvalue "Local") 0.0 (`self.SectionLength`))))

(fn `GetMovementDirection`
  (returns (Direction :type "Vector Structure"))
  (return (* (`SplineComponent.GetDirectionAtDistanceAlongSpline` (`self.Spline`) (`self.CurrendPositionOnSpline`) "Local") (`self.DirectionMultiplier`))))

(fn `GetNextStepOnRail`
  (params (StepSize :type "Float (double-precision)"))
  (returns (EndReached :type Boolean) (WorldPosition :type "Vector Structure"))
  (bind _output_get (set `self.CurrendPositionOnSpline` (+ (* StepSize (`self.DirectionMultiplier`)) (`self.CurrendPositionOnSpline`))))
  (bind _returnvalue (`self.IsEndReached`))
  (return _returnvalue (`SplineComponent.GetLocationAtDistanceAlongSpline` (`self.Spline`) _output_get "World")))

(fn `GetProgressOnSpline`
  (params (Location :type "Vector Structure"))
  (returns (Output :type "Float (double-precision)"))
  (bind _spline (`self.Spline`))
  (bind _returnvalue (`SplineComponent.FindInputKeyClosestToWorldLocation` (`self.Spline`) Location))
  (bind _returnvalue_2 (`KismetMathLibrary.FFloor` _returnvalue))
  (bind _returnvalue_3 (+ _returnvalue_2 1))
  (bind _returnvalue_4 (`SplineComponent.GetDistanceAlongSplineAtSplinePoint` _spline _returnvalue_3))
  (bind _output_get (set `self.CurrendPositionOnSpline` (- _returnvalue_4 (* (- (`SplineComponent.GetDistanceAlongSplineAtSplinePoint` _spline _returnvalue_2) _returnvalue_4) (- _returnvalue (`KismetMathLibrary.Conv_IntToDouble` _returnvalue_3))))))
  (`self.IsEndReached`)
  (return _output_get))

(fn `GetStartPos/Tangent`
  (params (LoopIndex :type Integer))
  (returns (Pos :type "Vector Structure") (Tan :type "Vector Structure"))
  (bind _spline (`self.Spline`))
  (bind _returnvalue (* LoopIndex (`self.SectionLength`)))
  (return (`SplineComponent.GetLocationAtDistanceAlongSpline` _spline _returnvalue "Local") (`KismetMathLibrary.ClampVectorSize` (`SplineComponent.GetTangentAtDistanceAlongSpline` _spline _returnvalue "Local") 0.0 (`self.SectionLength`))))

(fn `IsEndReached`
  (returns (ReturnValue :type Boolean))
  (bind _currendpositiononspline (`self.CurrendPositionOnSpline`))
  (return (or (>= _currendpositiononspline (`SplineComponent.GetSplineLength` (`self.Spline`))) (<= _currendpositiononspline 0.0))))

(fn `SetForward`
  (params (Mesh :type "SplineMeshComponent Object Reference"))
  (switch `/Game/Blueprints/Enumerator/Forward` (`self.Forward`)
    (:`NewEnumerator0`
      (`SplineMeshComponent.SetForwardAxis` Mesh "X" true))
    (:`NewEnumerator1`
      (`SplineMeshComponent.SetForwardAxis` Mesh "Y" true))
    (:`NewEnumerator2`
      (`SplineMeshComponent.SetForwardAxis` Mesh "Z" true))))

(fn `SetMovementDirection`
  (params (WorldLocation :type "Vector Structure (by ref)") (ActorForward :type "Vector Structure"))
  (bind _output (`self.GetProgressOnSpline` WorldLocation))
  (set `self.DirectionMultiplier` (`KismetMathLibrary.SelectFloat` -1.0 1.0 (<= (`KismetMathLibrary.Dot_VectorVector` (`SplineComponent.GetDirectionAtDistanceAlongSpline` (`self.Spline`) _output "Local") ActorForward) 0.0))))

(fn `UserConstructionScript`
  (bind _loopindex (`self.LoopIndex`))
  (bind _meshscale (`self.MeshScale`))
  (bind _returnvalue (`KismetMathLibrary.FTrunc` (/ (`SplineComponent.GetSplineLength` (`self.Spline`)) (`self.SectionLength`))))
  (if (`self.FullLengthMesh`)
    (for _index (range _returnvalue)
      (set `self.LoopIndex` _index)
      (bind _returnvalue_2 (`AddComponent|NODE_AddSplineMeshComponent-0` :!label _label))
      (`StaticMeshComponent.SetStaticMesh` _returnvalue_2 (`self.SplineMesh`))
      (`self.SetForward` _returnvalue_2)
      (`SplineMeshComponent.SetStartScale` _returnvalue_2 (`KismetMathLibrary.MakeVector2D` _meshscale _meshscale) true)
      (`SplineMeshComponent.SetEndScale` _returnvalue_2 (`KismetMathLibrary.MakeVector2D` _meshscale _meshscale) true)
      (bind (_pos _tan) (`self.GetStartPos/Tangent` _loopindex))
      (bind (_pos_2 _tan_2) (`self.GetEndPos/Tangent` _loopindex))
      (`SplineMeshComponent.SetStartAndEnd` _returnvalue_2 _pos _tan _pos_2 _tan_2 true)
      (`PrimitiveComponent.SetCollisionEnabled` _returnvalue_2 "QueryAndPhysics"))
    (else
      (for _index_2 (range (+ _returnvalue 1))
        (set `self.LoopIndex` _index_2)
        (goto _label)))))