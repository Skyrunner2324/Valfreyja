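; Actor component that propels the player character toward a target location as a triggered movement ability, with a sound on launch.
; TriggerAbility zeroes velocity, sets launch speed and fixes the direction once.
; Each tick overrides velocity through LaunchCharacter rather than interpolating, reducing speed to a minimum near the target using the character's time-slippage delta.
; The ability ends within reach distance without clearing velocity, and ignores retriggers while active.
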(event `self.ReceiveBeginPlay`
  (set `self.playerCharacter` (cast `/Game/Blueprints/Characters/BP_PlayerCharacter` (`GameplayStatics.GetPlayerCharacter` 0) :!pure true))
  (set `self.playerController` (cast `/Game/Blueprints/Controller/BP_PlayerController` (`GameplayStatics.GetPlayerController` 0) :!pure true)))

(event `self.ReceiveTick`
  (params (DeltaSeconds :type "Float (single-precision)"))
  (if (`self.TriggerTickAbility`)
    (`self.SetValueTickUseAbility`)
    (if (`self.CheckStopAbility`)
      (`self.StopAbility`)
      (else
        (if (`self.CheckReduceSpeed`)
          (set `self.speed` (`KismetMathLibrary.FClamp` (- (`self.speed`) (* (`self.valueToReduceSpeed`) (`TimeSlippageModifier.localManagedDeltaTime` (`/Game/Blueprints/Characters/BP_PlayerCharacter.TimeSlippageModifier` (`self.playerCharacter`))))) (`self.minSpeed`) 10000000000.0)))
        (`Character.LaunchCharacter` (`self.playerCharacter`) (* (`self.directionToTarget`) (`self.speed`)) true true)))))

(fn `CanUseAbility`
  (returns (useAbility :type Boolean))
  (return (not (`self.useAbility`))))

(fn `CheckReduceSpeed`
  (returns (ReturnValue :type Boolean))
  (return (< (`self.distanceToTarget`) (`self.distanceToReduceSpeed`))))

(fn `CheckStopAbility`
  (returns (ReturnValue :type Boolean))
  (return (< (`self.distanceToTarget`) (`self.reachTargetDistance`))))

(fn `GetDistanceToTarget`
  (returns (distance :type "Float (double-precision)"))
  (return (`KismetMathLibrary.Vector_Distance` (`self.targetLocation`) (`Actor.K2_GetActorLocation` (`self.playerCharacter`)))))

(fn `SetDirection`
  (set `self.directionToTarget` (`KismetMathLibrary.Normal` (- (`self.targetLocation`) (`Actor.K2_GetActorLocation` (`self.playerCharacter`))))))

(fn `SetNewTargetLocation`
  (params (targetLocation :type "Vector Structure"))
  (set `self.targetLocation` targetLocation))

(fn `SetValueTickUseAbility`
  (set `self.distanceToTarget` (`self.GetDistanceToTarget`)))

(fn `SetValueTriggerAbility`
  (params (targetLocation :type "Vector Structure"))
  (bind _soundability (`self.soundAbility`))
  (set `self.useAbility` true)
  (set `self.speed` (`self.speedLaunch`))
  ;[0 1 0.2423] Sound ability
  (`AkGameplayStatics.PostEvent` _soundability)
  (`KismetSystemLibrary.PrintString` (`KismetSystemLibrary.GetDisplayName` _soundability))
  (`self.SetNewTargetLocation` (`local.targetLocation`))
  (`self.SetDirection`))

(fn `StopAbility`
  (set `self.useAbility` false)
  (return))

(fn `TriggerAbility`
  (params (targetLocation :type "Vector Structure"))
  (if (`self.CanUseAbility`)
    (set `MovementComponent.Velocity` (0.0 0.0 0.0) (`Character.CharacterMovement` (`self.playerCharacter`)))
    (`self.SetValueTriggerAbility` (`local.targetLocation`))))

(fn `TriggerTickAbility`
  (returns (useAbility :type Boolean))
  (return (`self.useAbility`)))