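; Player controller component that auto-locks onto enemies appearing inside a screen-centred aim area shown by the WB_AimArea widget.
; Each tick without a target, it projects NearEnemies to screen space, keeps those inside the detection box and locks the one nearest the controlled pawn.
; A locked enemy is released once its projected point leaves the separate lock box.
; Both bounds derive from the widget's size boxes around the viewport centre.
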(event `self.ReceiveBeginPlay`
  (bind _asplayer_controller (cast `PlayerController` (`self.GetOwner`)))
  (bind _output_get (set `self.controllerRef` _asplayer_controller))
  (set `self.controlledPawnRef` (`Controller.K2_GetPawn` _output_get))
  (bind _returnvalue (`|CreateWidget` "/Game/UI/WB_AimArea.WB_AimArea_C" null (`self.aimAreaSizePct`) (`self.aimLockAreaSizePct`)))
  (bind _output_get_2 (set `self.aimArea` _returnvalue))
  (`UserWidget.AddToViewport` _output_get_2 0))

(event `self.ReceiveTick`
  (params (DeltaSeconds :type "Float (single-precision)"))
  (`self.enemyLocked`
    (:`then`
      (`self.IsEnemyInLockArea`
        (:`False`
          (set `self.enemyLocked` null)
          (`KismetSystemLibrary.PrintString` "Cible perdue"))))
    (:`else`
      (bind _enemies (`self.GetEnemiesInAimArea`))
      (if (not (`KismetArrayLibrary.Array_IsEmpty` _enemies))
        (bind _enemy (`self.GetNearestEnemy` _enemies))
        (set `self.enemyLocked` _enemy)
        (`KismetSystemLibrary.PrintString` "EnemyLocked")))))

(fn `GetEnemiesInAimArea`
  (returns (enemies :type "Array of BaseEnemy Object Reference"))
  (locals (enemiesInArea :type "Array of BaseEnemy Object Reference"))
  (bind (_minx _miny _maxx _maxy) (`self.GetAimAreaBounds`))
  (for _array_element (`self.nearEnemies`)
    (bind _screenlocation (`PlayerController.ProjectWorldLocationToScreen` (`self.controllerRef`) (+ (`Actor.K2_GetActorLocation` _array_element) (0.0 0.0 100.0)) true))
    (if (and (> (`KismetMathLibrary.BreakVector2D` _screenlocation) _minx) (> (`.Y` (`KismetMathLibrary.BreakVector2D` _screenlocation)) _miny) (< (`KismetMathLibrary.BreakVector2D` _screenlocation) _maxx) (< (`.Y` (`KismetMathLibrary.BreakVector2D` _screenlocation)) _maxy))
      (`KismetArrayLibrary.Array_Add` (`local.enemiesInArea`) (cast `BaseEnemy` _array_element :!pure true))))
  (return (`local.enemiesInArea`)))

(fn `GetNearestEnemy`
  (params (enemies :type "Array of BaseEnemy Object Reference"))
  (returns (enemy :type "BaseEnemy Object Reference"))
  (locals (nearestEnemy :type "BaseEnemy Object Reference"))
  (bind _returnvalue (`Actor.K2_GetActorLocation` (`self.controlledPawnRef`)))
  (for _array_element enemies
    (`local.nearestEnemy`
      (:`then`
        (if (>= (`KismetMathLibrary.Vector_Distance` _returnvalue (`Actor.K2_GetActorLocation` (`local.nearestEnemy`))) (`KismetMathLibrary.Vector_Distance` _returnvalue (`Actor.K2_GetActorLocation` _array_element)))
          (set `local.nearestEnemy` _array_element)))
      (:`else`
        (set `local.nearestEnemy` _array_element))))
  (return (`local.nearestEnemy`)))