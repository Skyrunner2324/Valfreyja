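; Actor component that manages arena gunner enemies over a set of spawn points, spawning one per point on Init and respawning them after death.
; A map tracks each point's occupancy, and respawns pick a random free point other than the previous one, falling back to it.
; Deaths queue timed respawns, counted down on a tick that uses the player's time-slippage delta and runs only while the queue has entries.
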(event `EnemyDeath`
  (params (linkedSpawn :type "/Game/Blueprints/Managers/EnemyWaves/BP_EnemySpawnPoint Object Reference (by ref)"))
  (`BlueprintMapLibrary.Map_Add` (`self.spawnPoints`) linkedSpawn)
  (`KismetArrayLibrary.Array_Add` (`self.spawnQueue`) (make `/Game/Blueprints/Managers/EnemyWaves/ST_EnemyRespawn` linkedSpawn (`self.timeBeforeRespawn`)))
  (`self.SetComponentTickEnabled` true))

(event `Init`
  (`self.ResetSpawnPoints`)
  (for _ (range (`BlueprintMapLibrary.Map_Length` (`self.spawnPoints`)))
    (`self.SpawnEnemy` null)))

(event `self.ReceiveTick`
  (params (DeltaSeconds :type "Float (single-precision)"))
  (for (_array_element _array_index) (`self.spawnQueue`)
    (bind (_previousspawnpoint _remainingtime) (break `/Game/Blueprints/Managers/EnemyWaves/ST_EnemyRespawn` _array_element))
    (bind _returnvalue (- _remainingtime (`TimeSlippageModifier.deltaTime` (`/Game/Blueprints/Characters/BP_PlayerCharacter.TimeSlippageModifier` (cast `/Game/Blueprints/Characters/BP_PlayerCharacter` (`GameplayStatics.GetPlayerCharacter` 0) :!pure true)))))
    (bind _structout (setmembers `/Game/Blueprints/Managers/EnemyWaves/ST_EnemyRespawn` :`StructRef` _array_element :`remainingTime` _returnvalue))
    (`KismetArrayLibrary.Array_Set` (`self.spawnQueue`) _array_index _structout)
    (if (<= _returnvalue 0.0)
      (`self.SpawnEnemy` _previousspawnpoint)
      (`KismetArrayLibrary.Array_RemoveItem` (`self.spawnQueue`) _structout)))
  (if (`KismetArrayLibrary.Array_IsEmpty` (`self.spawnQueue`))
    (`self.SetComponentTickEnabled` false)))

(fn `Disable`
  (`self.SetComponentTickEnabled` false)
  (`KismetArrayLibrary.Array_Clear` (`self.spawnQueue`)))

(fn `GetNewAvailableSpawn`
  (params (previousSpawn :type "/Game/Blueprints/Managers/EnemyWaves/BP_EnemySpawnPoint Object Reference"))
  (returns (selectedSpawn :type "/Game/Blueprints/Managers/EnemyWaves/BP_EnemySpawnPoint Object Reference"))
  (locals (spawns :type "Array of /Game/Blueprints/Managers/EnemyWaves/BP_EnemySpawnPoint Object Reference"))
  (bind _keys (`BlueprintMapLibrary.Map_Keys` (`self.spawnPoints`)))
  (bind _output_get (set `local.spawns` _keys))
  (`KismetArrayLibrary.Array_Shuffle` _output_get)
  (for _array_element (`local.spawns`)
    (if (and (!= _array_element (`local.previousSpawn`)) (not (`BlueprintMapLibrary.Map_Find` (`self.spawnPoints`) _array_element)))
      (return _array_element)))
  (return (`local.previousSpawn`)))

(fn `ResetSpawnPoints`
  (bind _spawnedenemies (`self.spawnedEnemies`))
  (bind _keys (`BlueprintMapLibrary.Map_Keys` (`self.spawnPoints`)))
  (for _array_element _keys
    (`BlueprintMapLibrary.Map_Add` (`self.spawnPoints`) _array_element)
    (for _array_element_2 _spawnedenemies
      (`/Engine/EditorBlueprintResources/StandardMacros.IsValid` _array_element_2
        (:`Is Valid`
          (`Actor.K2_DestroyActor` _array_element_2))))
    (`KismetArrayLibrary.Array_Clear` _spawnedenemies)))

(fn `SpawnEnemy`
  (params (previousSpawn :type "/Game/Blueprints/Managers/EnemyWaves/BP_EnemySpawnPoint Object Reference"))
  (bind _selectedspawn (`self.GetNewAvailableSpawn` previousSpawn))
  (`BlueprintMapLibrary.Map_Add` (`self.spawnPoints`) _selectedspawn true)
  (bind _returnvalue (`|SpawnActorFromClass` "/Game/Blueprints/Characters/Enemies/BP_ArenaGunnerEnemy.BP_ArenaGunnerEnemy_C" (`Actor.GetTransform` _selectedspawn) "AlwaysSpawn" "MultiplyWithRoot" null _selectedspawn null))
  (`KismetArrayLibrary.Array_AddUnique` (`self.spawnedEnemies`) _returnvalue)
  (add `/Game/Blueprints/Characters/Enemies/BP_ArenaGunnerEnemy.OnDeath` _returnvalue (`|CreateDelegate` :!event `EnemyDeath`)))