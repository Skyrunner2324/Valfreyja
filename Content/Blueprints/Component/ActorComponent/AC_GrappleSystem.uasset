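; Actor component that drives the player's grappling hook, pulling the character toward the current grapple point.
; Input fires only if the point is valid, recently rendered and no grapple is active, then plays a Wwise sound and starts a short freeze.
; After the freeze it locks the direction, and Tick repeatedly calls LaunchCharacter along it, slowing near the target and stopping within reach or if the point becomes invalid.
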(event `self.ReceiveBeginPlay`
  (set `self.playerCharacter` (cast `/Game/Blueprints/Characters/BP_PlayerCharacter` (`GameplayStatics.GetPlayerCharacter` 0) :!pure true))
  (set `self.splineGrapple` (`/Game/Blueprints/Characters/BP_PlayerCharacter.SplineGrapple` (`self.playerCharacter`))))

(event `EnhancedInput|/Game/Inputs/Actions/IA_UseGrapin`
  (params (ActionValue :type Boolean) (ElapsedSeconds :type "Float (double-precision)") (TriggeredSeconds :type "Float (double-precision)") (InputAction :type "InputAction Object Reference" :default "/Game/Inputs/Actions/IA_UseGrapin.IA_UseGrapin"))
  (:`Triggered`
    (`self.canUseGrapple`
      (:`CanGrapin`
        (set `self.grapin?` true)
        (set `self.freeze` true)
        (set `self.speed` (`self.speedLaunch`))
        (`KismetSystemLibrary.K2_SetTimer` null "UnFreeze" (`self.timeFreeze`))
        ;[0 1 0.2423] Grapple Sound
        (`AkGameplayStatics.PostEvent` "/Game/WwiseAudio/Events/Game/Grap/grap_shot.grap_shot")))))

(event `self.ReceiveTick`
  (params (DeltaSeconds :type "Float (single-precision)"))
  (if (and (`self.grapin?`) (not (`self.freeze`)))
    (`/Engine/EditorBlueprintResources/StandardMacros.IsValid` (`self.actualGrapplePoint`)
      (:`Is Valid`
        (set `self.distanceToGrapplePoint` (`self.GetDistanceToGrapplePoint`))
        (if (< (`self.distanceToGrapplePoint`) (`self.reachTargetDistance`))
          (set `self.grapin?` false :!label _label)
          (else
            (if (< (`self.distanceToGrapplePoint`) (`self.distanceToReduceSpeed`))
              (set `self.speed` (`KismetMathLibrary.FClamp` (- (`self.speed`) (* (`self.valueToReduceSpeed`) (`GameplayStatics.GetWorldDeltaSeconds`))) (`self.minSpeed`) 10000000000.0)))
            (`Character.LaunchCharacter` (`self.playerCharacter`) (* (`self.directionToGrapplePoint`) (`self.speed`)) true true))))
      (:`Is Not Valid`
        (goto _label)))))

(fn `GetDistanceToGrapplePoint`
  (returns (ReturnValue :type "Float (single-precision)"))
  (return (`Actor.GetDistanceTo` (`self.actualGrapplePoint`) (`self.playerCharacter`))))

(fn `UnFreeze`
  (set `self.freeze` false)
  (set `self.directionToGrapplePoint` (`KismetMathLibrary.Normal` (- (`Actor.K2_GetActorLocation` (`self.actualGrapplePoint`)) (`Actor.K2_GetActorLocation` (`self.playerCharacter`))))))