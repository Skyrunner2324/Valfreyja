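; Actor component that gives the player a crouch-slide when the crouch input starts, gated by a speed check.
; Sliding launches the character forward at max slide speed, swaps in slide friction and braking, and plays a sound.
; A looping timer adds downhill impulse from the floor normal and caps top speed.
; Releasing crouch or dropping below minimum speed stops the timer and restores the saved movement values.
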(event `self.ReceiveBeginPlay`
  (set `self.playerCharacter` (cast `/Game/Blueprints/Characters/BP_PlayerCharacter` (`GameplayStatics.GetPlayerCharacter` 0) :!pure true))
  (set `self.playerCharaterMovement` (`Character.CharacterMovement` (`self.playerCharacter`)))
  (set `self.baseGroundFriction` (`CharacterMovementComponent.GroundFriction` (`self.playerCharaterMovement`)))
  (set `self.baseBrakingDecelerationWalking` (`CharacterMovementComponent.BrakingDecelerationWalking` (`self.playerCharaterMovement`))))

(event `EnhancedInput|/Game/Inputs/Actions/IA_Crouch`
  (params (ActionValue :type Boolean) (ElapsedSeconds :type "Float (double-precision)") (TriggeredSeconds :type "Float (double-precision)") (InputAction :type "InputAction Object Reference" :default "/Game/Inputs/Actions/IA_Crouch.IA_Crouch"))
  ;[1 1 1] Crouch/Slide
  (:`Started`
    (`Character.Crouch` (`self.playerCharacter`))
    (`self.CheckCanSlide`)
    (set `self.slide` true)
    (`self.StartSlide`)
    ;;[0 1 0.2423] Slide sound
    (`AkGameplayStatics.PostEvent` null))
  (:`Completed`
    (`Character.UnCrouch` (`self.playerCharacter`))
    (`self.CancelSlide`)))

(event `BeginSlide`
  (bind (_currentfloor_bblockinghit _currentfloor_bwalkablefloor _currentfloor_blinetrace _currentfloor_floordist _currentfloor_linedist _currentfloor_hitresult) (break `FindFloorResult` (`CharacterMovementComponent.CurrentFloor` (`self.playerCharaterMovement`))))
  ;[1 1 1] Slide Loop
  (bind _returnvalue (`KismetSystemLibrary.K2_SetTimerDelegate` (delegate `BeginSlide`) 0.01 true))
  (set `self.timerHandlerBeginSlide` _returnvalue)
  (`CharacterMovementComponent.AddImpulse` (`self.playerCharaterMovement`) (`self.CalculateFloorInfluence` (`.Normal` (`GameplayStatics.BreakHitResult` _currentfloor_hitresult))) false)
  (`|ExecutionSequence`
    (:`then_0`
      (`self.CheckSlideGoToFast`))
    (:`then_1`
      (`self.CheckSlideGoTooSlowly`))))

(event `EndSlide`
  ;[1 1 1] Slide Loop
  (`KismetSystemLibrary.K2_ClearAndInvalidateTimerHandle` (`self.timerHandlerBeginSlide`)))

(fn `CalculateFloorInfluence`
  (params (floorNormal :type "Vector Structure"))
  (returns (returnValue :type "Vector Structure"))
  (if (== floorNormal (`KismetMathLibrary.Vector_Up`) :`ErrorTolerance` 0.0001)
    (return (0.0 0.0 0.0))
    (else
      (return (* (`KismetMathLibrary.Normal` (`KismetMathLibrary.Cross_VectorVector` (`local.floorNormal`) (`KismetMathLibrary.Cross_VectorVector` (`local.floorNormal`) (`KismetMathLibrary.Vector_Up`)))) (* (`KismetMathLibrary.FClamp` (- 1.0 (`KismetMathLibrary.Dot_VectorVector` (`local.floorNormal`) (`KismetMathLibrary.Vector_Up`)))) (`self.floorInfluenceWhenSlide`)))))))

(fn `CancelSlide`
  (`self.SetParameterSlide` (`self.baseGroundFriction`) (`self.baseBrakingDecelerationWalking`))
  (`self.EndSlide`)
  (set `self.slide` false))

(fn `CheckSlideGoToFast`
  (if (> (`KismetMathLibrary.VSize` (`Actor.GetVelocity` (`self.playerCharacter`))) (`self.maxSpeedSlide`))
    (set `MovementComponent.Velocity` (* (`KismetMathLibrary.Normal` (`Actor.GetVelocity` (`self.playerCharacter`))) (`self.maxSpeedSlide`)) (`self.playerCharaterMovement`))))

(fn `CheckSlideGoTooSlowly`
  (if (< (`KismetMathLibrary.VSize` (`Actor.GetVelocity` (`self.playerCharacter`))) (`self.minSpeedSlide`))
    (`self.CancelSlide`)))

(fn `SetParameterSlide`
  (params (`Ground Friction` :type "Float (single-precision)") (`Braking Deceleration Walking` :type "Float (single-precision)"))
  (set `CharacterMovementComponent.GroundFriction` `Ground Friction` (`self.playerCharaterMovement`))
  (set `CharacterMovementComponent.BrakingDecelerationWalking` (`local.Braking Deceleration Walking`) (`self.playerCharaterMovement`)))

(fn `StartSlide`
  (set `MovementComponent.Velocity` (* (`Actor.GetActorForwardVector` (`self.playerCharacter`)) (`self.maxSpeedSlide`)) (`self.playerCharaterMovement`))
  (`self.SetParameterSlide` (`self.slideGroundFriction`) (`self.slideBrakingDecelerationWalking`))
  (`self.BeginSlide`))