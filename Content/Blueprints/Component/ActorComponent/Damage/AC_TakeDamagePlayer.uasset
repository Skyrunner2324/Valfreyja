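; Player damage component that extends its parent's damage handling with player feedback.
; The TakeDamage override runs the parent logic, then casts the owner to BP_PlayerCharacter and sends the current-to-max health ratio to the HUD.
; It then posts the Wwise player-hit sound event, so neither feedback occurs if the cast fails.
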(fn `TakeDamage`
  (params (damageComponent :type "/Game/Blueprints/Component/ActorComponent/Damage/AC_DoDamage Object Reference"))
  (`parent.TakeDamage` damageComponent)
  (bind _asbp_player_character (cast `/Game/Blueprints/Characters/BP_PlayerCharacter` (`self.GetOwner`)))
  (`/Game/Blueprints/HUD/BP_PlayerHUD.PlayerHealth` (`/Game/Blueprints/Characters/BP_PlayerCharacter.HUD` _asbp_player_character) (/ (`self.GetCurrentHealth`) (`self.GetMaxHealth`)))
  (`AkGameplayStatics.PostEvent` "/Game/WwiseAudio/Events/Player/Feedback/SX_player_hit.SX_player_hit"))