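; Actor component that tracks the health of its owner and applies incoming damage.
; Current health starts at the maximum on BeginPlay, and both values are exposed through getter functions.
; TakeDamage reads the damage amount from a valid damage component passed to it, prints the pre-hit health and subtracts the damage, triggering CallDeath at zero or below.
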(event `self.ReceiveBeginPlay`
  (set `self.currentHealth` (`self.maxHealth`)))

(fn `GetCurrentHealth`
  (returns (currentHealth :type Integer))
  (return (`self.currentHealth`)))

(fn `GetMaxHealth`
  (returns (maxHealth :type Integer))
  (return (`self.maxHealth`)))

(fn `TakeDamage`
  (params (damageComponent :type "/Game/Blueprints/Component/ActorComponent/Damage/AC_DoDamage Object Reference"))
  (bind _currenthealth (`self.currentHealth`))
  (`/Engine/EditorBlueprintResources/StandardMacros.IsValid` (`local.damageComponent`)
    (:`Is Valid`
      (`KismetSystemLibrary.PrintString` (`KismetStringLibrary.Conv_IntToString` _currenthealth))
      (set `self.currentHealth` (- _currenthealth (`/Game/Blueprints/Component/ActorComponent/Damage/AC_DoDamage.damage` (`local.damageComponent`))))
      (if (<= (`self.currentHealth`) 0)
        (`self.Death`)))))