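; Player component that adds crouch and speed-gated slide with cooldown, triggered by crouch input or on landing while held.
; A looping timer adds slope-based impulses, caps speed and cancels slow slides, while friction and braking are swapped during slides.
; Crouch timers snap capsule height and interpolate camera height.
; A capsule trace gates standing after slow slides, with Tick retrying when blocked.
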(event `self.ReceiveBeginPlay`
  (`self.SetCharacterValue`)
  (`self.SetBaseValue`))

(event `EnhancedInput|/Game/Inputs/Actions/IA_Crouch`
  (params (ActionValue :type Boolean) (ElapsedSeconds :type "Float (double-precision)") (TriggeredSeconds :type "Float (double-precision)") (InputAction :type "InputAction Object Reference" :default "/Game/Inputs/Actions/IA_Crouch.IA_Crouch"))
  ;[1 1 1] Crouch/Slide
  (:`Started`
    (`self.TriggerCrouch`))
  (:`Completed`
    (set `self.keyHoldCrouch?` false)))

(event `BeginSlide`
  (bind (_currentfloor_bblockinghit _currentfloor_bwalkablefloor _currentfloor_blinetrace _currentfloor_floordist _currentfloor_linedist _currentfloor_hitresult) (break `FindFloorResult` (`CharacterMovementComponent.CurrentFloor` (`self.playerCharaterMovement`))))
  ;[1 1 1] Slide Loop
  (bind _returnvalue (`KismetSystemLibrary.K2_SetTimerDelegate` (delegate `BeginSlide`) 0.01 true))
  (set `self.timerHandleBeginSlide` _returnvalue)
  (`CharacterMovementComponent.AddImpulse` (`self.playerCharaterMovement`) (`self.CalculateFloorInfluence` (`.Normal` (`GameplayStatics.BreakHitResult` _currentfloor_hitresult))) false)
  (`|ExecutionSequence`
    (:`then_0`
      (`self.CheckSlideGoToFast`))
    (:`then_1`
      (`self.CheckSlideGoTooSlowly`))))

(event `EndSlide`
  ;[1 1 1] Slide Loop
  (`KismetSystemLibrary.K2_ClearAndInvalidateTimerHandle` (`self.timerHandleBeginSlide`)))

(event `self.ReceiveTick`
  (params (DeltaSeconds :type "Float (single-precision)"))
  ;[1 1 1] Check Can Stand
  (if (`self.checkCanStand`)
    (`self.CanStand`
      (:`CanStand`
        (`self.StartUnCrouch`)
        (set `self.checkCanStand` false)))))

(fn `BaseStartCrouchFunction`
  (params (functionName :type String) (walkSpeed :type "Float (double-precision)"))
  (`KismetSystemLibrary.K2_ClearAndInvalidateTimerHandle` (`self.timerHandleCrouch`))
  (set `CharacterMovementComponent.MaxWalkSpeed` (`local.walkSpeed`) (`self.playerCharaterMovement`))
  (`self.SetActualValue`)
  (bind _returnvalue (`KismetSystemLibrary.K2_SetTimer` null (`local.functionName`) 0.001 true))
  (set `self.timerHandleCrouch` _returnvalue)
  (return))

(fn `CalculateFloorInfluence`
  (params (floorNormal :type "Vector Structure"))
  (returns (returnValue :type "Vector Structure"))
  (if (== floorNormal (`KismetMathLibrary.Vector_Up`) :`ErrorTolerance` 0.0001)
    (return (0.0 0.0 0.0))
    (else
      (return (* (`KismetMathLibrary.Normal` (`KismetMathLibrary.Cross_VectorVector` (`local.floorNormal`) (`KismetMathLibrary.Cross_VectorVector` (`local.floorNormal`) (`KismetMathLibrary.Vector_Up`)))) (* (`KismetMathLibrary.FClamp` (- 1.0 (`KismetMathLibrary.Dot_VectorVector` (`local.floorNormal`) (`KismetMathLibrary.Vector_Up`)))) (`self.floorInfluenceWhenSlide`)))))))

(fn `CancelSlide`
  (if (`self.slide`)
    (`self.SetParameterSlide` (`self.baseGroundFriction`) (`self.baseBrakingDecelerationWalking`))
    (`self.EndSlide`)
    (set `self.slide` false)
    (`KismetSystemLibrary.K2_SetTimer` null "ResetCanSlide" (`self.delayBetweenSlide`))))

(fn `CheckCanClearTimerHandler`
  (params (targetCameraPosition :type "Float (double-precision)") (targetCapsuleHalfHeight :type "Float (double-precision)"))
  (if (and (`KismetMathLibrary.NearlyEqual_FloatFloat` (`self.actualPostionCamera`) (`local.targetCameraPosition`) 0.01) (`KismetMathLibrary.NearlyEqual_FloatFloat` (`self.actualCapsuleHalfHeight`) (`local.targetCapsuleHalfHeight`) 0.01))
    (`KismetSystemLibrary.K2_ClearAndInvalidateTimerHandle` (`self.timerHandleCrouch`))))

(fn `CheckCrouchAtLand`
  (if (`self.keyHoldCrouch?`)
    (`self.TriggerCrouch`)))

(fn `CheckSlideGoToFast`
  (if (> (`KismetMathLibrary.VSize` (`Actor.GetVelocity` (`self.playerCharacter`))) (`self.maxSpeedSlide`))
    (set `MovementComponent.Velocity` (* (`KismetMathLibrary.Normal` (`Actor.GetVelocity` (`self.playerCharacter`))) (`self.maxSpeedSlide`)) (`self.playerCharaterMovement`))))

(fn `CheckSlideGoTooSlowly`
  (if (< (`KismetMathLibrary.VSize` (`Actor.GetVelocity` (`self.playerCharacter`))) (`self.minSpeedSlide`))
    (`self.CancelSlide`)
    (`self.CanStand`
      (:`CanStand`
        (`self.TriggerUnCrouch`))
      (:`CantStand`
        (set `self.checkCanStand` true)))))

(fn `Crouch`
  (`self.LerpCrouchPosition` (`self.crouchHalfHeightCapsule`) (`self.crouchCameraPosition`)))

(fn `IsSliding`
  (returns (isSliding :type Boolean))
  (return (`self.slide`)))

(fn `LandEvent`
  (`KismetSystemLibrary.K2_SetTimer` null "CheckCrouchAtLand" 0.01))

(fn `LerpCrouchPosition`
  (params (targetCapsuleHalfHeight :type "Float (double-precision)") (targetCameraPosition :type "Float (double-precision)"))
  (bind (_relativelocation_x _relativelocation_y) (`KismetMathLibrary.BreakVector` (`SceneComponent.RelativeLocation` (`self.playerCharacterCamera`))))
  (set `self.actualCapsuleHalfHeight` (`KismetMathLibrary.FInterpTo` (`self.actualCapsuleHalfHeight`) (`local.targetCapsuleHalfHeight`) (`GameplayStatics.GetWorldDeltaSeconds`) (`self.speedLerpCrouch`)))
  (`CapsuleComponent.SetCapsuleHalfHeight` (`self.playerCharacterCapsuleComponent`) (`local.targetCapsuleHalfHeight`) true)
  (set `self.actualPostionCamera` (`KismetMathLibrary.FInterpTo` (`self.actualPostionCamera`) (`local.targetCameraPosition`) (`GameplayStatics.GetWorldDeltaSeconds`) (`self.speedLerpCrouch`)))
  (`SceneComponent.K2_SetRelativeLocation` (`self.playerCharacterCamera`) (`KismetMathLibrary.MakeVector` _relativelocation_x _relativelocation_y (`self.actualPostionCamera`)) false false)
  (`self.CheckCanClearTimerHandler` (`local.targetCameraPosition`) (`local.targetCapsuleHalfHeight`)))

(fn `ResetCanSlide`
  (set `self.canSlide` true))

(fn `SetActualValue`
  (bind (_relativelocation_x _relativelocation_y _relativelocation_z) (`KismetMathLibrary.BreakVector` (`SceneComponent.RelativeLocation` (`self.playerCharacterCamera`))))
  (set `self.actualCapsuleHalfHeight` (`CapsuleComponent.CapsuleHalfHeight` (`self.playerCharacterCapsuleComponent`)))
  (set `self.actualPostionCamera` _relativelocation_z))

(fn `SetBaseValue`
  (bind (_relativelocation_x _relativelocation_y _relativelocation_z) (`KismetMathLibrary.BreakVector` (`SceneComponent.RelativeLocation` (`self.playerCharacterCamera`))))
  (set `self.baseGroundFriction` (`CharacterMovementComponent.GroundFriction` (`self.playerCharaterMovement`)))
  (set `self.baseBrakingDecelerationWalking` (`CharacterMovementComponent.BrakingDecelerationWalking` (`self.playerCharaterMovement`)))
  (set `self.baseHalfHeightCapsule` (`CapsuleComponent.GetScaledCapsuleHalfHeight` (`self.playerCharacterCapsuleComponent`)))
  (set `self.baseCameraZPosition` _relativelocation_z)
  (set `self.baseWalkSpeed` (`CharacterMovementComponent.MaxWalkSpeed` (`self.playerCharaterMovement`))))

(fn `SetCharacterValue`
  (set `self.playerCharacter` (cast `/Game/Blueprints/Characters/BP_PlayerCharacter` (`GameplayStatics.GetPlayerCharacter` 0) :!pure true))
  (set `self.playerCharaterMovement` (`Character.CharacterMovement` (`self.playerCharacter`)))
  (set `self.playerCharacterCapsuleComponent` (`Character.CapsuleComponent` (`self.playerCharacter`)))
  (set `self.playerCharacterCamera` (`/Game/Blueprints/Characters/BP_PlayerCharacter.FirstPersonCamera` (`self.playerCharacter`))))

(fn `SetParameterSlide`
  (params (`Ground Friction` :type "Float (single-precision)") (`Braking Deceleration Walking` :type "Float (single-precision)"))
  (set `CharacterMovementComponent.GroundFriction` `Ground Friction` (`self.playerCharaterMovement`))
  (set `CharacterMovementComponent.BrakingDecelerationWalking` (`local.Braking Deceleration Walking`) (`self.playerCharaterMovement`)))

(fn `StartCrouch`
  (`self.BaseStartCrouchFunction` "Crouch" (`self.crouchWalkSpeed`)))

(fn `StartSlide`
  (set `self.canSlide` false)
  (set `MovementComponent.Velocity` (* (`Actor.GetActorForwardVector` (`self.playerCharacter`)) (`self.maxSpeedSlide`)) (`self.playerCharaterMovement`))
  (`self.SetParameterSlide` (`self.slideGroundFriction`) (`self.slideBrakingDecelerationWalking`))
  (`self.BeginSlide`)
  (set `self.slide` true))

(fn `StartUnCrouch`
  (`self.BaseStartCrouchFunction` "UnCrouch" (`self.baseWalkSpeed`)))

(fn `TriggerCrouch`
  (set `self.keyHoldCrouch?` true)
  (set `self.checkCanStand` false)
  (if (not (`NavMovementComponent.IsFalling` (`self.playerCharaterMovement`)))
    (`self.CheckCanSlide`)
    (`self.StartCrouch`)
    (`self.StartSlide`)
    ;[0 1 0.2423] Slide sound
    (`AkGameplayStatics.PostEvent` "/Game/WwiseAudio/Events/Game/Player/SX_player_slide.SX_player_slide")))

(fn `TriggerUnCrouch`
  (`self.StartUnCrouch`)
  (`self.CancelSlide`))

(fn `UnCrouch`
  (`self.LerpCrouchPosition` (`self.baseHalfHeightCapsule`) (`self.baseCameraZPosition`)))