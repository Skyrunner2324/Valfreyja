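; Player dash ability component that sweeps the character toward the last input direction, or forward without input, with camera, FOV and HUD icon feedback.
; A timeline drives the location lerp, its rate adjusted for local and global time scales, and ends when blocked.
; Stopping starts a tick-based cooldown on time-slippage delta.
; Airborne dashes are limited to one outside slow motion; slow-motion dashes spend dilation and cancel sniper shots like any dash.
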(event `self.Init_`
  ;[1 1 1] Init
  (`parent.Init_`)
  (add `self.OnTimelineFinished` (`|CreateDelegate` :!event `EndTimeLineDash`))
  (add `self.OnTimelineUpdate` (`|CreateDelegate` :!event `LerpToTarget`))
  (set `self.dashIcon` (`/Game/UI/HUD/WB_HUD.WB_DashIcon` (`/Game/Blueprints/HUD/BP_PlayerHUD.hudWidget` (`/Game/Blueprints/Characters/BP_PlayerCharacter.HUD` (`self.playerCharacter`))))))

(event `CoolDownDash`
  ;[1 1 1] CoolDownDash
  (`self.SetComponentTickEnabled` true))

(event `self.ReceiveTick`
  (params (DeltaSeconds :type "Float (single-precision)"))
  (bind _currentsettings_cooldown (break `/Game/Blueprints/Struct/ST_DashParameters` (`self.currentSettings`)))
  ;[1 1 1] CoolDownDash
  (bind _output_get (set `self.elapsedCompletionTime` (+ (`self.elapsedCompletionTime`) (`TimeSlippage.applicationDeltaTime` (`/Game/Blueprints/Controller/BP_PlayerController.TimeSlippageRef` (`self.playerController`))))))
  (if (>= _output_get _currentsettings_cooldown)
    (set `self.coolDownOver` true)
    (set `self.elapsedCompletionTime` 0.0)
    (`|ExecutionSequence`
      (:`then_0`
        ;;[0 0 0] Limit to 1 dash in air when the slow motion is not active
        (if (or (not (`NavMovementComponent.IsFalling` (`Character.CharacterMovement` (`self.ownerCharacter`)))) (`|EnumEquality` (`/Game/Blueprints/Controller/BP_PlayerController.DilationType` (`self.playerController`)) "NewEnumerator2"))
          (`self.ResetDash`)))
      (:`then_1`
        (`self.SetComponentTickEnabled` false)))))

(fn `ApplyVelocity`
  (params (Velocity :type "Vector Structure")))

(fn `CanUseAbility`
  (returns (canUseAbility :type Boolean))
  (bind _asbp_player_controller (cast `/Game/Blueprints/Controller/BP_PlayerController` (`GameplayStatics.GetPlayerController` 0) :!pure true))
  (if (and (`parent.CanUseAbility`) (`self.canDash`))
    (`/Game/Blueprints/Libraries/MacroLibraries/BPML_TimeManagementActorComponent.DilationTypeDo` _asbp_player_controller
      (:`NoDilation`
        (return true))
      (:`WeakDilation`
        _)
      (:`StrongDilation`
        _))
    (if (> (`self.slowmoCost`) (`/Game/Blueprints/Controller/BP_PlayerController.GetCurrentDilationAbility` _asbp_player_controller))
      (return false)
      (else
        (return true)))
    (else
      (return false))))

(fn `DashUsed`
  (returns (out :type Boolean))
  (return (not (`self.canDash`))))

(fn `GetDefaultTargetLocation`
  (returns (ReturnValue :type "Vector Structure"))
  (return (+ (`Actor.K2_GetActorLocation` (`self.ownerCharacter`)) (`Actor.GetActorForwardVector` (`self.ownerCharacter`)))))

(fn `GetDirectionalDirection`
  (returns (ReturnValue :type "Vector Structure"))
  (return (`KismetMathLibrary.Normal` (`PawnMovementComponent.GetLastInputVector` (`Character.CharacterMovement` (`self.ownerCharacter`))))))

(fn `GetEndVelocity`
  (returns (ReturnValue :type "Vector Structure"))
  (bind _directiontotarget (`self.directionToTarget`))
  (bind _returnvalue_x (`KismetMathLibrary.BreakVector` (`KismetMathLibrary.InverseTransformDirection` (`Actor.GetTransform` (`self.ownerCharacter`)) _directiontotarget)))
  (return (select `bool` (>= _returnvalue_x (`self.maxAngleForwardDash`)) :`true` (* _directiontotarget (`self.minSpeed`)))))

(fn `Land`
  (if (`self.coolDownOver`)
    (`self.ResetDash`)))

(fn `LerpToTarget`
  (params (ratio :type "Float (double-precision)"))
  (bind (_sweephitresult _returnvalue) (`Actor.K2_SetActorLocation` (`self.ownerCharacter`) (`KismetMathLibrary.VLerp` (`self.startLocation`) (`self.targetLocation`) ratio) true false))
  (if (not _returnvalue)
    (`self.EndTimeLineDash`)))

(fn `ResetDash`
  (if (not (`self.canDash`))
    (`/Game/UI/HUD/WB_DashIcon.DashIconAppearAnim` (`self.dashIcon`)))
  (set `self.canDash` true)
  (set `self.coolDownOver` true)
  (set `self.useAbility` false)
  (`self.SetComponentTickEnabled` false)
  (set `self.elapsedCompletionTime` 0.0))

(fn `SetDirection`
  (params (targetLocation :type "Vector Structure"))
  (locals (localTargetLocation :type "Vector Structure"))
  (bind _returnvalue (`self.GetDirectionalDirection`))
  (set `local.localTargetLocation` (+ (`Actor.K2_GetActorLocation` (`self.ownerCharacter`)) _returnvalue))
  (if (<= (`KismetMathLibrary.VSize` _returnvalue) 0.0)
    (set `local.localTargetLocation` (`self.GetDefaultTargetLocation`)))
  (`parent.SetDirection` (`local.localTargetLocation`)))

(fn `SetTargetLocation`
  (locals (localTargetLocation :type "Vector Structure"))
  (bind (_currentsettings_cooldown _currentsettings_speeddash _currentsettings_dashdistance) (break `/Game/Blueprints/Struct/ST_DashParameters` (`self.currentSettings`)))
  (set `self.targetLocation` (+ (`Actor.K2_GetActorLocation` (`self.ownerCharacter`)) (* (`self.directionToTarget`) _currentsettings_dashdistance))))

(fn `StartTimeLineDash`
  (bind (_currentsettings_cooldown _currentsettings_speeddash) (break `/Game/Blueprints/Struct/ST_DashParameters` (`self.currentSettings`)))
  (`TimelineComponent.SetPlayRate` (`self.timeline`) (/ 1.0 (* _currentsettings_speeddash (* (`TimeSlippageModifier.GetLocalTimeScale` (`/Game/Blueprints/Characters/BP_PlayerCharacter.TimeSlippageModifier` (`self.playerCharacter`))) (`TimeSlippage.GetGlobalTimeScale` (`/Game/Blueprints/Controller/BP_PlayerController.TimeSlippageRef` (`self.playerController`)))))))
  (`TimelineComponent.PlayFromStart` (`self.timeline`)))

(fn `StopAbility`
  (`parent.StopAbility`)
  (`self.CoolDownDash`)
  (`TimelineComponent.Stop` (`self.timeline`))
  (set `/Game/Blueprints/Characters/BP_PlayerCharacter.stateFOV` "NewEnumerator2" (`self.playerCharacter`)))

(fn `TriggerAbility`
  (bind _asbp_player_controller (cast `/Game/Blueprints/Controller/BP_PlayerController` (`GameplayStatics.GetPlayerController` 0) :!pure true))
  ;[1 1 1] When cool down is over and we are in slowmo can dash (faire  un meilleur fix)
  (if (`self.coolDownOver`)
    (`/Game/Blueprints/Libraries/MacroLibraries/BPML_TimeManagementActorComponent.DilationTypeDo` (`self.playerController`)
      (:`NoDilation`
        _)
      (:`WeakDilation`
        (`self.ResetDash` :!label _label))
      (:`StrongDilation`
        (goto _label))))
  (if (`self.CanUseAbility`)
    (`parent.TriggerAbility`)
    (set `self.coolDownOver` false)
    (set `self.canDash` false)
    (set `self.startLocation` (`Actor.K2_GetActorLocation` (`self.ownerCharacter`)))
    (set `/Game/Blueprints/Characters/BP_PlayerCharacter.stateFOV` "NewEnumerator5" (`self.playerCharacter`))
    (`self.SetDirection` (0.0 0.0 0.0))
    (`self.SetTargetLocation`)
    (`self.StartTimeLineDash`)
    (`/Game/UI/HUD/WB_DashIcon.DashIconDisappearAnim` (`self.dashIcon`))
    (`|ExecutionSequence`
      (:`then_0`
        ;[1 1 1] Camera Effect
        (`PlayerCameraManager.StartCameraShake` :`self` (`GameplayStatics.GetPlayerCameraManager` 0) :`ShakeClass` "/Game/Feedbacks/ScrenShake/SCR_Dash.SCR_Dash_C" :`PlaySpace` "World"))
      (:`then_1`
        (`/Game/Blueprints/Characters/BP_PlayerCharacter.CancelSnipersShots` (`self.playerCharacter`)))
      (:`then_2`
        (`/Game/Blueprints/Libraries/MacroLibraries/BPML_TimeManagementActorComponent.DilationTypeDo` _asbp_player_controller
          (:`WeakDilation`
            _)
          (:`StrongDilation`
            _))
        (`/Game/Blueprints/Controller/BP_PlayerController.AddDilation` _asbp_player_controller (- 0.0 (`self.slowmoCost`)))))))