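; AC_Ability is an actor component that provides basic state handling for a player ability.
; On BeginPlay it caches the player character, player controller and owning character.
; TriggerAbility sets the UseAbility flag and posts a Wwise sound event, while StopAbility clears the flag.
; CanUseAbility allows use only while the flag is clear.
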(event `self.ReceiveBeginPlay`
  (set `self.playerCharacter` (cast `/Game/Blueprints/Characters/BP_PlayerCharacter` (`GameplayStatics.GetPlayerCharacter` 0) :!pure true))
  (set `self.playerController` (cast `/Game/Blueprints/Controller/BP_PlayerController` (`GameplayStatics.GetPlayerController` 0) :!pure true))
  (set `self.ownerCharacter` (cast `Character` (`self.GetOwner`) :!pure true)))

(fn `CanUseAbility`
  (returns (canUseAbility :type Boolean))
  (return (not (`self.useAbility`))))

(fn `StopAbility`
  (set `self.useAbility` false))

(fn `TriggerAbility`
  (set `self.useAbility` true)
  ;[0 1 0.2431] Trigger Sound Ability
  (`AkGameplayStatics.PostEvent` (`self.soundAbility`)))