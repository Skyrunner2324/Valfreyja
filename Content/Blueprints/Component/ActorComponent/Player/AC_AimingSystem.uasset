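; Player controller component that auto-locks the aim target in front of the first-person camera and marks it with a dot.
; Each tick, a camera sphere trace finds a candidate and a visibility line trace confirms line of sight.
; A new lock plays a sound and spawns BP_DotMarker, which a looping timer keeps on enemy targets.
; References refresh on the game mode's player reset event; older angle-based selection remains disconnected.
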(event `self.ReceiveBeginPlay`
  ;[1 1 1] begin play
  (bind _asskyrunner_game_mode (cast `SkyrunnerGameMode` (`GameplayStatics.GetGameMode`)))
  (add `SkyrunnerGameMode.OnPlayerResetEvent` _asskyrunner_game_mode (delegate `OnReset`)))

(event `OnReset`
  ;[1 1 1] begin play
  (`|ExecutionSequence`
    (:`then_0`
      (bind _asplayer_controller (cast `PlayerController` (`self.GetOwner`)))
      (bind _output_get (set `self.controllerRef` _asplayer_controller))
      (set `self.controlledPawnRef` (cast `/Game/Blueprints/Characters/BP_PlayerCharacter` (`Controller.K2_GetPawn` _output_get) :!pure true)))
    (:`then_1`
      (`self.SetComponentTickEnabled` true))))

(event `UpdateDotMarkerPos`
  (bind _targetlocked (`self.targetLocked`)
    (:`then`
      (`Actor.K2_SetActorLocation` (`self.dotMarker`) (`SceneComponent.K2_GetComponentLocation` _targetlocked) false false))
    (:`else`)))

(event `self.ReceiveTick`
  (params (DeltaSeconds :type "Float (single-precision)"))
  (`self.targetLocked`
    (:`then`
      (`self.GetTarget`)
      (`self.targetLocked`
        (:`then`)
        (:`else`
          (`self.UnlockTarget`))))
    (:`else`
      (`|ExecutionSequence`
        (:`then_0`
          (`self.dotMarker`
            (:`then`
              (`KismetSystemLibrary.K2_ClearAndInvalidateTimerHandle` (`self.dotMarkerUpdate`))
              (`Actor.K2_DestroyActor` (`self.dotMarker`)))
            (:`else`)))
        (:`then_1`
          (`self.GetTarget`)
          (bind _targetlocked (`self.targetLocked`)
            (:`then`
              (`AkGameplayStatics.PostEvent` "/Game/WwiseAudio/Events/Player/Feedback/SX_player_autolock.SX_player_autolock")
              (bind _returnvalue (`self.GetOwner` _targetlocked))
              (bind _returnvalue_2 (`|SpawnActorFromClass` "/Game/Blueprints/Characters/Enemies/BP_DotMarker.BP_DotMarker_C" (`SceneComponent.K2_GetComponentToWorld` _targetlocked) "Undefined" "MultiplyWithRoot" _returnvalue null))
              (bind _output_get (set `self.dotMarker` _returnvalue_2))
              (bind _asbase_enemy (cast `BaseEnemy` _returnvalue)
                (:`then`
                  (set `BaseEnemy.dotMarker` _output_get _asbase_enemy)
                  (bind _returnvalue_3 (`KismetSystemLibrary.K2_SetTimerDelegate` (delegate `UpdateDotMarkerPos`) 0.01 true))
                  (set `self.dotMarkerUpdate` _returnvalue_3))
                (:`CastFailed`
                  (`SceneComponent.K2_SetRelativeLocation` (`/Game/Blueprints/Characters/Enemies/BP_DotMarker.DotMarker` _output_get) (0.0 0.0 0.0) false true))))
            (:`else`)))))))

(event `UnlockTarget`
  (`/Engine/EditorBlueprintResources/StandardMacros.IsValid` (`self.targetLocked`)
    (:`Is Valid`
      (cast `BaseEnemy` (`self.GetOwner` (`self.targetLocked`))
        (:`then`
          (`KismetSystemLibrary.K2_ClearAndInvalidateTimerHandle` (`self.dotMarkerUpdate`))
          (`Actor.K2_DestroyActor` (`self.dotMarker`)))
        (:`CastFailed`
          _))
      (set `self.targetLocked` null))))

(fn `GetAngleBetweenTargetAndPlayer`
  (params (target :type "SceneComponent Object Reference"))
  (returns (ReturnValue :type "Float (double-precision)"))
  (return (`KismetMathLibrary.DegAcos` (`KismetMathLibrary.Dot_VectorVector` (`Actor.GetActorForwardVector` (`self.controllerRef`)) (`KismetMathLibrary.Normal` (- (`SceneComponent.K2_GetComponentLocation` target) (`Actor.K2_GetActorLocation` (`GameplayStatics.GetPlayerCharacter` 0))))))))

(fn `GetNearestTarget`
  (params (targets :type "Array of SceneComponent Object Reference"))
  (returns (target :type "SceneComponent Object Reference"))
  (locals (nearestTarget :type "SceneComponent Object Reference") (currentDistance :type "Float (double-precision)" :default 100000.0))
  (for _array_element targets
    (bind _returnvalue (`KismetMathLibrary.Vector_Distance` (`SceneComponent.K2_GetComponentLocation` _array_element) (`Actor.K2_GetActorLocation` (`self.controlledPawnRef`))))
    (if (< _returnvalue (`local.currentDistance`))
      (set `local.nearestTarget` _array_element)
      (set `local.currentDistance` _returnvalue)))
  (return (`local.nearestTarget`)))

(fn `GetTarget`
  (locals (target :type "Actor Object Reference"))
  (bind _firstpersoncamera (`/Game/Blueprints/Characters/BP_PlayerCharacter.FirstPersonCamera` (`self.controlledPawnRef`)))
  (bind _returnvalue (`SceneComponent.K2_GetComponentLocation` _firstpersoncamera))
  (bind (_outhit _returnvalue_2) (`KismetSystemLibrary.SphereTraceSingleForObjects` _returnvalue (+ _returnvalue (* (`SceneComponent.GetForwardVector` _firstpersoncamera) (`self.detectionDistance`))) (`self.detectionRadius`) (`self.objectTypes`)))
  (if _returnvalue_2
    (bind (_bblockinghit _binitialoverlap _time _distance _location _impactpoint _normal _impactnormal _physmat _hitactor) (`GameplayStatics.BreakHitResult` _outhit))
    (set `local.target` _hitactor)
    (bind _outhit_2 (`KismetSystemLibrary.LineTraceSingle` _returnvalue (+ _returnvalue (* (`KismetMathLibrary.Normal` (- (`Actor.K2_GetActorLocation` _hitactor) _returnvalue)) 5000.0)) "TraceTypeQuery1"))
    (bind (_bblockinghit_2 _binitialoverlap_2 _time_2 _distance_2 _location_2 _impactpoint_2 _normal_2 _impactnormal_2 _physmat_2 _hitactor_2 _hitcomponent) (`GameplayStatics.BreakHitResult` _outhit_2))
    (if (== _hitactor_2 (`local.target`))
      (set `self.targetLocked` _hitcomponent)
      (else
        (set `self.targetLocked` null)))
    (else
      (set `self.targetLocked` null))))

(fn `GetTargetsInAimArea`
  (returns (targets :type "Array of SceneComponent Object Reference"))
  (locals (targetsInArea :type "Array of SceneComponent Object Reference"))
  (for _array_element (`self.nearTargets`)
    (if (<= (`self.GetAngleBetweenTargetAndPlayer` _array_element) (`self.angleDetectionArea`))
      (`KismetArrayLibrary.Array_Add` (`local.targetsInArea`) _array_element)))
  (return (`local.targetsInArea`)))