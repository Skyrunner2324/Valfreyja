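; Player actor component that plays and stops controller force feedback effects on player controller 0.
; Looped requests go through the same play function, which also prints the effect name, and are stored uniquely in a pending list.
; Stopping ends the effect and removes the first entry matching either effect or tag.
; PlayPendingList replays every stored entry, allowing tracked feedback to be restarted.
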(fn `PlayForceFeedback`
  (params (params :type "/Game/Blueprints/Struct/ST_ForceFeedback Structure"))
  (`KismetSystemLibrary.PrintString` (`KismetSystemLibrary.GetDisplayName` params_forceFeedbackEffect_3_D560C12F4358ABBD117E72BD1EC62D78))
  (`PlayerController.K2_ClientPlayForceFeedback` (`GameplayStatics.GetPlayerController` 0) params_forceFeedbackEffect_3_D560C12F4358ABBD117E72BD1EC62D78 params_tag_6_34FF77374CFA8AF85A7F938FFE2A9397 params_looping_9_B65A1BC04E2501478E7C2AB02FE00B22 params_IgnoreTimeDilation_11_120C0247426C3A94EF863CAF913FBEDB params_playWhilePaused_13_043B283C4D7056A498034EA8501D2119))

(fn `PlayLoopedForceFeedback`
  (params (params :type "/Game/Blueprints/Struct/ST_ForceFeedback Structure"))
  (`self.PlayForceFeedback` params)
  (`KismetArrayLibrary.Array_AddUnique` (`self.PendingList`) params))

(fn `PlayPendingList`
  (for _array_element (`self.PendingList`)
    (`self.PlayForceFeedback` _array_element)))

(fn `StopForceFeedbackFromPendingList`
  (params (forceFeedbackEffect :type "ForceFeedbackEffect Object Reference") (tag :type Name))
  (`PlayerController.ClientStopForceFeedback` (`GameplayStatics.GetPlayerController` 0) forceFeedbackEffect tag)
  (for _array_element (`self.PendingList`)
    (bind (_forcefeedbackeffect _tag) (break `/Game/Blueprints/Struct/ST_ForceFeedback` _array_element))
    (if (or (== _forcefeedbackeffect (`local.forceFeedbackEffect`)) (== _tag (`local.tag`)))
      (`KismetArrayLibrary.Array_RemoveItem` (`self.PendingList`) _array_element)
      (break))))