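; Actor component that stores the player's respawn point and teleports its owner back to it on demand.
; BeginPlay records the owner's starting location and rotation as the initial spawn.
; SetExactSpawnLocation traces straight down from a given point and saves the hit location plus a vertical offset, leaving the saved rotation unchanged.
; Respawn teleports the owner, zeroes any character movement velocity and restores the first player controller's control rotation.
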(event `self.ReceiveBeginPlay`
  (bind _returnvalue (`self.GetOwner`))
  (set `self.currentRespawnLocation` (`Actor.K2_GetActorLocation` _returnvalue))
  (set `self.currentSpawnRotation` (`Actor.K2_GetActorRotation` _returnvalue)))

(fn `Respawn`
  (bind _returnvalue (`Actor.GetComponentByClass` (`self.GetOwner`) "/Script/Engine.CharacterMovementComponent"))
  (`Actor.K2_SetActorLocation` (`self.GetOwner`) (`self.currentRespawnLocation`) false true)
  (`|ExecutionSequence`
    (:`then_0`
      (`/Engine/EditorBlueprintResources/StandardMacros.IsValid` _returnvalue
        (:`Is Valid`
          (set `MovementComponent.Velocity` (0.0 0.0 0.0) _returnvalue))))
    (:`then_1`
      (`Controller.SetControlRotation` (`GameplayStatics.GetPlayerController` 0) (`self.currentSpawnRotation`)))))

(fn `SetExactSpawnLocation`
  (params (location :type "Vector Structure"))
  (bind _outhit (`KismetSystemLibrary.LineTraceSingle` location (`KismetMathLibrary.MakeVector` (.x location) (.y location) (- (.z location) 1000.0)) "TraceTypeQuery1"))
  (set `self.currentRespawnLocation` (+ (`.Location` (`GameplayStatics.BreakHitResult` _outhit)) (`self.verticalOffset`))))