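; Player grapple ability component that pulls the character to the current grapple point.
; Triggering spawns a hook and cable on the left arm, plays montage and feedback, adds score, and freezes briefly under time-dilation-aware delta.
; Timelines then drive hook visuals, movement updates that re-aim at the target with distance-based lerping, and a real-time watchdog that stops a stalled grapple.
; Stopping destroys visuals, restores rail collision and leaves exit velocity.
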(event EventInit
  (|CallParentFunction)
  (TimeLine|SetTimeLine)
  (TimeLine|BindEventTimeLine))

(fn UnFreeze
  (bind _localgrapplepoint (Variables|GrapllePoint|Private|GetlocalGrapplePoint))
  (Variables|Public|Setfreeze false)
  (Variables|GrapllePoint|Private|SetcounterFreeze 0.0)
  (Utilities|IsValid _localgrapplepoint
    (:Is%20Valid
      (bind _output_get (Variables|Default|SettargetLocation (Transformation|GetActorLocation _localgrapplepoint)))
      (CallFunction|SetDirection _output_get))))

(fn DestroyVisualGrapple
  (Utilities|IsValid (Variables|Visual|GetBP_GrappleCable)
    (:Is%20Valid
      (Actor|DestroyActor (Variables|Visual|GetBP_GrappleCable))
      (Actor|DestroyActor (Variables|Visual|GetBP_GrapplingHook)))))

(fn ShowGrapple
  ;[1 1 1] Spawn Grapple visual and hook
  (bind _returnvalue (Game|SpawnActorfromClass "/Game/Blueprints/Projectiles/Grapple/BP_GrapplingHook.BP_GrapplingHook_C" (Math|Transform|MakeTransform (.location (Transformation|GetActorTransform (Components|GetOwner))) "0, 0, 0" "1.000000,1.000000,1.000000") "AlwaysSpawn" "MultiplyWithRoot" 0 0))
  (Variables|Visual|SetBP_GrapplingHook _returnvalue)
  (bind _returnvalue_2 (Game|SpawnActorfromClass "/Game/Blueprints/Projectiles/Grapple/BP_GrappleCable.BP_GrappleCable_C" (Math|Transform|MakeTransform (.location (Transformation|GetActorTransform (Components|GetOwner))) "0, 0, 0" "1.000000,1.000000,1.000000") "AlwaysSpawn" "MultiplyWithRoot" 0 0))
  (Variables|Visual|SetBP_GrappleCable _returnvalue_2)
  ;[1 1 1] Attack grapple to the arm player and the end of the cable to the hook
  (Transformation|AttachComponentToComponent (Variables|Visual|GetBP_GrappleCable) (Variables|/Game/Blueprints/Characters/BP_PlayerCharacter.BP_PlayerCharacter_C|GetSK_LeftArm (Variables|Default|GetplayerCharacter)) "GrapplePoint" "SnapToTarget" "SnapToTarget" "SnapToTarget" true)
  (Class|CableComponent|SetAttachEndto (Variables|/Game/Blueprints/Projectiles/Grapple/BP_GrappleCable.BP_GrappleCable_C|GetCable (Variables|Visual|GetBP_GrappleCable)) (Variables|Visual|GetBP_GrapplingHook) "None" "None"))

(fn StopAbility
  (if (Variables|Default|GetuseAbility)
    (Variables|/Game/Blueprints/LDElement/Grapple/BP_GrapplePoint.BP_GrapplePoint_C|SetisUsed (Variables|GrapllePoint|Private|GetlocalGrapplePoint) false)
    (|CallParentFunction)
    (Private|DestroyVisualGrapple)
    (Variables|/Script/Engine.MovementComponent|SetVelocity (Variables|/Script/Engine.Character|GetCharacterMovement (Variables|Default|GetownerCharacter)) (* (Variables|Default|GetdirectionToTarget) (Variables|Default|GetminSpeed)))
    (Audio|Components|Audio|Stop (Variables|TimeLine|GettimeLineLerpTargetObjectComponent))
    (Audio|Components|Audio|Stop (Variables|TimeLine|GettimeLineTimeoutObjectComponent))
    (Variables|Private|SetstartTimeLineTimeOut false)
    (Audio|Components|Audio|Stop (Variables|TimeLine|GettimeLineStartTimeOutObjectComponent))
    (Default|SetRailCollisoin (Variables|Default|GetPlayerRef) "QueryOnly")))

(fn GetDistancetoTarget
  (return (Math|Vector|Distance(Vector) (Variables|Default|GettargetLocation) (Transformation|GetActorLocation (Variables|Default|GetownerCharacter)))))

(fn CanUseAbility
  (Utilities|IsValid (Variables|GrapllePoint|Public|GetactualGrapplePoint)
    (:Is%20Valid
      (return (|CallParentFunction)))
    (:Is%20Not%20Valid
      (return false))))

(fn TriggerAbility
  (bind _actualgrapplepoint (Variables|GrapllePoint|Public|GetactualGrapplePoint))
  (if (CallFunction|CanUseAbility)
    (|CallParentFunction)
    (Utilities|IsValid (Variables|Default|GetPlayerRef)
      (:Is%20Valid
        _)
      (:Is%20Not%20Valid
        (bind _asbp_player_character (Utilities|Casting|CastToBP_PlayerCharacter (Game|GetPlayerCharacter 0)))
        (Variables|Default|SetPlayerRef _asbp_player_character)))
    (bind _output_get (Variables|GrapllePoint|Private|SetlocalGrapplePoint (Variables|GrapllePoint|Public|GetactualGrapplePoint)))
    (bind _asbp_enemy_grapple_point (Utilities|Casting|CastToBP_EnemyGrapplePoint _output_get)
      (:then
        (Default|GrappleStart _asbp_enemy_grapple_point self))
      (:CastFailed
        _))
    (Variables|Private|SetoffsetTargetLocation (Variables|/Game/Blueprints/LDElement/Grapple/BP_GrapplePoint.BP_GrapplePoint_C|GetoffsetTargetLocation (Variables|GrapllePoint|Public|GetactualGrapplePoint)))
    (Variables|Public|Setfreeze true)
    ;[1 1 1] Launch Anim Grapple Visual
    (Private|ShowGrapple)
    (Components|Timeline|SetPlayRate (Variables|TimeLine|GettimeLineVisualGrappleObjectComponent) (/ 1.0 (Variables|Settings|GettimeFreeze)))
    (Components|Timeline|PlayfromStart (Variables|TimeLine|GettimeLineVisualGrappleObjectComponent))
    ;[1 1 1] Launch Animation Player
    (Animation|Montage|MontagePlay (Components|SkeletalMesh|GetAnimInstance (Variables|/Game/Blueprints/Characters/BP_PlayerCharacter.BP_PlayerCharacter_C|GetSK_LeftArm (.AsBP%20Player%20Character (Utilities|Casting|CastToBP_PlayerCharacter (Components|GetOwner))))) (Variables|Default|GetANIM_HookArm) 1.1 "MontageLength" 0.0 true)
    ;[0 1 0] Stop Slide loop
    (Class|AkGameplayStatics|PostEvent "/Game/WwiseAudio/Events/Player/Movement/SX_player_slide_end_loop.SX_player_slide_end_loop")
    (Game|Feedback|ClientPlayForceFeedback (Game|GetPlayerController 0) "/Game/Feedbacks/LD_Elements/FFB_GrappleVibration.FFB_GrappleVibration" "None" false true false)
    (Components|Timeline|PlayfromStart (Variables|TimeLine|GettimeLineLerpTargetObjectComponent))
    (Components|Timeline|PlayfromStart (Variables|TimeLine|GettimeLineStartTimeOutObjectComponent))
    (Variables|/Game/Blueprints/LDElement/Grapple/BP_GrapplePoint.BP_GrapplePoint_C|SetisUsed _actualgrapplepoint true)
    (Default|ChangeLockWidget _actualgrapplepoint true true)
    (Default|CallAddScore 250)
    (Default|SetRailCollisoin (Variables|Default|GetPlayerRef) "NoCollision")))

(fn CounterFreeze
  (Variables|GrapllePoint|Private|SetcounterFreeze (+ (Variables|GrapllePoint|Private|GetcounterFreeze) (Variables|/Script/Skyrunner.TimeSlippageModifier|GetlocalManagedDeltaTime (Variables|/Game/Blueprints/Characters/BP_PlayerCharacter.BP_PlayerCharacter_C|GetTimeSlippageModifier (Variables|Default|GetplayerCharacter)))))
  (if (>= (Variables|GrapllePoint|Private|GetcounterFreeze) (Variables|Settings|GettimeFreeze))
    (Private|UnFreeze)))

(fn LerpVisualGrapple
  (params (scale :type Float%20%28single-precision%29))
  (bind _bp_grapplinghook (Variables|Visual|GetBP_GrapplingHook)
    (:then
      (Transformation|SetActorLocation _bp_grapplinghook (Math|Vector|Lerp(Vector) (Transformation|GetActorLocation (Variables|Visual|GetBP_GrapplingHook)) (Transformation|GetActorLocation (Variables|GrapllePoint|Private|GetlocalGrapplePoint)) scale) false false))
    (:else)))

(fn ApplyVelocity
  (params (Velocity :type Vector :default "0, 0, 0"))
  (Character|LaunchCharacter (Variables|Default|GetownerCharacter) Velocity true true))

(fn TimeoutUpdate
  (params (scale :type Float%20%28double-precision%29))
  (bind _ownercharacter (Variables|Default|GetownerCharacter))
  (bind _returnvalue (Transformation|GetActorLocation _ownercharacter))
  (if (not (and (Variables|Public|Getfreeze) (not (Variables|Default|GetstartTimeOutUpdate))))
    (if (< (Math|Vector|Distance(Vector) (Variables|Default|GetOldPlayerLocation) _returnvalue) (Math|Float|SelectFloat (Variables|Settings|GetsecurityStopGrappleSlowMo) (Variables|Settings|GetsecurityStopGrapple) (> (Class|TimeSlippageModifier|GetLocalTimeScale (Variables|/Game/Blueprints/Characters/BP_PlayerCharacter.BP_PlayerCharacter_C|GetTimeSlippageModifier (Variables|Default|GetplayerCharacter))) 1.0)))
      (bind _output_get (Variables|Default|SetTimeoutTimer (- (Variables|Default|GetTimeoutTimer) (Class|TimeDefaults|GetWorldDeltaRealTimeSeconds))))
      (if (<= _output_get 0.0)
        (CallFunction|StopAbility)
        (else
          (Variables|Default|SetOldPlayerLocation _returnvalue :!label _label)))
      (else
        (Variables|Default|SetTimeoutTimer (Variables|Default|GetMaxTimeoutTimer))
        (goto _label)))))

(fn Reset
  (|CallParentFunction)
  (Animation|Montage|MontageStop (Components|SkeletalMesh|GetAnimInstance (Variables|/Game/Blueprints/Characters/BP_PlayerCharacter.BP_PlayerCharacter_C|GetSK_LeftArm (.AsBP%20Player%20Character (Utilities|Casting|CastToBP_PlayerCharacter (Components|GetOwner))))) 0.0 (Variables|Default|GetANIM_HookArm)))

(fn SetDirection
  (params (targetLocation :type Vector :default "0, 0, 0"))
  (|CallParentFunction (- targetLocation (Variables|Private|GetoffsetTargetLocation))))

(fn SetTimeLine
  (Variables|TimeLine|SettimeLineVisualGrapple (Class|MultipleTimelineHandlesComponent|GetTimeline "TimeLineVisualGrapple"))
  (Variables|TimeLine|SettimeLineVisualGrappleObjectComponent (Variables|/Script/TimelineHandleComponent.InstancedTimelineHandle|Gettimeline (Variables|TimeLine|GettimeLineVisualGrapple)))
  (Variables|TimeLine|SettimeLineTimeout (Class|MultipleTimelineHandlesComponent|GetTimeline "TimeLineTimeOut"))
  (Variables|TimeLine|SettimeLineTimeoutObjectComponent (Variables|/Script/TimelineHandleComponent.InstancedTimelineHandle|Gettimeline (Variables|TimeLine|GettimeLineTimeout)))
  (Variables|TimeLine|SettimeLineLerpTarget (Class|MultipleTimelineHandlesComponent|GetTimeline "TimeLineLerpTarget"))
  (Variables|TimeLine|SettimeLineLerpTargetObjectComponent (Variables|/Script/TimelineHandleComponent.InstancedTimelineHandle|Gettimeline (Variables|TimeLine|GettimeLineLerpTarget)))
  (Variables|TimeLine|SettimeLineStartTimeOut (Class|MultipleTimelineHandlesComponent|GetTimeline "TimeLineStartTimeOut"))
  (Variables|TimeLine|SettimeLineStartTimeOutObjectComponent (Variables|/Script/TimelineHandleComponent.InstancedTimelineHandle|Gettimeline (Variables|TimeLine|GettimeLineStartTimeOut))))

(fn BindEventTimeLine
  (EventDispatchers|BindEventtoOnTimelineUpdate (Variables|TimeLine|GettimeLineVisualGrapple) (EventDispatchers|CreateEvent :!event LerpVisualGrapple))
  (Audio|Components|Audio|Stop (Variables|TimeLine|GettimeLineVisualGrappleObjectComponent))
  (EventDispatchers|BindEventtoOnTimelineUpdate (Variables|TimeLine|GettimeLineTimeout) (EventDispatchers|CreateEvent :!event TimeoutUpdate))
  (EventDispatchers|BindEventtoOnTimelineUpdate (Variables|TimeLine|GettimeLineLerpTarget) (EventDispatchers|CreateEvent :!event UpdateTriggerAbility))
  (EventDispatchers|BindEventtoOnTimelineUpdate (Variables|TimeLine|GettimeLineStartTimeOut) (EventDispatchers|CreateEvent :!event StartTimeOut)))

(fn UpdateTriggerAbility
  (params (ratio :type Float%20%28double-precision%29))
  (bind _returnvalue (|(({312FAF6B-466F-FEE3-8982-E8967FB4B647}-{99991C55-4DEA-4B19-07E3-00A6D5718A6B})/({9055D663-4C8B-4EBF-67DB-87A4BF43A572}-{99991C55-4DEA-4B19-07E3-00A6D5718A6B}))))
  (if (Variables|Public|Getfreeze)
    (Private|CounterFreeze)
    (else
      (Variables|Private|SetdistanceToTarget (Private|GetDistancetoTarget))
      (CallFunction|LerptoTarget _returnvalue)
      ;[1 1 1] if there's an obstacle, head for the grapple anyway
      (if (and (Variables|Default|GetuseAbility) (> _returnvalue 0.0))
        (CallFunction|SetDirection (Variables|Default|GettargetLocation))))))

(fn StartTimeOut
  (params (scale :type Float%20%28double-precision%29))
  (if (not (Variables|Public|Getfreeze))
    (Variables|Private|SetcounterStopTimeOut (+ (Variables|Private|GetcounterStopTimeOut) (Class|TimeDefaults|GetWorldDeltaRealTimeSeconds)))
    (if (and (>= (Variables|Private|GetcounterStopTimeOut) (Variables|Private|GettimeToStopTimeOut)) (not (Variables|Private|GetstartTimeLineTimeOut)))
      (Components|Timeline|PlayfromStart (Variables|TimeLine|GettimeLineTimeoutObjectComponent))
      (Variables|Private|SetstartTimeLineTimeOut true)
      (Audio|Components|Audio|Stop (Variables|TimeLine|GettimeLineStartTimeOutObjectComponent))
      (Variables|Private|SetcounterStopTimeOut 0.0))))