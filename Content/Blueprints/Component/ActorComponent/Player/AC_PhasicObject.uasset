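; Actor component that makes its owner phase in and out of solidity with the global time scale.
; On BeginPlay it caches the owner's primitive component and collision setting, applies the current TimeSlippage scale, and binds to time scale changes.
; ToggleCollision disables collision and shows the secondary material whenever time scale differs from normal, otherwise restoring the cached collision and primary material.
; An Inverted flag reverses this, so the object is non-solid at normal speed.
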(event `self.ReceiveBeginPlay`
  (set `self.PrimitiveComponentRef` (`Actor.GetComponentByClass` (`self.GetOwner`) "/Script/Engine.PrimitiveComponent"))
  (set `self.DefaultCollisionPreset` (`PrimitiveComponent.GetCollisionEnabled` (`self.PrimitiveComponentRef`)))
  (`self.ToggleCollision` (`TimeSlippage.GetGlobalTimeScale` (`self.timeSlippage`)))
  (add `self.OnTimeScaleChangedEvent` (`|CreateDelegate` :!event `ToggleCollision`)))

(fn `ToggleCollision`
  (params (newScale :type "Float (single-precision)"))
  (bind _returnvalue (select `bool` (`self.bInverted`) :`false` (!= newScale 1.0) :`true` (== newScale 1.0)))
  (`PrimitiveComponent.SetCollisionEnabled` (`self.PrimitiveComponentRef`) (select `bool` _returnvalue :`false` (`self.DefaultCollisionPreset`) :`true` "NoCollision"))
  (`PrimitiveComponent.SetMaterial` (`self.PrimitiveComponentRef`) 0 (select `bool` _returnvalue :`false` (`self.PrimaryMaterial`) :`true` (`self.SecondaryMaterial`))))