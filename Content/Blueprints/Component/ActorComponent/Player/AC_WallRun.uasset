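; Player component that runs wall-running on BP_WallRun actors, including jump-off, camera and audio feedback.
; Tick sphere-traces both sides while falling, then repeatedly launches the character along the wall normal crossed with up, easing gravity and refilling jumps.
; A forward-offset line trace follows wall changes; losing the wall, looking away, landing or jumping ends the run and briefly suppresses re-entry.
; A timeline yaws the camera along the wall while Tick interpolates roll tilt.
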(event Custom|Initialize
  (params (character :type BP%20Player%20Character%20Object%20Reference))
  (bind _output_get (Variables|Character|Private|SetplayerCharacter character))
  (bind _output_get_2 (Variables|Default|SetcharacterMovement (Variables|/Script/Engine.Character|GetCharacterMovement _output_get)))
  (Variables|Gravity|Private|SetdefaultGravity (Variables|/Script/Engine.CharacterMovementComponent|GetGravityScale _output_get_2))
  (bind _asbp_player_controller (Utilities|Casting|CastToBP_PlayerController (Game|GetPlayerController 0)))
  (Variables|Character|Private|SetplayerController _asbp_player_controller))

(event Custom|LandEvent
  (WallRun|Private|WallRunEnd (Variables|Settings|WallRun|Reset|GetresetTimeWallrunLand)))

(event Custom|JumpEvent
  (WallRun|Private|WallRunJump))

(event Custom|ResetDilationWallRun
  (Utilities|FlowControl|DoOnce false) ; enters at Reset
)

(event Custom|ResetWallRunSupression
  (Utilities|Time|ClearTimerbyFunctionName 0 "ResetWallRunSupression")
  (Variables|WallRun|Private|SetwallRunSupressed false))

(event Custom|ResetCameraToWall
  (Utilities|FlowControl|DoOnce false) ; enters at Reset
)

(event Custom|TimeLIneCameraToWall
  (params (scale :type Float%20%28single-precision%29))
  (bind _playercontroller (Variables|Character|Private|GetplayerController))
  (bind _returnvalue (Pawn|GetControlRotation _playercontroller :!class /Script/Engine.Controller))
  (Pawn|SetControlRotation (Variables|Character|Private|GetplayerController) (Math|Rotator|MakeRotator (.roll _returnvalue) (.pitch _returnvalue) (.yaw (Math|Rotator|Lerp(Rotator) (Variables|Default|GetstartCameraLerpRotation) (Variables|Default|GetendCameraLerpRotation) scale true)))))

(event Custom|CameraToWall
  (Utilities|FlowControl|DoOnce false
    (:Completed
      (Variables|Default|SetstartCameraLerpRotation (Pawn|GetControlRotation (Variables|Character|Private|GetplayerController) :!class /Script/Engine.Controller))
      (Variables|Default|SetendCameraLerpRotation (Math|Rotator|FindLookatRotation (Math|Vector|VectorZero) (* (Math|Vector|CrossProduct (Variables|WallRun|Private|GetwallRunNormal) "0.000000,0.000000,1.000000") (Variables|WallRun|Private|GetwallRunDirection_))))
      (Components|Timeline|SetPlayRate (Variables|Default|Gettimeline) (/ 1.0 (Variables|Settings|Camera|GetspeedAnimationCameraToWall)))
      (Components|Timeline|PlayfromStart (Variables|Default|Gettimeline)))))

(event Custom|AddDilationWallRun
  (Utilities|FlowControl|DoOnce false
    (:Completed
      (Default|AddDilation (Variables|Character|Private|GetplayerController) (Variables|/Game/Blueprints/Characters/BP_PlayerCharacter.BP_PlayerCharacter_C|GetaddDilationWallRun (Variables|Character|Private|GetplayerCharacter))))))

(event EventBeginPlay
  (EventDispatchers|BindEventtoOnTimelineUpdate (delegate Custom|TimeLIneCameraToWall)))

(event EventTick
  (params (DeltaSeconds :type Float%20%28single-precision%29))
  (Camera|Private|CameraTick)
  (if (not (Variables|WallRun|Private|GetwallRunSupressed))
    (WallRun|Private|WallRunUpdate)))

(fn WallRunUpdate
  (bind _playercontroller (Variables|Character|Private|GetplayerController))
  (bind _returnvalue (Transformation|GetActorForwardVector _playercontroller))
  (if (Variables|WallRun|Public|GetwallRunning)
    (WallRun|Private|LaunchCharactertoWall (Variables|WallRun|Private|GetwallRunDirection_))
    (Variables|WallRun|Private|SetstockWallRunNormal (Variables|WallRun|Private|GetwallRunNormal))
    (Variables|/Script/Engine.CharacterMovementComponent|SetGravityScale (Variables|Default|GetcharacterMovement) (Math|Interpolation|FInterpTo (Variables|/Script/Engine.CharacterMovementComponent|GetGravityScale (Variables|Default|GetcharacterMovement)) (Variables|Settings|WallRun|Gravity|GetwallRunTargetGravity) (Utilities|Time|GetWorldDeltaSeconds) 1e+01))
    (Utilities|FlowControl|Sequence
      (:then_0
        (Variables|Default|SetcounterCheckWallRunEnd (+ (Variables|Default|GetcounterCheckWallRunEnd) (Variables|/Script/Skyrunner.TimeSlippageModifier|GetlocalManagedDeltaTime (Variables|/Game/Blueprints/Characters/BP_PlayerCharacter.BP_PlayerCharacter_C|GetTimeSlippageModifier (Variables|Character|Private|GetplayerCharacter)))))
        (if (>= (Variables|Default|GetcounterCheckWallRunEnd) (+ (Variables|Settings|Camera|GetspeedAnimationCameraToWall) (Variables|Settings|WallRun|Detection|GettimeToDetectIfWallRunEnd)))
          (if (> (Class|KismetMathLibrary|DegAcos (Math|Vector|DotProduct (Math|Vector|MakeVector (.x _returnvalue) (.y _returnvalue) 0.0) (Math|Vector|MakeVector (.x (Variables|WallRun|Private|GetwallRunNormal)) (.y (Variables|WallRun|Private|GetwallRunNormal)) 0.0))) (Variables|Settings|WallRun|Detection|GetangleToEndWallRun))
            (WallRun|Private|WallRunEnd (Variables|Settings|WallRun|Reset|GetresetTimeWallRunEnd)))))
      (:then_1
        ;[1 1 1] Detection if there is a wall in front of him
        (bind (_outhit _returnvalue_2) (Collision|LineTraceByChannel (+ (Transformation|GetActorLocation (Variables|Character|Private|GetplayerCharacter)) (* (Math|Vector|CrossProduct (Variables|WallRun|Private|GetwallRunNormal) (Math|Vector|MakeVector 0.0 0.0 1.0)) (* (Variables|WallRun|Private|GetwallRunDirection_) (Variables|Settings|WallRun|Detection|GetforwardRaycastWallRunLengthDetection)))) (+ (+ (Transformation|GetActorLocation (Variables|Character|Private|GetplayerCharacter)) (* (Math|Vector|CrossProduct (Variables|WallRun|Private|GetwallRunNormal) (Math|Vector|MakeVector 0.0 0.0 1.0)) (* (Variables|WallRun|Private|GetwallRunDirection_) (Variables|Settings|WallRun|Detection|GetforwardRaycastWallRunLengthDetection)))) (* (Math|Vector|NegateVector (Variables|WallRun|Private|GetwallRunNormal)) (Variables|Settings|WallRun|Detection|GetrightRaycastWallRunLengthDetection))) "TraceTypeQuery1" false 0 "ForDuration" true "(R=1.000000,G=0.000000,B=0.000000,A=1.000000)" "(R=0.000000,G=0.000000,B=0.000000,A=1.000000)"))
        (if _returnvalue_2
          (if (Utilities|Operators|NotEqual(!=) (.impactnormal _outhit) (Variables|WallRun|Private|GetwallRunNormal) 0.0)
            (Variables|WallRun|Private|SetwallRunNormal (.impactnormal _outhit))
            (Variables|Default|SetcounterCheckWallRunEnd 0.0))
          (else
            (WallRun|Private|WallRunEnd (Variables|Settings|WallRun|Reset|GetresetTimeWallRunEnd))))))
    (else
      (bind _onwall (WallRun|Private|WallRunMovement (Transformation|GetActorLocation (Variables|Character|Private|GetplayerCharacter)) (.right (Utilities|WallRundEndVector)) "0, 0, 0" -1.0))
      (if _onwall
        (bind _output_get (Variables|WallRun|Public|SetwallRunning true))
        (Variables|WallRun|Private|SetwallRunningR _output_get)
        (Variables|WallRun|Private|SetwallRunningL false)
        (Variables|WallRun|Private|SetwallRunDirection_ -1.0)
        (elif (Variables|WallRun|Private|GetwallRunningR)
          (WallRun|Private|WallRunEnd (Variables|Settings|WallRun|Reset|GetresetTimeWallRunEnd))
          (else
            (bind _onwall_2 (WallRun|Private|WallRunMovement (Transformation|GetActorLocation (Variables|Character|Private|GetplayerCharacter)) (.left (Utilities|WallRundEndVector)) "0, 0, 0" 1.0))
            (if _onwall_2
              (bind _output_get_2 (Variables|WallRun|Public|SetwallRunning true))
              (Variables|WallRun|Private|SetwallRunningL _output_get_2)
              (Variables|WallRun|Private|SetwallRunningR false)
              (Variables|WallRun|Private|SetwallRunDirection_ 1.0))))))))

(fn WallRunMovement
  (params (startRaycast :type Vector) (endRightRaycast :type Vector) (endLeftRaycast :type Vector) (wallRunDirection :type Float%20%28double-precision%29))
  (bind (_hitnormal _validwallvector) (Utilities|DetectionCanWallRun startRaycast endRightRaycast wallRunDirection)
    (:True
      (if (and _validwallvector (Default|GetIsFalling (Variables|Character|Private|GetplayerController)))
        (Variables|WallRun|Private|SetwallRunNormal _hitnormal)
        (Default|ResetDash (Variables|/Game/Blueprints/Characters/BP_PlayerCharacter.BP_PlayerCharacter_C|GetDash (Variables|Character|Private|GetplayerCharacter)))
        (return true)
        (else
          (return false))))
    (:false
      (return false))))

(fn WallRunEnd
  (params (resetTime :type Float%20%28double-precision%29))
  (if (Variables|WallRun|Public|GetwallRunning)
    (Variables|WallRun|Public|SetwallRunning false)
    (Variables|WallRun|Private|SetwallRunningR false)
    (Variables|WallRun|Private|SetwallRunningL false)
    (Variables|/Script/Engine.CharacterMovementComponent|SetGravityScale (Variables|Default|GetcharacterMovement) (Variables|Gravity|Private|GetdefaultGravity))
    (WallRun|Private|SupressWallrun resetTime)
    ;[0 1 0.2431] Stop sound wallRun
    (Class|AkGameplayStatics|SetRTPCValue "/Game/WwiseAudio/Game_Parameters/Default_Work_Unit/RTPC_PlayerMovement.RTPC_PlayerMovement" 4.5)
    (CallFunction|ResetCameratoWall)
    (CallFunction|ResetDilationWallRun)
    (Variables|Default|SetcounterCheckWallRunEnd 0.0)))

(fn SupressWallrun
  (params (delay :type Float%20%28double-precision%29))
  (Variables|WallRun|Private|SetwallRunSupressed true)
  (Utilities|Time|SetTimerbyFunctionName 0 "ResetWallRunSupression" delay))

(fn CameraTick
  (if (Variables|WallRun|Private|GetwallRunningL)
    (Camera|Private|CameraTilt (Variables|Settings|Camera||GetvalueCameraTilt))
    (Class|AkGameplayStatics|SetRTPCValue "/Game/WwiseAudio/Game_Parameters/Default_Work_Unit/RTPC_PlayerMovement.RTPC_PlayerMovement" 3.5 :!label _label)
    (elif (Variables|WallRun|Private|GetwallRunningR)
      (Camera|Private|CameraTilt (* (Variables|Settings|Camera||GetvalueCameraTilt) -1.0))
      (goto _label)
      (else
        (Camera|Private|CameraTilt 0.0)))))

(fn CameraTilt
  (params (targetRoll :type Float%20%28double-precision%29))
  (bind _playercharacter (Variables|Character|Private|GetplayerCharacter))
  (bind _speedanimationcameratilt (Variables|Settings|Camera|GetspeedAnimationCameraTilt))
  (bind _playercontroller (Variables|Character|Private|GetplayerController))
  (bind _returnvalue (Pawn|GetControlRotation _playercontroller :!class /Script/Engine.Controller))
  (bind _timeslippagemodifier (Variables|/Game/Blueprints/Characters/BP_PlayerCharacter.BP_PlayerCharacter_C|GetTimeSlippageModifier _playercharacter))
  (bind (_roll _pitch _yaw) (Math|Rotator|BreakRotator _returnvalue))
  (bind _localmanageddeltatime (Variables|/Script/Skyrunner.TimeSlippageModifier|GetlocalManagedDeltaTime _timeslippagemodifier))
  (bind _returnvalue_2 (Math|Interpolation|RInterpTo _returnvalue (Math|Rotator|MakeRotator targetRoll _pitch _yaw) _localmanageddeltatime _speedanimationcameratilt))
  (Pawn|SetControlRotation (Variables|Character|Private|GetplayerController) (Math|Rotator|MakeRotator (.roll _returnvalue_2) (.pitch _returnvalue_2) (.yaw _returnvalue_2))))

(fn WallRunJump
  (bind _wallrunnormal (Variables|WallRun|Private|GetwallRunNormal))
  (if (Variables|WallRun|Public|GetwallRunning)
    (WallRun|Private|WallRunEnd (Variables|Settings|WallRun|Reset|GetresetTimeWallRunJump))
    (Character|LaunchCharacter (Variables|Character|Private|GetplayerCharacter) (Math|Vector|MakeVector (|({D19FCD3F-489E-D8E6-1FBF-E1B0E97A1E86}*XwallRunNormal) (.x _wallrunnormal)) (|({D19FCD3F-489E-D8E6-1FBF-E1B0E97A1E86}*YwallRunNormal) (.y _wallrunnormal)) (Variables|Settings|WallRun|Speed|GetwallRunJumpHeight)) false true)))

(fn GetRightVectorPlayerCharacter
  (params (lengthRightVector :type Float%20%28double-precision%29))
  (return (* (Transformation|GetActorRightVector (Variables|Character|Private|GetplayerCharacter)) lengthRightVector)))

(fn AssociateVectorPlayer
  (params (lengthRightVector :type Float%20%28double-precision%29))
  (return (+ (Transformation|GetActorLocation (Variables|Character|Private|GetplayerCharacter)) (Character|Direction|Private|GetRightVectorPlayerCharacter lengthRightVector))))

(fn LaunchCharactertoWall
  (params (wallRunDirection :type Float%20%28double-precision%29))
  (if (Utilities|Operators|NotEqual(!=) (Variables|WallRun|Private|GetstockWallRunNormal) (Variables|WallRun|Private|GetwallRunNormal) 0.0)
    (CallFunction|ResetCameratoWall))
  (Character|LaunchCharacter (Variables|Character|Private|GetplayerCharacter) (WallRun|Private|VectorWallDirection wallRunDirection) true (not (Variables|Settings|WallRun|Gravity|GetwallRunGravity)))
  (Variables|/Game/Blueprints/Controller/BP_PlayerController.BP_PlayerController_C|SetnbJump (Variables|Character|Private|GetplayerController) (Variables|/Game/Blueprints/Controller/BP_PlayerController.BP_PlayerController_C|GetmaxJump (Variables|Character|Private|GetplayerController)))
  ;[0 1 0.2431] Launch Sound WallRun
  (Class|AkGameplayStatics|PostEvent)
  (Variables|WallRun|Private|SetwallRunDirection_ wallRunDirection)
  (CallFunction|CameratoWall)
  (CallFunction|AddDilationWallRun))

(fn VectorWallDirection
  (params (wallRunDirection :type Float%20%28double-precision%29))
  (return (* (Math|Vector|CrossProduct (Variables|WallRun|Private|GetwallRunNormal) (Math|Vector|VectorUp)) (* (Variables|Settings|WallRun|Speed|GetwallRunSpeed) wallRunDirection))))