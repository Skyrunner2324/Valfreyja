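; Player actor component that propels its owning character toward a target location as an ability.
; It caches the normalized direction to the target, then sets CharacterMovement velocity along it, blending speed between minimum and launch values by a clamped ratio.
; The ability stops when that ratio reaches zero.
; When the timeline ends, it also stops, sweeps the character onto the target and leaves it moving at minimum speed.
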(fn `ApplyVelocity`
  (params (Velocity :type "Vector Structure"))
  (set `MovementComponent.Velocity` Velocity (`Character.CharacterMovement` (`self.ownerCharacter`))))

(fn `EndTimeLine`
  (`self.StopAbility`)
  (`Actor.K2_SetActorLocation` (`self.ownerCharacter`) (`self.targetLocation`) true false)
  (set `MovementComponent.Velocity` (`self.GetEndVelocity`) (`Character.CharacterMovement` (`self.ownerCharacter`))))

(fn `GetEndVelocity`
  (returns (ReturnValue :type "Vector Structure"))
  (return (* (`self.directionToTarget`) (`self.minSpeed`))))

(fn `LerpToTarget`
  (params (ratio :type "Float (double-precision)"))
  (bind _returnvalue (`KismetMathLibrary.FClamp` ratio))
  (if (`self.useAbility`)
    (set `self.speed` (`KismetMathLibrary.Lerp` (`self.minSpeed`) (`self.speedLaunch`) _returnvalue))
    (if (<= _returnvalue 0.0)
      (`self.StopAbility`)
      (else
        (`self.ApplyVelocity` (* (`self.directionToTarget`) (`self.speed`)))))))

(fn `SetDirection`
  (params (targetLocation :type "Vector Structure"))
  (set `self.directionToTarget` (`KismetMathLibrary.Normal` (- targetLocation (`Actor.K2_GetActorLocation` (`self.ownerCharacter`))))))