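; Player ability component that handles crouching and a momentum slide, triggered on use or on landing with crouch held.
; Sliding sets max speed, lowers or swaps ground friction and braking, then each tick adds slope-based impulse, caps speed and stops when too slow.
; Looping timers interpolate capsule and camera height using time-slippage delta, and a capsule trace delays standing until there is room.
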(event `self.Init_`
  ;[1 1 1] Init
  (`parent.Init_`)
  (`self.SetCharacterValue`)
  (`self.SetBaseValue`))

(event `self.ReceiveTick`
  (params (DeltaSeconds :type "Float (single-precision)"))
  ;[1 1 1] Check Can Stand
  (`|ExecutionSequence`
    (:`then_0`
      (if (`self.checkCanStand`)
        (`self.CanStand`
          (:`CanStand`
            (`self.StartUnCrouch`)
            (set `self.checkCanStand` false)))))
    (:`then_1`
      ;[1 1 1] Slide Loop
      (if (`self.isSliding`)
        (`self.SlideLoop`)))))

(fn `BaseStartCrouchFunction`
  (params (Event :type Delegate) (walkSpeed :type "Float (double-precision)"))
  (`KismetSystemLibrary.K2_ClearAndInvalidateTimerHandle` (`self.timerHandleCrouch`))
  (`self.SetActualCrouchValue` (`local.walkSpeed`))
  (bind _returnvalue (`KismetSystemLibrary.K2_SetTimerDelegate` (`local.Event`) (`GameplayStatics.GetWorldDeltaSeconds`) true))
  (set `self.timerHandleCrouch` _returnvalue)
  (return))

(fn `CalculateAngleBetweenSlideDirectionAndForward`
  (returns (angleBetweenSlopeDirectionAndForward :type "Float (double-precision)"))
  (bind (_returnvalue_x _returnvalue_y) (`KismetMathLibrary.BreakVector` (`Actor.GetActorForwardVector` (`self.ownerCharacter`))))
  (bind (_normalizevector_x _normalizevector_y) (`KismetMathLibrary.BreakVector2D` (`self.Normalize2dVector` (`KismetMathLibrary.MakeVector2D` _returnvalue_x _returnvalue_y))))
  (bind (_returnvalue_x_2 _returnvalue_y_2) (`KismetMathLibrary.BreakVector` (`KismetMathLibrary.SelectVector` (`self.startSlideDirection`) (`self.SlopeDirectionCalculation` (`self.floorNormal`)) (== (`self.floorNormal`) (0.0 0.0 1.0) :`ErrorTolerance` 0.0001))))
  (bind (_normalizevector_x_2 _normalizevector_y_2) (`KismetMathLibrary.BreakVector2D` (`self.Normalize2dVector` (`KismetMathLibrary.MakeVector2D` _returnvalue_x_2 _returnvalue_y_2))))
  (return (`KismetMathLibrary.DegAcos` (`KismetMathLibrary.DotProduct2D` (`KismetMathLibrary.MakeVector2D` _normalizevector_x_2 _normalizevector_y_2) (`KismetMathLibrary.MakeVector2D` _normalizevector_x _normalizevector_y)))))

(fn `CalculateSlideVelocity`
  (params (floorNormal :type "Vector Structure"))
  (returns (velocityFloorInfluence :type "Vector Structure"))
  (return (* (`self.SlopeDirectionCalculation` (`local.floorNormal`)) (`self.SlopeAngleCalculation` (`local.floorNormal`)))))

(fn `CancelSlide`
  (`self.SetParameterSlide` (`self.baseGroundFriction`) (`self.baseBrakingDecelerationWalking`))
  (`KismetSystemLibrary.K2_SetTimer` null "ResetCanSlide" (`self.delayBetweenSlide`))
  (set `self.useAbility` false)
  (set `/Game/Blueprints/Characters/BP_PlayerCharacter.stateFOV` "NewEnumerator2" (`self.playerCharacter`))
  (set `self.isSliding` false))

(fn `CanUseAbility`
  (returns (canUseAbility :type Boolean))
  (return (`parent.CanUseAbility`)))

(fn `CheckCanClearTimerHandler`
  (params (targetCameraPosition :type "Float (double-precision)") (targetCapsuleHalfHeight :type "Float (double-precision)"))
  (if (and (`KismetMathLibrary.NearlyEqual_FloatFloat` (`self.actualPostionCamera`) (`local.targetCameraPosition`) 0.01) (`KismetMathLibrary.NearlyEqual_FloatFloat` (`self.actualCapsuleHalfHeight`) (`local.targetCapsuleHalfHeight`) 0.01))
    (`KismetSystemLibrary.K2_ClearAndInvalidateTimerHandle` (`self.timerHandleCrouch`))))

(fn `CheckSlideAtLand`
  (if (`self.keyHoldCrouch?`)
    (`self.TriggerAbility`)))

(fn `CheckSlideGoTooFast`
  (if (> (`KismetMathLibrary.VSize` (`Actor.GetVelocity` (`self.playerCharacter`))) (`self.maxSpeedSlide`))
    (set `MovementComponent.Velocity` (* (`KismetMathLibrary.Normal` (`Actor.GetVelocity` (`self.playerCharacter`))) (`self.maxSpeedSlide`)) (`self.playerCharaterMovement`))))

(fn `CheckSlideGoTooSlowly`
  (if (`self.GoToSlowly?`)
    (`self.StopAbility`)))

(fn `Crouch`
  (`self.LerpCrouchPosition` (`self.crouchHalfHeightCapsule`) (`self.crouchCameraPosition`)))

(fn `GoToSlowly?`
  (returns (stopSlide :type Boolean))
  (return (< (`KismetMathLibrary.VSize` (`Actor.GetVelocity` (`self.playerCharacter`))) (`self.minSpeedSlide`))))

(fn `LandEvent`
  (`KismetSystemLibrary.K2_SetTimer` null "CheckSlideAtLand" 0.01))

(fn `LerpCrouchPosition`
  (params (targetCapsuleHalfHeight :type "Float (double-precision)") (targetCameraPosition :type "Float (double-precision)"))
  (bind (_relativelocation_x _relativelocation_y) (`KismetMathLibrary.BreakVector` (`SceneComponent.RelativeLocation` (`self.playerCharacterCamera`))))
  ;[1 1 1] Lerp Capsule half height
  (set `self.actualCapsuleHalfHeight` (`KismetMathLibrary.FInterpTo` (`self.actualCapsuleHalfHeight`) (`local.targetCapsuleHalfHeight`) (`TimeSlippageModifier.localManagedDeltaTime` (`self.timeSlippageModifier`)) (`self.speedLerpCrouch`)))
  (`CapsuleComponent.SetCapsuleHalfHeight` (`self.playerCharacterCapsuleComponent`) (`self.actualCapsuleHalfHeight`) true)
  ;[1 1 1] Lerp Camera Position
  (set `self.actualPostionCamera` (`KismetMathLibrary.FInterpTo` (`self.actualPostionCamera`) (`local.targetCameraPosition`) (`TimeSlippageModifier.localManagedDeltaTime` (`self.timeSlippageModifier`)) (`self.speedLerpCrouch`)))
  (`SceneComponent.K2_SetRelativeLocation` (`self.playerCharacterCamera`) (`KismetMathLibrary.MakeVector` _relativelocation_x _relativelocation_y (`self.actualPostionCamera`)) false false)
  (`self.CheckCanClearTimerHandler` (`local.targetCameraPosition`) (`local.targetCapsuleHalfHeight`)))

(fn `Normalize2dVector`
  (params (vector :type "Vector2D Structure"))
  (returns (normalizeVector :type "Vector2D Structure"))
  (return (`KismetMathLibrary.Normal2D` (`KismetMathLibrary.MakeVector2D` vector_X vector_Y))))

(fn `ResetCanSlide`
  (set `self.canSlide` true))

(fn `ResetCrouchPosition`
  (params (targetCapsuleHalfHeight :type "Float (double-precision)") (targetCameraPosition :type "Float (double-precision)"))
  (bind (_relativelocation_x _relativelocation_y) (`KismetMathLibrary.BreakVector` (`SceneComponent.RelativeLocation` (`self.playerCharacterCamera`))))
  ;[1 1 1] Lerp Capsule half height
  (set `self.actualCapsuleHalfHeight` (`local.targetCapsuleHalfHeight`))
  (`CapsuleComponent.SetCapsuleHalfHeight` (`self.playerCharacterCapsuleComponent`) (`self.actualCapsuleHalfHeight`) true)
  ;[1 1 1] Lerp Camera Position
  (set `self.actualPostionCamera` (`local.targetCameraPosition`))
  (`SceneComponent.K2_SetRelativeLocation` (`self.playerCharacterCamera`) (`KismetMathLibrary.MakeVector` _relativelocation_x _relativelocation_y (`self.actualPostionCamera`)) false false))

(fn `RotateSlideVelocity`
  (locals (rotationVectorDirection :type "Rotator Structure"))
  ;[1 1 1] Rotation Calcul
  (set `local.rotationVectorDirection` (`KismetMathLibrary.MakeRotator` 0.0 0.0 (* (`self.forceStrafe`) (* (`/Game/Blueprints/Controller/BP_PlayerController.turn_angle` (`self.playerController`)) (`KismetMathLibrary.SelectInt` 1 -1 (<= (`self.CalculateAngleBetweenSlideDirectionAndForward`) 90.0))) (`TimeSlippageModifier.localManagedDeltaTime` (`/Game/Blueprints/Characters/BP_PlayerCharacter.TimeSlippageModifier` (`self.playerCharacter`))))))
  ;[1 1 1] Set velocity with rotation
  (set `MovementComponent.Velocity` (`KismetMathLibrary.GreaterGreater_VectorRotator` (`Actor.GetVelocity` (`self.ownerCharacter`)) (`local.rotationVectorDirection`)) (`Character.CharacterMovement` (`self.ownerCharacter`))))

(fn `SetActualCrouchValue`
  (params (walkSpeed :type "Float (double-precision)"))
  (bind (_relativelocation_x _relativelocation_y _relativelocation_z) (`KismetMathLibrary.BreakVector` (`SceneComponent.RelativeLocation` (`self.playerCharacterCamera`))))
  (set `self.actualCapsuleHalfHeight` (`CapsuleComponent.CapsuleHalfHeight` (`self.playerCharacterCapsuleComponent`)))
  (set `self.actualPostionCamera` _relativelocation_z)
  (set `CharacterMovementComponent.MaxWalkSpeed` (`local.walkSpeed`) (`self.playerCharaterMovement`)))

(fn `SetBaseValue`
  (bind (_relativelocation_x _relativelocation_y _relativelocation_z) (`KismetMathLibrary.BreakVector` (`SceneComponent.RelativeLocation` (`self.playerCharacterCamera`))))
  (set `self.baseGroundFriction` (`CharacterMovementComponent.GroundFriction` (`self.playerCharaterMovement`)))
  (set `self.baseBrakingDecelerationWalking` (`CharacterMovementComponent.BrakingDecelerationWalking` (`self.playerCharaterMovement`)))
  (set `self.baseHalfHeightCapsule` (`CapsuleComponent.GetScaledCapsuleHalfHeight` (`self.playerCharacterCapsuleComponent`)))
  (set `self.baseCameraZPosition` _relativelocation_z)
  (set `self.baseWalkSpeed` (`CharacterMovementComponent.MaxWalkSpeed` (`self.playerCharaterMovement`))))

(fn `SetCharacterValue`
  (set `self.playerCharaterMovement` (`Character.CharacterMovement` (`self.playerCharacter`)))
  (set `self.playerCharacterCapsuleComponent` (`Character.CapsuleComponent` (`self.playerCharacter`)))
  (set `self.playerCharacterCamera` (`/Game/Blueprints/Characters/BP_PlayerCharacter.FirstPersonCamera` (`self.playerCharacter`)))
  (set `self.timeSlippageModifier` (`/Game/Blueprints/Characters/BP_PlayerCharacter.TimeSlippageModifier` (`self.playerCharacter`))))

(fn `SetParameterSlide`
  (params (groundFriction :type "Float (single-precision)") (brakingDecelerationWalking :type "Float (single-precision)"))
  (set `CharacterMovementComponent.GroundFriction` groundFriction (`Character.CharacterMovement` (`self.ownerCharacter`)))
  (set `CharacterMovementComponent.BrakingDecelerationWalking` (`local.brakingDecelerationWalking`) (`Character.CharacterMovement` (`self.ownerCharacter`))))

(fn `SlideLoop`
  (bind (_currentfloor_bblockinghit _currentfloor_bwalkablefloor _currentfloor_blinetrace _currentfloor_floordist _currentfloor_linedist _currentfloor_hitresult) (break `FindFloorResult` (`CharacterMovementComponent.CurrentFloor` (`self.playerCharaterMovement`))))
  (bind (_bblockinghit _binitialoverlap _time _distance _location _impactpoint _normal) (`GameplayStatics.BreakHitResult` _currentfloor_hitresult))
  ;[1 1 1] Slide Loop
  ;;[1 1 1] Add slide velocity depending on the slope angle
  (if (`self.useAbility`)
    (if (!= _normal (`self.floorNormal`) :`ErrorTolerance` 0.001)
      (set `self.startSlideDirection` (`KismetMathLibrary.Normal` (`Actor.GetVelocity` (`self.ownerCharacter`))))
      (set `self.floorNormal` _normal))
    (`CharacterMovementComponent.AddImpulse` (`self.playerCharaterMovement`) (* (`self.CalculateSlideVelocity` (`self.floorNormal`)) (`TimeSlippageModifier.localManagedDeltaTime` (`/Game/Blueprints/Characters/BP_PlayerCharacter.TimeSlippageModifier` (`self.playerCharacter`)))) false)
    (`|ExecutionSequence`
      (:`then_0`
        (`self.CheckSlideGoTooFast`))
      (:`then_1`
        (`self.CheckSlideGoTooSlowly`)))))

(fn `SlopeAngleCalculation`
  (params (floorNormal :type "Vector Structure"))
  (returns (ReturnValue :type "Float (double-precision)"))
  (return (* (`KismetMathLibrary.FClamp` (- 1.0 (`KismetMathLibrary.Dot_VectorVector` (`local.floorNormal`) (`KismetMathLibrary.Vector_Up`)))) (`self.floorInfluenceWhenSlide`))))

(fn `SlopeDirectionCalculation`
  (params (floorNormal :type "Vector Structure"))
  (returns (slopeDirection :type "Vector Structure"))
  (return (`KismetMathLibrary.Normal` (`KismetMathLibrary.Cross_VectorVector` (`local.floorNormal`) (`KismetMathLibrary.Cross_VectorVector` (`local.floorNormal`) (`KismetMathLibrary.Vector_Up`))))))

(fn `StartCrouch`
  (`self.BaseStartCrouchFunction` (`|CreateDelegate` :!event `Crouch`) (`self.crouchWalkSpeed`)))

(fn `StartSlide`
  (set `self.canSlide` false)
  (set `self.startSlideDirection` (`Actor.GetActorForwardVector` (`self.playerCharacter`)))
  (set `MovementComponent.Velocity` (* (`self.startSlideDirection`) (`self.maxSpeedSlide`)) (`self.playerCharaterMovement`))
  (`self.SetParameterSlide` (`self.slideGroundFriction`) (`self.slideBrakingDecelerationWalking`))
  (set `self.isSliding` true))

(fn `StartUnCrouch`
  (`self.BaseStartCrouchFunction` (`|CreateDelegate` :!event `UnCrouch`) (`self.baseWalkSpeed`)))

(fn `StopAbility`
  (bind _useability (`self.useAbility`))
  (set `self.keyHoldCrouch?` false)
  (`KismetSystemLibrary.PrintString` (`KismetStringLibrary.Concat_StrStr` "Use ability: " (`KismetStringLibrary.Conv_BoolToString` _useability)))
  (if _useability
    (`parent.StopAbility`)
    (`self.CancelSlide`)
    (`PlayerCameraManager.StopCameraShake` (`GameplayStatics.GetPlayerCameraManager` 0) (`self.cameraShake`) true)
    (`self.CanStand`
      (:`CanStand`
        (`self.StartUnCrouch`))
      (:`CantStand`
        (set `self.checkCanStand` true)))))

(fn `TriggerAbility`
  (if (`self.CanUseAbility`)
    (`parent.TriggerAbility`)
    (`self.StartCrouch`)
    (`self.CheckCanSlide`
      (:`True`
        (`self.StartSlide`)
        (bind _returnvalue (`PlayerCameraManager.StartCameraShake` :`self` (`GameplayStatics.GetPlayerCameraManager` 0) :`ShakeClass` "/Game/Feedbacks/ScrenShake/SCR_Slide.SCR_Slide_C" :`PlaySpace` "World"))
        (set `self.cameraShake` _returnvalue)))))

(fn `UnCrouch`
  (`self.LerpCrouchPosition` (`self.baseHalfHeightCapsule`) (`self.baseCameraZPosition`)))