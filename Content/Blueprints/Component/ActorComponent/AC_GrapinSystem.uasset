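; Actor component that gives the player a grapple, flinging the character toward the current grapple point.
; On the grapple input, a check requires that ActualGrapplePoint is valid and was recently rendered.
; It then computes a projectile toss velocity to that point, launches the character with it and posts a Wwise sound.
; An alternative spline-path grapple using a predicted arc and zero gravity is present but disconnected.
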(event `self.ReceiveBeginPlay`
  (`KismetSystemLibrary.Delay` 0.0)
  (set `self.splineGrapple` (`/Game/Blueprints/Characters/BP_PlayerCharacter.SplineGrapple` (`self.playerCharacter`))))

(event `EnhancedInput|/Game/Inputs/Actions/IA_UseGrapin`
  (params (ActionValue :type Boolean) (ElapsedSeconds :type "Float (double-precision)") (TriggeredSeconds :type "Float (double-precision)") (InputAction :type "InputAction Object Reference" :default "/Game/Inputs/Actions/IA_UseGrapin.IA_UseGrapin"))
  (:`Triggered`
    (`self.canUseGrapple`
      (:`CanGrapin`
        (bind _tossvelocity (`GameplayStatics.BlueprintSuggestProjectileVelocity` (`Actor.K2_GetActorLocation` (`self.playerCharacter`)) (`Actor.K2_GetActorLocation` (`self.actualGrapplePoint`)) (`self.speedLaunch`) 0.0 "DoNotTrace"))
        (`Character.LaunchCharacter` (`self.playerCharacter`) _tossvelocity true true)
        ;[0 1 0.2423] Grapple Sound
        (`AkGameplayStatics.PostEvent` "/Game/WwiseAudio/Events/Game/Grap/game_grap_shot.game_grap_shot")))))