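; Actor component that adds wall running, wall jumps and camera tilt to the player character, set up through Initialize.
; A looping timer traces right, then left, for runnable walls while falling, launching the character along the wall (normal cross up) and easing gravity toward a target.
; Landing, jumping or losing the wall restores gravity and briefly suppresses wall running; jumps push off along the normal.
; Tick interpolates control-rotation roll according to wall side.
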(event Custom|Initialize
  (params (character :type BP%20Player%20Character%20Object%20Reference))
  (bind _output_get (Variables|Character|Private|SetplayerCharacter character))
  (bind _output_get_2 (Variables|Default|SetcharacterMovement (Variables|/Script/Engine.Character|GetCharacterMovement _output_get)))
  (Variables|Gravity|Private|SetdefaultGravity (Variables|/Script/Engine.CharacterMovementComponent|GetGravityScale _output_get_2))
  (Utilities|Time|SetTimerbyEvent (delegate Custom|WallRunEventUpdate) 0.02 true)
  (bind _asbp_player_controller_ground (Utilities|Casting|CastToBP_PlayerControllerGround (Game|GetPlayerController 0)))
  (Variables|Chracter|Private|SetcharacterController _asbp_player_controller_ground))

(event Custom|LandEvent
  (WallRun|WallRunEnd (Variables|WallRun|GetresetTimeWallrunLand)))

(event Custom|JumpEvent
  (WallRun|WallRunJump))

(event Custom|WallRunEventUpdate
  (if (not (Variables|WallRun|Private|GetwallRunSupressed))
    (WallRun|WallRunUpdate)))

(event Custom|ResetWallRunSupression
  (Development|PrintString "ResetWallRunSupression")
  (Utilities|Time|ClearTimerbyFunctionName 0 "ResetWallRunSupression")
  (Variables|WallRun|Private|SetwallRunSupressed false))

(event EventTick
  (params (DeltaSeconds :type Float%20%28single-precision%29))
  (Camera|CameraTick))

(fn WallRunUpdate
  (bind (_right _left) (Utilities|WallRundEndVector))
  (bind _onwall (WallRun|WallRunMovement (Transformation|GetActorLocation (Variables|Character|Private|GetplayerCharacter)) _right _left -1.0))
  (if _onwall
    (bind _output_get (Variables|WallRun|Public|SetwallRunning true))
    (Variables|WallRun|Private|SetwallRunningR _output_get)
    (Variables|WallRun|Private|SetwallRunningL false)
    (Variables|/Script/Engine.CharacterMovementComponent|SetGravityScale (Variables|Default|GetcharacterMovement) (Math|Interpolation|FInterpTo (Variables|/Script/Engine.CharacterMovementComponent|GetGravityScale (Variables|Default|GetcharacterMovement)) (Variables|Gravity||GetwallRunTargetGravity) (Utilities|Time|GetWorldDeltaSeconds) 1e+01) :!label _label)
    (elif (Variables|WallRun|Private|GetwallRunningR)
      (WallRun|WallRunEnd 1.0)
      (else
        (bind _onwall_2 (WallRun|WallRunMovement (Transformation|GetActorLocation (Variables|Character|Private|GetplayerCharacter)) (.left (Utilities|WallRundEndVector)) "0, 0, 0" 1.0))
        (if _onwall_2
          (Variables|WallRun|Public|SetwallRunning true)
          (Variables|WallRun|Private|SetwallRunningR false)
          (Variables|WallRun|Private|SetwallRunningL true)
          (goto _label)
          (else
            (WallRun|WallRunEnd 1.0)))))))

(fn WallRunMovement
  (params (startRaycast :type Vector) (endRightRaycast :type Vector) (endLeftRaycast :type Vector) (wallRunDirection :type Float%20%28double-precision%29))
  (bind (_hitnormal _validwallvector) (Utilities|DetectionCanWallRun startRaycast endRightRaycast)
    (:True
      (if (and _validwallvector (AI|Components|NavMovement|IsFalling (Variables|Default|GetcharacterMovement)))
        (Variables|WallRun|Private|SetwallRunNormal _hitnormal)
        (CallFunction|LaunchCharactertoWall wallRunDirection)
        (return true)
        (else
          (return false))))
    (:false
      (return false))))

(fn WallRunEnd
  (params (resetTime :type Float%20%28double-precision%29))
  (if (Variables|WallRun|Public|GetwallRunning)
    (Variables|WallRun|Public|SetwallRunning false)
    (Variables|WallRun|Private|SetwallRunningR false)
    (Variables|WallRun|Private|SetwallRunningL false)
    (Variables|/Script/Engine.CharacterMovementComponent|SetGravityScale (Variables|Default|GetcharacterMovement) (Variables|Gravity|Private|GetdefaultGravity))
    (WallRun|SupressWallrun resetTime)))

(fn SupressWallrun
  (params (delay :type Float%20%28double-precision%29))
  (Variables|WallRun|Private|SetwallRunSupressed true)
  (Utilities|Time|SetTimerbyFunctionName 0 "ResetWallRunSupression" delay))

(fn CameraTick
  (if (Variables|WallRun|Private|GetwallRunningL)
    (Camera|CameraTilt (Variables|Camera|GetvalueCameraTilt))
    (elif (Variables|WallRun|Private|GetwallRunningR)
      (Camera|CameraTilt (* (Variables|Camera|GetvalueCameraTilt) -1.0))
      (else
        (Camera|CameraTilt 0.0)))))

(fn CameraTilt
  (params (targetRoll :type Float%20%28double-precision%29))
  (bind _playercharacter (Variables|Character|Private|GetplayerCharacter))
  (bind _returnvalue (Pawn|GetController _playercharacter))
  (bind _returnvalue_2 (Pawn|GetControlRotation _returnvalue :!class /Script/Engine.Controller))
  (bind (_roll _pitch _yaw) (Math|Rotator|BreakRotator _returnvalue_2))
  (Pawn|SetControlRotation (Pawn|GetController (Variables|Character|Private|GetplayerCharacter)) (Math|Interpolation|RInterpTo _returnvalue_2 (Math|Rotator|MakeRotator targetRoll _pitch _yaw) (Utilities|Time|GetWorldDeltaSeconds) (Variables|Camera|GetspeedAnimationCameraTilt))))

(fn WallRunJump
  (bind _wallrunnormal (Variables|WallRun|Private|GetwallRunNormal))
  (if (Variables|WallRun|Public|GetwallRunning)
    (WallRun|WallRunEnd (Variables|WallRun|GetresetTimeWallRunJump))
    (Character|LaunchCharacter (Variables|Character|Private|GetplayerCharacter) (Math|Vector|MakeVector (|({D19FCD3F-489E-D8E6-1FBF-E1B0E97A1E86}*XwallRunNormal) (.x _wallrunnormal)) (|({D19FCD3F-489E-D8E6-1FBF-E1B0E97A1E86}*YwallRunNormal) (.y _wallrunnormal)) (Variables|WallRun|GetwallRunJumpHeight)) false true)))

(fn GetForwardVectorPlayerCharacter
  (params (lengthForwardVector :type Float%20%28double-precision%29))
  (return (* (Transformation|GetActorForwardVector (Variables|Character|Private|GetplayerCharacter)) lengthForwardVector)))

(fn GetRightVectorPlayerCharacter
  (params (lengthRightVector :type Float%20%28double-precision%29))
  (return (* (Transformation|GetActorRightVector (Variables|Character|Private|GetplayerCharacter)) lengthRightVector)))

(fn AssociateVectorPlayer
  (params (lengthRightVector :type Float%20%28double-precision%29) (lengthForwardVector :type Float%20%28double-precision%29))
  (return (+ (Transformation|GetActorLocation (Variables|Character|Private|GetplayerCharacter)) (Character|Direction|GetRightVectorPlayerCharacter lengthRightVector) (Character|Direction|GetForwardVectorPlayerCharacter lengthForwardVector))))

(fn LaunchCharactertoWall
  (params (wallRunDirection :type Float%20%28double-precision%29))
  (Character|LaunchCharacter (Variables|Character|Private|GetplayerCharacter) (Utilities|PlayertoWallVector) false false)
  (Character|LaunchCharacter (Variables|Character|Private|GetplayerCharacter) (* (Math|Vector|CrossProduct (Variables|WallRun|Private|GetwallRunNormal) "0.000000,0.000000,1.000000") (* (Variables|WallRun|GetwallRunSpeed) wallRunDirection)) true (not (Variables|Gravity|GetwallRunGravity))))