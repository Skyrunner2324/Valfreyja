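; Actor component that gives the player character a dash ability, built on a parent ability class and triggered by IA_Dash toward the forward vector.
; It overrides parent hooks, counting time with the character's time-slippage delta to decide when to reduce speed and stop.
; Dashing is blocked during grapple use or cooldown, which restarts after a delay once the dash stops.
; A successful dash cancels snipers' shots.
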(event `self.ReceiveBeginPlay`
  (`parent.ReceiveBeginPlay`)
  (`self.SetCharacterValue`))

(event `EnhancedInput|/Game/Inputs/Actions/IA_Dash`
  (params (ActionValue :type Boolean) (ElapsedSeconds :type "Float (double-precision)") (TriggeredSeconds :type "Float (double-precision)") (InputAction :type "InputAction Object Reference" :default "/Game/Inputs/Actions/IA_Dash.IA_Dash"))
  ;[1 1 1] Dash
  (:`Started`
    (`self.TriggerAbility` (+ (`Actor.K2_GetActorLocation` (`self.playerCharacter`)) (`Actor.GetActorForwardVector` (`self.playerCharacter`))))))

(event `CoolDownDash`
  ;[1 1 1] CoolDownDash
  (`KismetSystemLibrary.Delay` (`self.delayBeforeNext`))
  (set `self.canDash` true))

(fn `CanUseAbility`
  (returns (useAbility :type Boolean))
  (return (and (`parent.CanUseAbility`) (`self.canDash`) (not (`/Game/Blueprints/Component/ActorComponent/AC_LerpToTarget.useAbility` (`/Game/Blueprints/Characters/BP_PlayerCharacter.GrappleSystem` (`self.playerCharacter`)))))))

(fn `CheckReduceSpeed`
  (returns (ReturnValue :type Boolean))
  (return (>= (`self.counterDash`) (`self.timeToReduceSpeed`))))

(fn `CheckStopAbility`
  (returns (ReturnValue :type Boolean))
  (return (>= (`self.counterDash`) (`self.timeToDash`))))

(fn `SetCharacterValue`
  (set `self.playerCharaterMovement` (`Character.CharacterMovement` (`self.playerCharacter`))))

(fn `SetValueTickUseAbility`
  (set `self.counterDash` (+ (`self.counterDash`) (`TimeSlippageModifier.localManagedDeltaTime` (`/Game/Blueprints/Characters/BP_PlayerCharacter.TimeSlippageModifier` (`self.playerCharacter`))))))

(fn `SetValueTriggerAbility`
  (params (targetLocation :type "Vector Structure"))
  (`parent.SetValueTriggerAbility` targetLocation)
  (set `self.canDash` false))

(fn `StopAbility`
  (`parent.StopAbility`)
  (set `self.counterDash` 0.0)
  (`self.CoolDownDash`))

(fn `TriggerAbility`
  (params (targetLocation :type "Vector Structure"))
  (returns (canUseAbility :type Boolean))
  (bind _canuseability (`parent.TriggerAbility` targetLocation))
  (if _canuseability
    (`|ExecutionSequence`
      (:`then_0`)
      (:`then_1`
        (`/Game/Blueprints/Characters/BP_PlayerCharacter.CancelSnipersShots` (`self.playerCharacter`)))
      (:`then_2`
        (return true)))
    (else
      (return false))))

(fn `TriggerTickAbility`
  (returns (useAbility :type Boolean))
  (return (`parent.TriggerTickAbility`)))