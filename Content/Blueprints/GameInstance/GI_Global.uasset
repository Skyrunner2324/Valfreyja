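; GI_Global is a Game Instance that holds game-wide helpers for localization, load timing and Wwise audio.
; It stores the current culture and fires a localization change dispatcher when the culture is set or a refresh is requested.
; Loading time is printed as the difference between start and end real-time samples, using only their PartialSeconds component.
; Audio wrappers load the Init bank and post an AkEvent on an actor, then set a state.
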(event `CallLocalizationUpdate`
  (`self.OnLocalizationCultureChange` (`self.currentCulture`)))

(fn `LoadInitBankGameInstance`
  (`AkGameplayStatics.LoadInitBank`))

(fn `PostEventGameInstance`
  (params (AkEvent :type "AkAudioEvent Object Reference") (Actor :type "Actor Object Reference") (StateValue :type "AkStateValue Object Reference"))
  (`AkGameplayStatics.PostEvent` AkEvent Actor)
  (`AkGameplayStatics.SetState` StateValue))

(fn `PrintLastLoadingTime`
  (`self.SaveEndLoadingTime`)
  (`KismetSystemLibrary.PrintString` (`KismetStringLibrary.BuildString_Double` "Last loading time : " "" (- (`self.EndLoadingTime`) (`self.StartLoadingTime`))) true true (struct :`G` 1.0 :`A` 1.0)))

(fn `SaveEndLoadingTime`
  (set `self.EndLoadingTime` (`.PartialSeconds` (`GameplayStatics.GetAccurateRealTime`))))

(fn `SaveStartLoadingTime`
  (set `self.StartLoadingTime` (`.PartialSeconds` (`GameplayStatics.GetAccurateRealTime`))))

(fn `SetCurrentCulture`
  (params (value :type "/Game/Blueprints/Enumerator/E_LocalizationCulture Enum" :default "NewEnumerator0"))
  (bind _output_get (set `self.currentCulture` value))
  (`self.OnLocalizationCultureChange` _output_get))