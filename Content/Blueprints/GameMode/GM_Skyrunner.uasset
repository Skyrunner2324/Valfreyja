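; Skyrunner game mode that manages the pause and death menus and the pause state for a win screen.
; BeginPlay creates both menu widgets hidden; toggle functions set game pause, input mode, button focus, Wwise state and sound, and player HUD visibility.
; ToggleWinScreen creates no win widget: it toggles pause, hides the HUD and always sets UI-only input focused on the pause widget.
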(event `self.ReceiveBeginPlay`
  (`|ExecutionSequence`
    (:`then_0`
      ;[1 1 1] create pause widget
      (bind _returnvalue (`|CreateWidget` "/Game/UI/Menu/WB_PauseMenu.WB_PauseMenu_C"))
      (`UserWidget.AddToViewport` _returnvalue 0)
      (bind _output_get (set `self.PauseWidget` _returnvalue))
      (`Widget.SetVisibility` _output_get "Hidden"))
    (:`then_1`
      ;[1 1 1] create death widget
      (bind _returnvalue_2 (`|CreateWidget` "/Game/UI/Menu/WB_DeathMenu.WB_DeathMenu_C"))
      (`UserWidget.AddToViewport` _returnvalue_2 0)
      (bind _output_get_2 (set `self.DeathWidget` _returnvalue_2))
      (`Widget.SetVisibility` _output_get_2 "Hidden"))))

(fn `ShowDeathMenu`
  (params (bVisible :type Boolean))
  (`GameplayStatics.SetGamePaused` bVisible)
  (`AkGameplayStatics.SetState` "/Game/WwiseAudio/States/Default_Work_Unit/GameStatus/GameStatus-InMenu.GameStatus-InMenu")
  (`Widget.SetVisibility` (`self.DeathWidget`) (select `bool` (`local.bVisible`) :`false` "Hidden" :`true` "Visible" :!type "ESlateVisibility Enum"))
  (if (`local.bVisible`)
    (`AkGameplayStatics.PostEvent` "/Game/WwiseAudio/Events/UI/ui_pause.ui_pause")
    (`WidgetBlueprintLibrary.SetInputMode_UIOnlyEx` (`GameplayStatics.GetPlayerController` 0) (`self.DeathWidget`))
    (`Widget.SetFocus` (`/Game/UI/Menu/WB_DeathMenu.RespawnButtonHandle` (`self.DeathWidget`)))
    (`self.ShowPlayerHUD` false)
    (else
      (`WidgetBlueprintLibrary.SetInputMode_GameOnly` (`GameplayStatics.GetPlayerController` 0))
      (`AkGameplayStatics.SetState` "/Game/WwiseAudio/States/Default_Work_Unit/GameStatus/GameStatus-InGame.GameStatus-InGame")
      (`self.ShowPlayerHUD` true))))

(fn `ShowPlayerHUD`
  (params (bVisible :type Boolean))
  (bind _asbp_player_character (cast `/Game/Blueprints/Characters/BP_PlayerCharacter` (`GameplayStatics.GetPlayerCharacter` 0)))
  (`/Game/Blueprints/HUD/BP_PlayerHUD.Show` (`/Game/Blueprints/Characters/BP_PlayerCharacter.HUD` _asbp_player_character) (select `bool` bVisible :`false` "Hidden" :`true` "Visible" :!type "ESlateVisibility Enum")))

(fn `TogglePause`
  (`GameplayStatics.SetGamePaused` (not (`GameplayStatics.IsGamePaused`)))
  (`AkGameplayStatics.SetState` "/Game/WwiseAudio/States/Default_Work_Unit/GameStatus/GameStatus-InMenu.GameStatus-InMenu")
  (`Widget.SetVisibility` (`self.PauseWidget`) (select `bool` (`GameplayStatics.IsGamePaused`) :`false` "Hidden" :`true` "Visible" :!type "ESlateVisibility Enum"))
  (if (`GameplayStatics.IsGamePaused`)
    (`AkGameplayStatics.PostEvent` "/Game/WwiseAudio/Events/UI/ui_pause.ui_pause")
    (`WidgetBlueprintLibrary.SetInputMode_UIOnlyEx` (`GameplayStatics.GetPlayerController` 0) (`self.PauseWidget`))
    (`Widget.SetFocus` (`/Game/UI/Menu/WB_PauseMenu.ResumeButtonHandle` (`self.PauseWidget`)))
    (`self.ShowPlayerHUD` false)
    (else
      (`WidgetBlueprintLibrary.SetInputMode_GameOnly` (`GameplayStatics.GetPlayerController` 0))
      (`AkGameplayStatics.SetState` "/Game/WwiseAudio/States/Default_Work_Unit/GameStatus/GameStatus-InGame.GameStatus-InGame")
      (`self.ShowPlayerHUD` true))))

(fn `ToggleWinScreen`
  (`GameplayStatics.SetGamePaused` (not (`GameplayStatics.IsGamePaused`)))
  (`AkGameplayStatics.SetState` "/Game/WwiseAudio/States/Default_Work_Unit/GameStatus/GameStatus-InMenu.GameStatus-InMenu")
  (`AkGameplayStatics.PostEvent` "/Game/WwiseAudio/Events/UI/ui_pause.ui_pause")
  (`WidgetBlueprintLibrary.SetInputMode_UIOnlyEx` (`GameplayStatics.GetPlayerController` 0) (`self.PauseWidget`))
  (bind _asbp_player_character (cast `/Game/Blueprints/Characters/BP_PlayerCharacter` (`GameplayStatics.GetPlayerCharacter` 0)))
  (`/Game/Blueprints/HUD/BP_PlayerHUD.Show` (`/Game/Blueprints/Characters/BP_PlayerCharacter.HUD` _asbp_player_character) "Hidden"))

(fn `UserConstructionScript`)