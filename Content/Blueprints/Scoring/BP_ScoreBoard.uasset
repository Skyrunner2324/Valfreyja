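; Scoreboard Blueprint that tracks combo score, checkpoint splits and time and score leaderboards for runs.
; Grapple, dash, slide and wallrun components feed points into a temporary score and multiplier, whose timeline-driven countdown pauses while rail riding, sliding or wallrunning and banks the combo on expiry.
; Checkpoints report deltas against stored times from the visible chrono widget.
; Finishing adds a time bonus, records a randomly named run and saves through GI_Global.
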(event `BindActions`
  (`KismetSystemLibrary.Delay` 0.1)
  (bind _asbp_player_character (cast `/Game/Blueprints/Characters/BP_PlayerCharacter` (`GameplayStatics.GetPlayerCharacter` 0)))
  (bind _output_get (set `self.PlayerRef` _asbp_player_character))
  (add `/Game/Blueprints/Component/ActorComponent/Player/AC_GrappleSystem.AddScore_` (`/Game/Blueprints/Characters/BP_PlayerCharacter.GrappleSystem` _output_get) (delegate `AddScore`))
  (add `/Game/Blueprints/Component/ActorComponent/Player/AC_Dash.AddScore_` (`/Game/Blueprints/Characters/BP_PlayerCharacter.Dash` _output_get) (delegate `AddScore`))
  (add `/Game/Blueprints/Component/ActorComponent/Player/AC_Slide.AddScore_` (`/Game/Blueprints/Characters/BP_PlayerCharacter.Slide` _output_get) (delegate `AddScore`))
  (add `/Game/Blueprints/Component/ActorComponent/Player/AC_WallRun.AddScore_` (`/Game/Blueprints/Characters/BP_PlayerCharacter.WallRun` _output_get) (delegate `AddScore`)))

(event `AddScore`
  (params (Value :type Integer))
  (set `self.TempScore` (+ (`self.TempScore`) Value))
  (`self.AddMultiplierProgress` Value)
  (`self.UpdateTempScore_` (`self.Multiplier`) (`self.TempScore`)))

(event `InitCheckpointArray`
  (bind _outactors (`GameplayStatics.GetAllActorsOfClass` "/Game/Blueprints/Scoring/TimeCheck.TimeCheck_C"))
  (`KismetArrayLibrary.Array_Set` (`self.CheckpointTimes`) (- (`KismetArrayLibrary.Array_Length` _outactors) 1) 0.0 true))

(event `StopMultiplier`
  (bind _multiplier (`self.Multiplier`))
  (bind _output_get (set `self.TotalScore` (+ (`self.TotalScore`) (* (`self.TempScore`) (`self.Multiplier`))) :!label _label))
  (`self.DisplayScore_` _output_get)
  (`self.UpdateMultiplierTimer_` 0.0)
  (set `self.TempScore` 0)
  (if (> _multiplier (`self.MaxMultiplier`))
    (set `self.MaxMultiplier` _multiplier))
  (set `self.Multiplier` 0)
  (set `self.MultiplierProgress` 0)
  (`self.UpdateTempScore_` (`self.Multiplier`) (`self.TempScore`))
  (`self.UpdateMultiplierProgress_` 0.0)
  (`Timeline|MultiplierProgression` :!via `Stop` :!label _label_2
    (:`Update`
      (bind _multiplierexpired (`self.UpdateMultiplierTimer`))
      (`self.UpdateMultiplierTimer_` (/ (`self.MultiplierCrtTime`) (`self.MultiplierMaxTime`)))
      (if _multiplierexpired
        (goto _label)))))

(event `DepleteMultiplier`
  (bind _multipliermaxtime (`self.MultiplierMaxTime`))
  (bind _returnvalue (+ (`self.MultiplierCrtTime`) (* 0.25 _multipliermaxtime)))
  (set `self.MultiplierCrtTime` (`KismetMathLibrary.FClamp` _returnvalue _returnvalue _multipliermaxtime))
  (goto _label_2 :!via `PlayFromStart`))

(event `StopDepleteMultiplier`
  (goto _label_2 :!via `Stop`))

(event `self.K2_OnReset`
  (`self.StopDepleteMultiplier`))

(fn `AddMultiplierProgress`
  (params (ValueToAdd :type Integer))
  (if (== (`self.Multiplier`) 0)
    (set `self.Multiplier` 1)
    (set `self.MultiplierCrtTime` (`self.MultiplierMaxTime`)))
  (bind _output_get (set `self.MultiplierProgress` (+ ValueToAdd (`self.MultiplierProgress`))))
  (if (>= _output_get (`self.MultiplierThreshold`))
    (`self.UpdateMultiplierTimer_` 1.0)
    (set `self.MultiplierProgress` 0)
    (`/Engine/EditorBlueprintResources/StandardMacros.IncrementInt` (`self.Multiplier`)
      (:`  `
        (set `self.MultiplierCrtTime` (`self.MultiplierMaxTime`))
        (`self.MultiplierUpgraded_`))))
  (`self.UpdateMultiplierProgress_` (/ (`self.MultiplierProgress`) (`self.MultiplierThreshold`)))
  (`self.DepleteMultiplier`))

(fn `CheckpointReached`
  (params (ID :type Integer) (AlreadyTriggered :type Boolean))
  (bind _checkpointtimes (`self.CheckpointTimes`))
  (bind _alreadytriggered (`local.AlreadyTriggered`))
  (bind _output (`|GetArrayItem` _checkpointtimes ID))
  (bind _time (`self.GetTime`))
  (if (== (`KismetArrayLibrary.Array_Length` _checkpointtimes) 0)
    (`self.InitCheckpointArray`))
  (if (not (== _output 0.0))
    (bind _returnvalue (- _time _output))
    (if (> _returnvalue 0.0)
      (bind _returnvalue_2 (`KismetStringLibrary.TimeSecondsToString` _returnvalue))
      (`self.GateReached_` (`KismetStringLibrary.Concat_StrStr` "+" _returnvalue_2) _alreadytriggered)
      (else
        (`self.GateReached_` _returnvalue_2 _alreadytriggered))))
  (`KismetArrayLibrary.Array_Set` _checkpointtimes ID _time true))

(fn `GenerateRunName`
  (bind _names (`self.Names`))
  (bind _output_get (set `self.RunName` (`|GetArrayItem` _names (`KismetMathLibrary.RandomInteger` (`KismetArrayLibrary.Array_Length` _names)))))
  (if (`.ReturnValue` (`BlueprintMapLibrary.Map_Find` (`self.TimeLeaderBoard`) _output_get)) :!label _label
    (set `self.RunName` (`KismetStringLibrary.Concat_StrStr` _output_get (`KismetStringLibrary.Conv_IntToString` (`KismetMathLibrary.RandomInteger` 10))))
    (goto _label)))

(fn `GetChrono`
  (returns (Chrono :type "/Game/UI/HUD/WB_Chrono Object Reference"))
  (bind _foundwidgets (`WidgetBlueprintLibrary.GetAllWidgetsOfClass` "/Game/UI/HUD/WB_Chrono.WB_Chrono_C" false))
  (for _array_element _foundwidgets
    (if (`Widget.IsVisible` _array_element)
      (return _array_element))))

(fn `GetTime`
  (returns (Time :type "Float (double-precision)"))
  (bind _chrono (`self.GetChrono`))
  (bind _chronovalue (`/Game/UI/HUD/WB_Chrono.ChronoValue` _chrono))
  (`KismetSystemLibrary.PrintString` (`KismetStringLibrary.Conv_DoubleToString` _chronovalue))
  (return _chronovalue))

(fn `ResetTemp`
  (set `self.TempScore` 0)
  (set `self.Multiplier` 1)
  (set `self.MultiplierCrtTime` 0.01))

(fn `RunFinished`
  (params (FinalTime :type "Float (double-precision) (by ref)") (bHideTutorialWhenFinished :type Boolean))
  (bind _timeleaderboard (`self.TimeLeaderBoard`))
  (bind _runname (`self.RunName`))
  (bind _finaltime (`local.FinalTime`))
  (`|ExecutionSequence`
    (:`then_0`
      (set `self.CurrentTime` FinalTime)
      (`self.GenerateRunName`)
      (set `self.TotalScore` (+ (`self.TotalScore`) (* 500000 (`KismetMathLibrary.FClamp` (- 1.0 (/ FinalTime 600))))))
      (`self.StopMultiplier`)
      (if (> _finaltime 0.0)
        (`BlueprintMapLibrary.Map_Add` _timeleaderboard _runname _finaltime)
        (`BlueprintMapLibrary.Map_Add` (`self.ScoreLeaderBoard`) _runname (`self.TotalScore`))
        (`self.SortLeaderBoards`)
        (`|ExecutionSequence`
          (:`then_0`
            (bind _values (`BlueprintMapLibrary.Map_Values` _timeleaderboard))
            (if (== (`|GetArrayItem` _values) (`local.FinalTime`))
              (bind _asgi_global (cast `/Game/Blueprints/GameInstance/GI_Global` (`GameplayStatics.GetGameInstance`)))
              (`/Game/Blueprints/GameInstance/GI_Global.SaveCheckPoints` _asgi_global)))
          (:`then_1`
            (bind _asgi_global_2 (cast `/Game/Blueprints/GameInstance/GI_Global` (`GameplayStatics.GetGameInstance`)))
            (`/Game/Blueprints/GameInstance/GI_Global.SaveScoreboard` _asgi_global_2)))))
    (:`then_1`
      (if bHideTutorialWhenFinished
        (bind _asgi_global_3 (cast `/Game/Blueprints/GameInstance/GI_Global` (`GameplayStatics.GetGameInstance`)))
        (`/Game/Blueprints/GameInstance/GI_Global.SetHideTutorial` _asgi_global_3 true)))))

(fn `SplitMaps`
  (returns (TimeKeys :type "Array of String") (TimeValues :type "Array of Float (double-precision)") (ScoreKeys :type "Array of String") (ScoreValues :type "Array of Integer") (HasValues :type Boolean))
  (bind _timeleaderboard (`self.TimeLeaderBoard`))
  (bind _scoreleaderboard (`self.ScoreLeaderBoard`))
  (if (> (`BlueprintMapLibrary.Map_Length` _timeleaderboard) 0)
    (bind _keys (`BlueprintMapLibrary.Map_Keys` _timeleaderboard))
    (bind _values (`BlueprintMapLibrary.Map_Values` _timeleaderboard))
    (bind _keys_2 (`BlueprintMapLibrary.Map_Keys` _scoreleaderboard))
    (bind _values_2 (`BlueprintMapLibrary.Map_Values` _scoreleaderboard))
    (return _keys _values _keys_2 _values_2 true)
    (else
      (return _ _ _ _ false))))

(fn `TryFindChrono`
  (bind _foundwidgets (`WidgetBlueprintLibrary.GetAllWidgetsOfClass` "/Game/UI/HUD/WB_Chrono.WB_Chrono_C" false))
  (if (> (`KismetArrayLibrary.Array_Length` _foundwidgets) 0)
    _))

(fn `UpdateMultiplierTimer`
  (returns (MultiplierExpired :type Boolean))
  (bind _playerref (`self.PlayerRef`))
  (if (not (or (`/Game/Blueprints/Characters/BP_PlayerCharacter.IsOnRail` _playerref) (`/Game/Blueprints/Component/ActorComponent/Player/AC_Slide.isSliding` (`/Game/Blueprints/Characters/BP_PlayerCharacter.Slide` _playerref)) (`/Game/Blueprints/Component/ActorComponent/Player/AC_WallRun.IsWallrunning` (`/Game/Blueprints/Characters/BP_PlayerCharacter.WallRun` _playerref))))
    (set `self.MultiplierCrtTime` (- (`self.MultiplierCrtTime`) (* (`TimeDefaults.GetWorldDeltaRealTimeSeconds`) (`self.MultiplierDepleteRate`)))))
  (return (<= (`self.MultiplierCrtTime`) 0.0)))

(fn `UserConstructionScript`)