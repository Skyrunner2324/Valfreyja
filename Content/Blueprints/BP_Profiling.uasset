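; Profiling helper actor that runs a list of console commands and shows an on-screen FPS counter.
; On BeginPlay it executes the commands, then looks up a BP_TimeSlippage actor in the map.
; If found, it creates a WB_FrameRateCounter widget and updates it each Tick with that actor's rounded Framerate.
; If missing, it prints a red warning and disables its tick.
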(event `self.ReceiveBeginPlay`
  (`self.ExecuteCommands`)
  (bind _bfound (`self.GetTimeSlippageRef`))
  (if _bfound
    (`self.CreateFrameRateWidget`)))

(event `self.ReceiveTick`
  (params (DeltaSeconds :type "Float (single-precision)"))
  (`TextBlock.SetText` (`/Game/UI/WB_FrameRateCounter.TextBlock_0` (`self.FrameRateCounter`)) (`KismetTextLibrary.Conv_StringToText` (`KismetStringLibrary.BuildString_Double` "" "" (`self.GetFrameRate` 100.0) " FPS"))))

(fn `CreateFrameRateWidget`
  (bind _returnvalue (`|CreateWidget` "/Game/UI/WB_FrameRateCounter.WB_FrameRateCounter_C"))
  (`UserWidget.AddToViewport` _returnvalue 0)
  (set `self.FrameRateCounter` _returnvalue))

(fn `ExecuteCommands`
  (for _array_element (`self.ConsoleCommands`)
    (`KismetSystemLibrary.ExecuteConsoleCommand` _array_element null)))

(fn `GetFrameRate`
  (params (FloatPrecision :type "Float (double-precision)" :default 100.0))
  (returns (ReturnValue :type "Float (double-precision)"))
  (return (/ (`KismetMathLibrary.Conv_Int64ToDouble` (`KismetMathLibrary.Round64` (* (`TimeSlippage.framerate` (`self.TimeSlippageRef`)) FloatPrecision))) FloatPrecision)))

(fn `GetTimeSlippageRef`
  (returns (bFound :type Boolean))
  (locals (bFoundRef :type Boolean :default false))
  (`|ExecutionSequence`
    (:`then_0`
      (bind _outactors (`GameplayStatics.GetAllActorsOfClass` "/Game/Blueprints/TimeManagement/BP_TimeSlippage.BP_TimeSlippage_C"))
      (bind _output (`|GetArrayItem` _outactors))
      (`/Engine/EditorBlueprintResources/StandardMacros.IsValid` _output
        (:`Is Valid`
          (set `self.TimeSlippageRef` _output)
          (`self.SetActorTickEnabled` true)
          (set `local.bFoundRef` true))
        (:`Is Not Valid`
          (`KismetSystemLibrary.PrintString` "Cannot find BP_TimeSlippage object in map, tick disabled" true true (struct :`R` 0.996 :`A` 1.0))
          (`self.SetActorTickEnabled` false))))
    (:`then_1`
      (return (`local.bFoundRef`)))))

(fn `UserConstructionScript`)