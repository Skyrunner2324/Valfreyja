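; Sound trigger box that, when the player character enters it, broadcasts a max sequence point value and switches an audio state.
; On BeginPlay it caches MaxNumberSequencePointOutsideArena from the player character, despite the asset's "inside Arena" name.
; Box overlaps by the player fire the EnterTriggerBox dispatcher with that cached value, then call SetState with StateValue.
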(event `self.ReceiveBeginPlay`
  (set `self.playerCharacter` (cast `/Game/Blueprints/Characters/BP_PlayerCharacter` (`GameplayStatics.GetPlayerCharacter` 0) :!pure true))
  (set `self.maxNumberSequencePoint` (`/Game/Blueprints/Characters/BP_PlayerCharacter.maxNumberSequencePointOutsideArena` (`self.playerCharacter`))))

(event `self.Box.OnComponentBeginOverlap`
  (params (OverlappedComponent :type "PrimitiveComponent Object Reference") (OtherActor :type "Actor Object Reference") (OtherComp :type "PrimitiveComponent Object Reference") (OtherBodyIndex :type Integer) (bFromSweep :type Boolean) (SweepResult :type "HitResult Structure (by ref)"))
  (cast `/Game/Blueprints/Characters/BP_PlayerCharacter` OtherActor)
  (`self.EnterTriggerBox` (`self.maxNumberSequencePoint`))
  (`AkGameplayStatics.SetState` (`self.State Value`)))

(fn `UserConstructionScript`)