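; Player-triggered sound box that sets up Wwise audio on entry, apparently for the Sky Alpha area.
; When an actor tagged Player overlaps it, it sets the music zone, music number, large reverb and in-game status states, then posts the main ambience play event.
; It then disables its own collision to act as a one-shot trigger, and OnReset turns collision back on to re-arm it.
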(event `self.ReceiveActorBeginOverlap`
  (params (OtherActor :type "Actor Object Reference"))
  (if (`self.ActorHasTag` OtherActor "Player")
    (`AkGameplayStatics.SetState` "/Game/WwiseAudio/States/Default_Work_Unit/Music/Music_Zone/Music_Zone-A.Music_Zone-A")
    (`AkGameplayStatics.SetState` "/Game/WwiseAudio/States/Default_Work_Unit/Music/Music_Number/Music_Number-Music__01.Music_Number-Music__01")
    (`AkGameplayStatics.SetState` "/Game/WwiseAudio/States/Default_Work_Unit/Reverb_States/Reverb_States-Large.Reverb_States-Large")
    (`AkGameplayStatics.SetState` "/Game/WwiseAudio/States/Default_Work_Unit/GameStatus/GameStatus-InGame.GameStatus-InGame")
    (`AkGameplayStatics.PostEvent` "/Game/WwiseAudio/Events/Ambience/ENV_AMB_Play_AmbienceMain.ENV_AMB_Play_AmbienceMain")
    (`self.DisableSelf`)))

(event `EnableSelf`
  (`self.SetActorEnableCollision` true))

(event `DisableSelf`
  (`self.SetActorEnableCollision` false))

(event `self.K2_OnReset`
  (`self.EnableSelf`))

(fn `UserConstructionScript`)