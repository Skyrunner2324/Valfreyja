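; BP_TutoText is a tutorial prompt actor that reveals its Widget component while the player character overlaps it and hides it when they leave.
; On BeginPlay it passes its InputAction variable to the hosted widget, which can be either WB_FTUEJump or WB_FTUEHookExecute.
; The hook widget takes that action as its first input and the grapple action IA_UseGrapin as its second.
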(event `self.ReceiveBeginPlay`
  (bind _returnvalue (`WidgetComponent.GetUserWidgetObject` (`self.Widget`)))
  (bind _aswb_ftuejump (cast `/Game/UI/InGame/WB_FTUEJump` _returnvalue)
    (:`then`
      (set `/Game/UI/InGame/WB_FTUEJump.InputAction` (`self.Input Action`) _aswb_ftuejump))
    (:`CastFailed`
      (bind _aswb_ftuehook_execute (cast `/Game/UI/InGame/WB_FTUEHookExecute` _returnvalue))
      (set `/Game/UI/InGame/WB_FTUEHookExecute.InputAction1` (`self.Input Action`) _aswb_ftuehook_execute)
      (set `/Game/UI/InGame/WB_FTUEHookExecute.InputAction2` "/Game/Inputs/Actions/IA_UseGrapin.IA_UseGrapin" _aswb_ftuehook_execute))))

(event `self.ReceiveActorBeginOverlap`
  (params (OtherActor :type "Actor Object Reference"))
  (cast `/Game/Blueprints/Characters/BP_PlayerCharacter` OtherActor)
  (`SceneComponent.SetHiddenInGame` (`self.Widget`) false false))

(event `self.ReceiveActorEndOverlap`
  (params (OtherActor :type "Actor Object Reference"))
  (cast `/Game/Blueprints/Characters/BP_PlayerCharacter` OtherActor)
  (`SceneComponent.SetHiddenInGame` (`self.Widget`) true false))

(fn `UserConstructionScript`)