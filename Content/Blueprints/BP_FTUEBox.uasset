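; BP_FTUEBox is a one-time trigger actor for the first-time user experience, holding the player in place for what appears to be a grapple tutorial.
; On player overlap it freezes the character, binds to the GrappleSystem's FTUE-complete event and switches game status to InFTUI.
; While frozen, Tick zeroes the character's movement velocity each frame.
; When the grapple system reports completion, it unfreezes, restores InGame status and marks itself completed.
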(event `self.ReceiveActorBeginOverlap`
  (params (OtherActor :type "Actor Object Reference"))
  (if (not (`self.Completed`))
    (bind _asbp_player_character (cast `/Game/Blueprints/Characters/BP_PlayerCharacter` OtherActor))
    (set `self.PlayerFrozen` true)
    (`/Engine/EditorBlueprintResources/StandardMacros.IsValid` (`self.PlayerRef`)
      (:`Is Not Valid`
        (bind _output_get (set `self.PlayerRef` _asbp_player_character))
        (add `/Game/Blueprints/Component/ActorComponent/Player/AC_GrappleSystem.FTUEComplete_` (`/Game/Blueprints/Characters/BP_PlayerCharacter.GrappleSystem` _output_get) (delegate `FTUEComplete`))
        (`AkGameplayStatics.SetState` "/Game/WwiseAudio/States/Default_Work_Unit/GameStatus/GameStatus-InFTUI.GameStatus-InFTUI")))))

(event `FTUEComplete`
  (if (not (`self.Completed`))
    (set `self.PlayerFrozen` false)
    (set `self.Completed` true)
    (`AkGameplayStatics.SetState` "/Game/WwiseAudio/States/Default_Work_Unit/GameStatus/GameStatus-InGame.GameStatus-InGame")))

(event `self.ReceiveTick`
  (params (DeltaSeconds :type "Float (single-precision)"))
  (if (`self.PlayerFrozen`)
    (set `MovementComponent.Velocity` (0.0 0.0 0.0) (`Character.CharacterMovement` (`self.PlayerRef`)))))

(fn `UserConstructionScript`)