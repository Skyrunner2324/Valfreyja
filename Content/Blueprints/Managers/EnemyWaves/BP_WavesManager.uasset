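; Arena wave manager that runs sequential enemy waves once the player enters its ArenaSize volume, updating the HUD wave indicator.
; SpawnWave spawns each enemy at the SpawnerTag spawn point with a matching ID and tags it for per-arena counting.
; EnemyManager removal events trigger the next wave at its threshold, or broadcast WavesFinished when the last is cleared.
; ResetWave clears and respawns the current wave; BaseEnemiesManager is enabled on entry only with SpawnChips.
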(event `self.ReceiveBeginPlay`
  (`|ExecutionSequence`
    (:`then_0`
      (bind _returnvalue (`GameplayStatics.GetActorOfClass` "/Game/Blueprints/Managers/BP_EnemyManager.BP_EnemyManager_C"))
      (`/Engine/EditorBlueprintResources/StandardMacros.IsValid` _returnvalue
        (:`Is Valid`
          (set `self.enemyManager` _returnvalue)
          ;[1 1 1] Loan Soluce 2
          (bind _outactors (`GameplayStatics.GetAllActorsOfClassWithTag` "/Game/Blueprints/Managers/EnemyWaves/BP_EnemySpawnPoint.BP_EnemySpawnPoint_C" (`self.SpawnerTag`)))
          (set `self.spawnPoints` _outactors))
        (:`Is Not Valid`
          (`KismetSystemLibrary.PrintString` "NO ENEMY MANAGER FOUND" true true (struct :`R` 1.0 :`G` 0.858274 :`A` 1.0) 3.0))))
    (:`then_1`
      (set `/Game/Blueprints/Component/ActorComponent/AC_BaseEnemiesManager.wavesManager` self (`self.BaseEnemies Manager`)))))

(event `self.ArenaSize.OnComponentBeginOverlap`
  (params (OverlappedComponent :type "PrimitiveComponent Object Reference") (OtherActor :type "Actor Object Reference") (OtherComp :type "PrimitiveComponent Object Reference") (OtherBodyIndex :type Integer) (bFromSweep :type Boolean) (SweepResult :type "HitResult Structure (by ref)"))
  (bind _baseenemies_manager (`self.BaseEnemies Manager`))
  (bind _waves (`self.Waves`))
  (bind _output_enemies (break `/Game/Blueprints/Managers/EnemyWaves/ST_Wave` (`|GetArrayItem` _waves)))
  (cast `/Game/Blueprints/Characters/BP_PlayerCharacter` OtherActor)
  (add `/Game/Blueprints/Managers/BP_EnemyManager.EnemyRemoved` (`self.enemyManager`) (delegate `OnEnemyRemoved`))
  (if (== (`self.currentWave`) 0)
    (`self.SpawnWave`)
    ;[1 1 1] remove ?
    (bind _output_get (set `self.WB Wave Indicator` (`/Game/UI/HUD/WB_HUD.WB_WaveIndicator` (`/Game/Blueprints/HUD/BP_PlayerHUD.hudWidget` (cast `/Game/Blueprints/HUD/BP_PlayerHUD` (`PlayerController.GetHUD` (`GameplayStatics.GetPlayerController` 0)) :!pure true)))))
    (`/Game/UI/HUD/WB_WaveIndicator.EnterArena` _output_get (`KismetArrayLibrary.Array_Length` _waves) (`BlueprintMapLibrary.Map_Length` _output_enemies))
    (set `self.isArenaOn` true)
    (if (`self.spawnChips`)
      (`/Game/Blueprints/Component/ActorComponent/AC_BaseEnemiesManager.Init` _baseenemies_manager)
      (else
        (`/Game/Blueprints/Component/ActorComponent/AC_BaseEnemiesManager.Disable` _baseenemies_manager)))
    (add `self.WaveEnemyDied` (delegate `testevent`))))

(event `testevent`
  (`KismetSystemLibrary.PrintString` "no waying"))

(event `OnEnemyRemoved`
  (params (EnemyAmount :type Integer) (EnemyTags :type Name))
  (bind _currentwave (`self.currentWave`))
  (bind _waves (`self.Waves`))
  (bind _enemycount (`/Game/Blueprints/Managers/BP_EnemyManager.GetEnemyCountWithTag` (`self.enemyManager`) (`self.SpawnerTag`)))
  (bind (_output_enemies _output_spawnthreshold) (break `/Game/Blueprints/Managers/EnemyWaves/ST_Wave` (`|GetArrayItem` _waves _currentwave)))
  (`self.IsSpawnerTagInArray` EnemyTags
    (:`Found`
      (`self.WaveEnemyDied`))
    (:`NotFound`
      _))
  (`/Game/UI/HUD/WB_WaveIndicator.SetEnemiesCount` (`self.WB Wave Indicator`) _enemycount)
  (if (>= _currentwave (`KismetArrayLibrary.Array_Length` _waves))
    (if (== _enemycount 0)
      (`self.WavesFinished`)
      (remove `/Game/Blueprints/Managers/BP_EnemyManager.EnemyRemoved` (`self.enemyManager`) (delegate `OnEnemyRemoved`))
      (set `self.isArenaOn` false)
      (`KismetSystemLibrary.PrintString` "WAVES FINISHED" true true (struct :`R` 1.0 :`G` 0.858274 :`A` 1.0) 3.0)
      (if (`self.showUI`)
        (`/Game/UI/HUD/WB_WaveIndicator.LeaveArena` (`self.WB Wave Indicator`))))
    (elif (<= _enemycount _output_spawnthreshold)
      (`self.SpawnWave`)
      (`KismetSystemLibrary.PrintString` "WAVE SPAWN" true true (struct :`R` 1.0 :`G` 0.858274 :`A` 1.0) 3.0)
      (if (`self.showUI`)
        (`/Game/UI/HUD/WB_WaveIndicator.SetWave` (`self.WB Wave Indicator`) (`self.currentWave`) _enemycount)))))

(fn `FindSpawn`
  (params (spawnID :type Integer))
  (returns (spawnPoint :type "/Game/Blueprints/Managers/EnemyWaves/BP_EnemySpawnPoint Object Reference"))
  (for _array_element (`self.spawnPoints`)
    (if (== (`/Game/Blueprints/Managers/EnemyWaves/BP_EnemySpawnPoint.ID` _array_element) spawnID)
      (return _array_element)))
  (`KismetSystemLibrary.PrintString` (`KismetStringLibrary.Concat_StrStr` "can't find spawn " (`KismetStringLibrary.Conv_IntToString` spawnID)) true true (struct :`R` 1.0 :`G` 1.0 :`A` 1.0) 3.0)
  (return null))

(fn `ResetWave`
  (bind _enemymanager (`self.enemyManager`))
  (bind _currentwave (`self.currentWave`))
  (bind _spawnertag (`self.SpawnerTag`))
  (if (`self.isArenaOn`)
    (`/Engine/EditorBlueprintResources/StandardMacros.IsValid` _enemymanager
      (:`Is Valid`
        (`/Game/Blueprints/Managers/BP_EnemyManager.ClearArenaEnemies` _enemymanager _spawnertag)
        (`/Engine/EditorBlueprintResources/StandardMacros.DecrementInt` _currentwave
          (:`  `
            (`self.SpawnWave`)
            (`/Game/UI/HUD/WB_WaveIndicator.SetWave` (`self.WB Wave Indicator` :!enabledstate Disabled) _currentwave (`/Game/Blueprints/Managers/BP_EnemyManager.GetEnemyCountWithTag` _enemymanager _spawnertag) :!enabledstate Disabled)
            (`/Game/Blueprints/Component/ActorComponent/AC_BaseEnemiesManager.Init` (`self.BaseEnemies Manager`))))))))

(fn `SpawnEnemy`
  (params (enemyID :type Integer) (waveID :type Integer))
  (bind (_value _returnvalue) (`BlueprintMapLibrary.Map_Find` (`.enemies_4_7E58626E4D6723DDDF8ABEB1D4212FE3` (break `/Game/Blueprints/Managers/EnemyWaves/ST_Wave` (`|GetArrayItem` (`self.Waves`) waveID))) enemyID))
  (if _returnvalue
    (bind _spawnpoint (`self.FindSpawn` enemyID))
    ;[0.2094 0.2094 0.2094] experimental check
    (`/Engine/EditorBlueprintResources/StandardMacros.IsValid` _spawnpoint
      (:`Is Valid`
        (bind _returnvalue_2 (`|SpawnActorFromClass` _value (`self.GetTransform` _spawnpoint) "AlwaysSpawn" "MultiplyWithRoot" null 2.0 null))
        (`KismetArrayLibrary.Array_AddUnique` (`Actor.Tags` _returnvalue_2) (`self.SpawnerTag`))
        (`KismetSystemLibrary.PrintString` (`KismetStringLibrary.Concat_StrStr` "SPAWNED " (`KismetSystemLibrary.GetDisplayName` _returnvalue_2)) true true (struct :`R` 1.0 :`G` 0.858274 :`A` 1.0))
        (return)))
    (else
      (`KismetSystemLibrary.PrintString` (`KismetStringLibrary.Concat_StrStr` "cant find enemy " (`KismetStringLibrary.Conv_IntToString` enemyID)) true true (struct :`R` 1.0 :`G` 1.0 :`A` 1.0) 3.0))))

(fn `SpawnWave`
  (bind _currentwave (`self.currentWave`))
  (bind _output_enemies (break `/Game/Blueprints/Managers/EnemyWaves/ST_Wave` (`|GetArrayItem` (`self.Waves`) _currentwave)))
  (`self.SpawningWave` _currentwave)
  (bind _keys (`BlueprintMapLibrary.Map_Keys` _output_enemies))
  (for _array_element _keys
    (`self.SpawnEnemy` _array_element _currentwave))
  (`/Engine/EditorBlueprintResources/StandardMacros.IncrementInt` _currentwave))

(fn `UserConstructionScript`)