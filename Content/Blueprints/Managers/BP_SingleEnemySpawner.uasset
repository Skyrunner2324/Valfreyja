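; BP_SingleEnemySpawner is a spawner actor that keeps a single enemy at its location, respawning it after death.
; A timeline started on BeginPlay acts as the delay; when it finishes with no valid enemy, SpawnEnemy creates the configured type and fire rate, with shield reset on stun end enabled.
; It binds RespawnSingleEnemy to that enemy's damage-component death event, which restarts the timeline.
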(event `self.ReceiveBeginPlay`
  (`TimelineComponent.PlayFromStart` (`self.SpawnTimeline`)))

(event `RespawnSingleEnemy`
  (`TimelineComponent.PlayFromStart` (`self.SpawnTimeline`)))

(fn `SpawnEnemy`
  (bind _returnvalue (`|SpawnActorFromClass` (`self.EnemyType`) (`self.GetTransform`) "AlwaysSpawn" "MultiplyWithRoot" null true (`self.SpawnedEnemyFireRate`) null))
  (set `self.SpawnedEnemyRef` _returnvalue))

(fn `UserConstructionScript`)