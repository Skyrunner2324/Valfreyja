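; Enemy manager Blueprint that tracks registered enemies and signals when all have been removed.
; NewEnemy adds to the Enemies list and RemoveEnemy removes from it, calling the EnemiesCleared dispatcher when the count reaches zero.
; BeginPlay binds debug print handlers to EnemiesCleared and EnemyRemoved, though nothing here calls EnemyRemoved.
; Additions and successful removals also print the enemy's name.
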(event `self.ReceiveBeginPlay`
  (add `self.EnemiesCleared` (delegate `Debug_EnemiesCleared`))
  (add `self.EnemyRemoved` (delegate `Debug_EnemyRemoved`)))

(event `Debug_EnemiesCleared`
  (`KismetSystemLibrary.PrintString` "Enemies cleared" true true (struct :`R` 1.0 :`G` 0.664964 :`A` 1.0) 3.0))

(event `Debug_EnemyRemoved` :!signature `self.EnemyRemoved`
  (params (EnemyAmount :type Integer))
  (`KismetSystemLibrary.PrintString` (`KismetStringLibrary.Concat_StrStr` "Enemies left: " (`KismetStringLibrary.Conv_IntToString` EnemyAmount))))

(fn `GetEnemyCount`
  (returns (Count :type Integer))
  (return (`KismetArrayLibrary.Array_Length` (`self.enemies`))))

(fn `NewEnemy`
  (params (Enemy :type "BaseEnemy Object Reference"))
  (`KismetArrayLibrary.Array_Add` (`self.enemies`) Enemy)
  (`KismetSystemLibrary.PrintString` (`KismetStringLibrary.Concat_StrStr` (`KismetSystemLibrary.GetDisplayName` Enemy) " added")))

(fn `RemoveEnemy`
  (params (Enemy :type "BaseEnemy Object Reference"))
  (bind _returnvalue (`KismetArrayLibrary.Array_RemoveItem` (`self.enemies`) Enemy))
  (if _returnvalue
    (`KismetSystemLibrary.PrintString` (`KismetStringLibrary.Concat_StrStr` (`KismetSystemLibrary.GetDisplayName` Enemy) " removed"))
    (if (== (`self.GetEnemyCount`) 0)
      (`self.EnemiesCleared`))))

(fn `UserConstructionScript`)