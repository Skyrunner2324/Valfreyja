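; BP_EntropyBullet is a special projectile that can be reset when the player lines their aim up with it.
; On BeginPlay it stores the player character's forward vector, a stand-in for the unfinished shooter lookup.
; Aiming requires matching that direction and having the bullet near screen center, checked every tick to swap its material.
; A debug key calls ResetActor while aimed; velocity-reversal logic is left disconnected.
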(event EventBeginPlay
  (|CallParentFunction)
  (Variables|Default|SetDirection (CallFunction|GetShooterForward))
  (Input|EnableInput (Game|GetPlayerController 0)))

(event Collision|EventActorBeginOverlap
  (params (OtherActor :type Actor%20Object%20Reference)))

(event EventTick
  (params (DeltaSeconds :type Float%20%28single-precision%29))
  (|CallParentFunction DeltaSeconds)
  (if (CallFunction|IsAimingatBullet)
    (Rendering|Material|SetMaterial (Variables|Default|GetStaticMesh) 0 "/AnimationSharing/AnimSharingRed.AnimSharingRed")
    (else
      (Rendering|Material|SetMaterial (Variables|Default|GetStaticMesh) 0 "/Game/Materials/Instance_Material/LD_Blockout/MI_LDYellow.MI_LDYellow"))))

(event EventOnReset)

(event Input|KeyboardEvents|DebugKeyN
  (params (Key :type Key%20Structure :default "None") (ActionValue :type Input%20Action%20Value%20Structure))
  (:Pressed
    (if (CallFunction|IsAimingatBullet)
      (Class|BulletBase|ResetActor))))

(fn ConstructionScript
  (|CallParentFunction))

(fn GetShooterForward
  (return (Transformation|GetActorForwardVector (Game|GetPlayerCharacter 0))))

(fn IsAimingatBullet
  (return (and (Utilities|Operators|EqualEqual (CallFunction|GetShooterForward) (Variables|Default|GetDirection) (Variables|Default|GetDirectionMatchTolerance)) (Utilities|Operators|EqualEqual (.ScreenPosition (Class|GameplayStatics|ProjectWorldtoScreen (Game|GetPlayerController 0) (Transformation|GetActorLocation) true)) (* (Viewport|GetViewportSize) 0.5) (Variables|Default|GetCenterTolerance)))))