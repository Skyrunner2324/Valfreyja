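; BP_ExplosionRayon is a timed spherical explosion area, filed with the player bullet Blueprints.
; Collision stays off from BeginPlay until Init sets the sphere radius and lifespan and enables query and physics collision.
; Init also draws a debug sphere and scales the Gfx component to the radius.
; Init zeroes damage on the DoDamageTrap and DoDamageEnemie components, leaving its enemy and trap damage inputs unused.
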(event EventBeginPlay
  (Collision|SetCollisionEnabled (Variables|Default|GetSphere) "NoCollision"))

(fn ConstructionScript)

(fn Init
  (params (sphereRadius :type Float%20%28single-precision%29) (timeExplosionRemains :type Float%20%28single-precision%29) (damageEnemi :type Integer) (damageTrap :type Integer))
  (bind _returnvalue (|((radius*1.275000)/baseRadius) sphereRadius 64.0))
  (Components|Sphere|SetSphereRadius (Variables|Default|GetSphere) sphereRadius true)
  (Actor|SetLifeSpan timeExplosionRemains)
  (Variables|/Game/Blueprints/Component/ActorComponent/Damage/AC_DoDamage.AC_DoDamage_C|Setdamage (Variables|Default|GetDoDamageTrap) 0.0)
  (Variables|/Game/Blueprints/Component/ActorComponent/Damage/AC_DoDamage.AC_DoDamage_C|Setdamage (Variables|Default|GetDoDamageEnemie) 0.0)
  (Collision|SetCollisionEnabled (Variables|Default|GetSphere) "QueryAndPhysics")
  ;[1 1 1] visuals
  (Utilities|FlowControl|Sequence
    (:then_0
      (Rendering|Debug|DrawDebugSphere (Transformation|GetActorLocation) (Variables|/Script/Engine.SphereComponent|GetSphereRadius (Variables|Default|GetSphere)) 12 "(R=1.000000,G=1.000000,B=1.000000,A=1.000000)" (Actor|GetLifeSpan) 2.0))
    (:then_1
      (Transformation|SetWorldScale3D (Variables|Default|Getgfx) (Math|Vector|MakeVector _returnvalue _returnvalue _returnvalue)))))