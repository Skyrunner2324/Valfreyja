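; Grenade launcher player bullet that spawns an area explosion when it hits something.
; On Hit it runs the parent logic, then spawns a BP_ExplosionRayon at its location and initialises it with radius, lingering time and separate enemy and trap damage.
; Init stores those explosion values on the bullet so they can be handed to the explosion actor.
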(event `self.ReceiveHit`
  (params (MyComp :type "PrimitiveComponent Object Reference") (Other :type "Actor Object Reference") (OtherComp :type "PrimitiveComponent Object Reference") (bSelfMoved :type Boolean) (HitLocation :type "Vector Structure") (HitNormal :type "Vector Structure") (NormalImpulse :type "Vector Structure") (Hit :type "HitResult Structure (by ref)"))
  (`parent.ReceiveHit` MyComp Other OtherComp bSelfMoved HitLocation HitNormal NormalImpulse Hit)
  (bind _returnvalue (`|SpawnActorFromClass` "/Game/Blueprints/Projectiles/Bullet/PlayerBullet/BP_ExplosionRayon.BP_ExplosionRayon_C" (`KismetMathLibrary.MakeTransform` (`self.K2_GetActorLocation`)) "Undefined" "MultiplyWithRoot" null null))
  (`/Game/Blueprints/Projectiles/Bullet/PlayerBullet/BP_ExplosionRayon.Init` _returnvalue (`self.explosionRayon`) (`self.timeExplosionRemains`) (`self.damagePerHitEnemie`) (`self.damagePerHitTrap`)))

(fn `Init`
  (params (explosionRayon :type "Float (double-precision)") (timeExplosionRemains :type "Float (double-precision)") (damagePerHitEnemie :type Integer) (damagePerHitTrap :type Integer))
  (set `self.explosionRayon` explosionRayon)
  (set `self.timeExplosionRemains` timeExplosionRemains)
  (set `self.damagePerHitEnemie` damagePerHitEnemie)
  (set `self.damagePerHitTrap` damagePerHitTrap))

(fn `UserConstructionScript`
  (`parent.UserConstructionScript`))