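; Base pooled bullet actor that handles impacts, lifetime and response to the game's time dilation.
; Time scale changes set the TimeSlippageModifier's local target from the player controller's dilation state, with no and weak dilation sharing one value.
; Hits play Wwise audio, optionally return the bullet to its pool, and spawn a physics field to break Chaos meshes.
; Lifetime counts in locally dilated delta time unless infinite.
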(event `self.TimeSlippageModifier.OnTimeScaleChangedEvent`
  (params (newScale :type "Float (single-precision)"))
  (`self.ChangeTargetLocalTimeScale` newScale))

(event `self.ReceiveBeginPlay`
  (bind _asbp_player_controller (cast `/Game/Blueprints/Controller/BP_PlayerController` (`GameplayStatics.GetPlayerController` 0)))
  (set `self.controllerRef` _asbp_player_controller)
  (`self.ChangeTargetLocalTimeScale` 0.0))

(event `self.ReceiveHit`
  (params (MyComp :type "PrimitiveComponent Object Reference") (Other :type "Actor Object Reference") (OtherComp :type "PrimitiveComponent Object Reference") (bSelfMoved :type Boolean) (HitLocation :type "Vector Structure") (HitNormal :type "Vector Structure") (NormalImpulse :type "Vector Structure") (Hit :type "HitResult Structure (by ref)"))
  ;[0.05035 0.05035 0.05035] Hit enemies
  (`|ExecutionSequence`
    (:`then_0`
      ;;[0 1 0.2423] Bullet Hit at Location
      (`AkGameplayStatics.SpawnAkComponentAtLocation` (`self.ImpactSound`) HitLocation (struct) true)
      (if (`self.bDestroyable`)
        (`self.DestroyBullet`)))
    (:`then_1`
      (`self.ImpactDestructibleObjects` HitLocation))))

(event `self.FellOutOfWorldImpl`
  (params (dmgType :type "DamageType Object Reference"))
  (`self.DestroyBullet`))

(event `DestroyBullet`
  (set `self.counterForDestroy` 0.0)
  ;[1 1 1] Remove pool object
  (`PoolObject.OnDeath` (`self.PoolObject`) self))

(event `self.ReceiveTick`
  (params (DeltaSeconds :type "Float (single-precision)"))
  (if (not (`self.bInfiniteLifeSpan`))
    (bind _output_get (set `self.counterForDestroy` (+ (`self.counterForDestroy`) (`TimeSlippageModifier.localManagedDeltaTime` (`self.TimeSlippageModifier`)))))
    (if (>= _output_get (`self.timeToDestroy`))
      (`self.DestroyBullet`))))

(fn `ChangeTargetLocalTimeScale`
  (params (newScale :type "Float (single-precision)"))
  (`/Game/Blueprints/Libraries/MacroLibraries/BPML_TimeManagementActor.DilationTypeDo` (`self.controllerRef`)
    (:`NoDilation`
      (set `TimeSlippageModifier.localTimeScaleTarget` (`self.WeakDilationTargetLocalTimeScale`) (`self.TimeSlippageModifier`) :!label _label))
    (:`WeakDilation`
      (goto _label))
    (:`StrongDilation`
      (set `TimeSlippageModifier.localTimeScaleTarget` (`self.StrongDilationTargetLocalTimeScale`) (`self.TimeSlippageModifier`)))))

(fn `ImpactDestructibleObjects`
  (params (ImpactPos :type "Vector Structure"))
  ;[1 1 1] Create physics field then activate it to cause impact on Chaos meshes
  (bind _returnvalue (`|SpawnActorFromClass` "/Engine/EditorResources/FieldNodes/FS_MasterField.FS_MasterField_C" (`KismetMathLibrary.Conv_VectorToTransform` ImpactPos) "Undefined" "MultiplyWithRoot" null null))
  (set `/Engine/EditorResources/FieldNodes/FS_MasterField.ActivationType` "NewEnumerator4" _returnvalue)
  (`/Engine/EditorResources/FieldNodes/FS_MasterField.CE_Trigger` _returnvalue))

(fn `InitBullet`
  (`PrimitiveComponent.SetCollisionEnabled` (`self.CollisionComponent`) "QueryOnly"))

(fn `PlayerHit`
  (params (hitLocation :type "Vector Structure"))
  (set `self.counterForDestroy` 0.0)
  (`PoolObject.OnDeath` (`self.PoolObject`) self)
  (`self.ImpactDestructibleObjects` (`local.hitLocation`)))

(fn `RemoveBullet`
  (set `self.counterForDestroy` 0.0)
  (`PoolObject.OnDeath` (`self.PoolObject`) self))

(fn `UserConstructionScript`)