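; Enemy explosion actor that deals damage within a sphere for a limited lifetime.
; Collision stays off from BeginPlay until Init sets the radius, lifespan and damage, then enables query-only overlaps.
; Overlapping actors with an AC_TakeDamage component take damage from ACDoDamagePlayer, with damage mercy requested.
; Init also scales Gfx to match the radius and draws a debug sphere for the explosion's lifetime.
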(event OnComponentBeginOverlap(Sphere)
  (params (OverlappedComponent :type Primitive%20Component%20Object%20Reference) (OtherActor :type Actor%20Object%20Reference) (OtherComp :type Primitive%20Component%20Object%20Reference) (OtherBodyIndex :type Integer) (bFromSweep :type Boolean) (SweepResult :type Hit%20Result%20Structure%20%28by%20ref%29))
  (bind _returnvalue (Actor|GetComponentbyClass OtherActor "/Game/Blueprints/Component/ActorComponent/Damage/AC_TakeDamage.AC_TakeDamage_C"))
  (Utilities|IsValid _returnvalue
    (:Is%20Valid
      (Default|TakeDamage _returnvalue (Variables|Default|GetAC_DoDamagePlayer) 0.0 true))))

(event EventBeginPlay
  (Collision|SetCollisionEnabled (Variables|Default|GetSphere) "NoCollision"))

(fn ConstructionScript)

(fn Init
  (params (sphereRadius :type Float%20%28single-precision%29) (timeExplosionRemains :type Float%20%28single-precision%29) (damagePlayer :type Float%20%28double-precision%29))
  (bind _returnvalue (|((radius*1.275000)/baseRadius) sphereRadius 64.0))
  (Components|Sphere|SetSphereRadius (Variables|Default|GetSphere) sphereRadius true)
  (Actor|SetLifeSpan timeExplosionRemains)
  (Variables|/Game/Blueprints/Component/ActorComponent/Damage/AC_DoDamage.AC_DoDamage_C|Setdamage (Variables|Default|GetAC_DoDamagePlayer) damagePlayer)
  (Collision|SetCollisionEnabled (Variables|Default|GetSphere) "QueryOnly")
  ;[1 1 1] visuals
  (Utilities|FlowControl|Sequence
    (:then_0
      (Rendering|Debug|DrawDebugSphere (Transformation|GetActorLocation) (Variables|/Script/Engine.SphereComponent|GetSphereRadius (Variables|Default|GetSphere)) 12 "(R=1.000000,G=1.000000,B=1.000000,A=1.000000)" (Actor|GetLifeSpan) 2.0))
    (:then_1
      (Transformation|SetWorldScale3D (Variables|Default|Getgfx) (Math|Vector|MakeVector _returnvalue _returnvalue _returnvalue)))))