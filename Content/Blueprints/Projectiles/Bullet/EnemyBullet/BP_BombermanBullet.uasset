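; BP_BombermanBullet is a pooled enemy bullet that acts as a timed bomb, exploding after a delay.
; InitBullet arms the timer, and Tick counts it down with TimeSlippageModifier's managed delta time.
; At zero it spawns BP_EnemyExplosion with its collision radius, duration and player damage, then returns to the pool.
; The construction script scales a disk mesh to the blast radius, and the empty PlayerHit leaves contact without effect.
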(event `self.ReceiveBeginPlay`
  (`parent.ReceiveBeginPlay`))

(event `self.ReceiveTick`
  (params (DeltaSeconds :type "Float (single-precision)"))
  (`parent.ReceiveTick` DeltaSeconds)
  (if (<= (`self.DelayTimer`) 0.0)
    (set `self.counterForDestroy` 0.0)
    (bind _returnvalue (`|SpawnActorFromClass` "/Game/Blueprints/Projectiles/Bullet/EnemyBullet/BP_EnemyExplosion.BP_EnemyExplosion_C" (`KismetMathLibrary.MakeTransform` (`self.K2_GetActorLocation`)) "Undefined" "MultiplyWithRoot" null null))
    (`/Game/Blueprints/Projectiles/Bullet/EnemyBullet/BP_EnemyExplosion.Init` _returnvalue (`SphereComponent.SphereRadius` (`self.CollisionComponent`)) (`self.ExplosionDuration`) (`/Game/Blueprints/Component/ActorComponent/Damage/AC_DoDamage.damage` (`self.AC_DoDamagePlayer`)))
    ;[1 1 1] Remove pool object
    (`PoolObject.OnDeath` (`self.PoolObject`) self)
    (else
      (set `self.DelayTimer` (- (`self.DelayTimer`) (`TimeSlippageModifier.localManagedDeltaTime` (`self.TimeSlippageModifier`)))))))

(fn `InitBullet`
  (`parent.InitBullet`)
  (set `self.DelayTimer` (`self.ExplosionDelay`)))

(fn `PlayerHit`
  (params (hitLocation :type "Vector Structure")))

(fn `UserConstructionScript`
  (bind _returnvalue (/ (`SphereComponent.SphereRadius` (`self.CollisionComponent`)) 100.0))
  (`parent.UserConstructionScript`)
  (`SceneComponent.SetRelativeScale3D` (`self.StaticMesh`) (`KismetMathLibrary.MakeVector` 0.25 _returnvalue _returnvalue)) ; Collision component used to set explosion scale\nTarget mesh is a disk with a radius of 100 at scale 1\nmesh scaled to explosion = explosion scale / 100
)