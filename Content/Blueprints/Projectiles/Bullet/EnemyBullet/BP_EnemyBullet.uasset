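; Enemy bullet projectile Blueprint that extends a parent bullet class with a trail effect.
; On init it runs the parent logic, then caches its normalized travel direction from the custom projectile movement velocity and its start position.
; It spawns the trail actor there, gives it a lifespan of TimeToDestroy and snaps it to the collision component.
; Hit handling and construction defer entirely to the parent.
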(event `self.ReceiveHit`
  (params (MyComp :type "PrimitiveComponent Object Reference") (Other :type "Actor Object Reference") (OtherComp :type "PrimitiveComponent Object Reference") (bSelfMoved :type Boolean) (HitLocation :type "Vector Structure") (HitNormal :type "Vector Structure") (NormalImpulse :type "Vector Structure") (Hit :type "HitResult Structure (by ref)"))
  (`parent.ReceiveHit` MyComp Other OtherComp bSelfMoved HitLocation HitNormal NormalImpulse Hit))

(fn `InitBullet`
  (bind (_returnvalue_location _returnvalue_rotation _returnvalue_scale) (`KismetMathLibrary.BreakTransform` (`self.GetTransform`)))
  (`parent.InitBullet`)
  (set `self.direction` (`KismetMathLibrary.Normal` (`MovementComponent.Velocity` (`self.CustomProjectileMovement`))))
  (set `self.startPosition` (`self.K2_GetActorLocation`))
  (bind _returnvalue (`|SpawnActorFromClass` (`self.classTrailBullet`) (`KismetMathLibrary.MakeTransform` (`self.startPosition`) _returnvalue_rotation _returnvalue_scale) "Undefined" "MultiplyWithRoot" null null))
  (bind _output_get (set `self.fxBullet` _returnvalue))
  (`self.SetLifeSpan` _output_get (`self.timeToDestroy`))
  (`self.K2_AttachToComponent` (`self.fxBullet`) (`self.CollisionComponent`) "None" "SnapToTarget" "SnapToTarget" "SnapToTarget" true))

(fn `UserConstructionScript`
  (`parent.UserConstructionScript`))