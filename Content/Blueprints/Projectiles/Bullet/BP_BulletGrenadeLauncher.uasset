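; Grenade launcher projectile Blueprint that turns its impact into a timed explosion.
; Init stores the explosion radius and remaining time.
; On Hit, it spawns a BP_ExplosionRayon at its own location, passing those values and its per-hit damage, then destroys itself.
; It also calls ImpactDestructibleObjects and plays the Wwise weapon impact sound at the hit location.
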(event `self.ReceiveHit`
  (params (MyComp :type "PrimitiveComponent Object Reference") (Other :type "Actor Object Reference") (OtherComp :type "PrimitiveComponent Object Reference") (bSelfMoved :type Boolean) (HitLocation :type "Vector Structure") (HitNormal :type "Vector Structure") (NormalImpulse :type "Vector Structure") (Hit :type "HitResult Structure (by ref)"))
  (bind _returnvalue (`|SpawnActorFromClass` "/Game/Blueprints/Projectiles/Bullet/BP_ExplosionRayon.BP_ExplosionRayon_C" (`KismetMathLibrary.MakeTransform` (`self.K2_GetActorLocation`)) "Undefined" "MultiplyWithRoot" null null))
  (`/Game/Blueprints/Projectiles/Bullet/BP_ExplosionRayon.Init` _returnvalue (`self.explosionRayon`) (`self.timeExplosionRemains`) (`self.damagePerHit`))
  (`self.K2_DestroyActor`)
  (`self.ImpactDestructibleObjects` HitLocation)
  ;[0 1 0.2423] Bullet Hit at Location
  (`AkGameplayStatics.SpawnAkComponentAtLocation` "/Game/WwiseAudio/Events/Game/Weapon/weapon_impact.weapon_impact" HitLocation (struct) true))

(fn `Init`
  (params (explosionRayon :type "Float (double-precision)") (timeExplosionRemains :type "Float (double-precision)"))
  (set `self.explosionRayon` explosionRayon)
  (set `self.timeExplosionRemains` timeExplosionRemains))

(fn `UserConstructionScript`
  (`parent.UserConstructionScript`))