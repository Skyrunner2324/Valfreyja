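; BP_BombermanBullet_old is a pooled bullet that explodes after a delay once it hits something.
; Hit plays an impact sound, arms DelayTimer and impacts destructible objects, while the PlayerHit override does nothing.
; Tick counts down using time-slippage delta time, then spawns and initializes a BP_EnemyExplosion and releases the bullet through PoolObject.
; InitBullet resets the timer to a large negative sentinel, preventing detonation before impact.
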(event `self.ReceiveBeginPlay`
  (`parent.ReceiveBeginPlay`))

(event `self.ReceiveTick`
  (params (DeltaSeconds :type "Float (single-precision)"))
  (bind _delaytimer (`self.DelayTimer`))
  (`parent.ReceiveTick` DeltaSeconds)
  (if (> _delaytimer -100.0)
    (if (<= _delaytimer 0.0)
      (set `self.counterForDestroy` 0.0)
      (bind _returnvalue (`|SpawnActorFromClass` "/Game/Blueprints/Projectiles/Bullet/BP_EnemyExplosion.BP_EnemyExplosion_C" (`KismetMathLibrary.MakeTransform` (`self.K2_GetActorLocation`)) "Undefined" "MultiplyWithRoot" null null))
      (`/Game/Blueprints/Projectiles/Bullet/BP_EnemyExplosion.Init` _returnvalue (`self.ExplosionRadius`) (`self.ExplosionDuration`) (`self.Damage Player`))
      ;[1 1 1] Remove pool object
      (`PoolObject.OnDeath` (`self.PoolObject`) self)
      (else
        (set `self.DelayTimer` (- (`self.DelayTimer`) (`TimeSlippageModifier.localManagedDeltaTime` (`self.TimeSlippageModifier`))))))))

(event `self.ReceiveHit`
  (params (MyComp :type "PrimitiveComponent Object Reference") (Other :type "Actor Object Reference") (OtherComp :type "PrimitiveComponent Object Reference") (bSelfMoved :type Boolean) (HitLocation :type "Vector Structure") (HitNormal :type "Vector Structure") (NormalImpulse :type "Vector Structure") (Hit :type "HitResult Structure (by ref)"))
  (`|ExecutionSequence`
    (:`then_0`
      ;[0 1 0.2423] Bullet Hit at Location
      (`AkGameplayStatics.SpawnAkComponentAtLocation` (`self.ImpactSound`) HitLocation (struct) true)
      (set `self.DelayTimer` (`self.ExplosionDelay`)))
    (:`then_1`
      (`self.ImpactDestructibleObjects` HitLocation))))

(fn `InitBullet`
  (`parent.InitBullet`)
  (set `self.DelayTimer` -10000.0) ; Needs to be defaulted under -100\nto prevent instant explosion
)

(fn `PlayerHit`
  (params (hitLocation :type "Vector Structure")))

(fn `UserConstructionScript`
  (`parent.UserConstructionScript`))