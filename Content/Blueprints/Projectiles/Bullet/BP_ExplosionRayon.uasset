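; BP_ExplosionRayon is a short-lived explosion area actor that carries separate damage values for enemies and traps.
; Its sphere collision is disabled on BeginPlay until Init sets the radius, lifespan and the damage on the DoDamageEnemie and DoDamageTrap components.
; Init then draws a debug sphere for the lifespan and enables query and physics collision.
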(event `self.ReceiveBeginPlay`
  (`PrimitiveComponent.SetCollisionEnabled` (`self.Sphere`) "NoCollision"))

(fn `Init`
  (params (sphereRadius :type "Float (single-precision)") (timeExplosionRemains :type "Float (single-precision)") (damageEnemi :type Integer) (damageTrap :type Integer))
  (`SphereComponent.SetSphereRadius` (`self.Sphere`) (`local.sphereRadius`) true)
  (`self.SetLifeSpan` (`local.timeExplosionRemains`))
  (set `/Game/Blueprints/Component/ActorComponent/Damage/AC_DoDamage.damage` (`local.damageTrap`) (`self.DoDamageTrap`))
  (set `/Game/Blueprints/Component/ActorComponent/Damage/AC_DoDamage.damage` (`local.damageEnemi`) (`self.DoDamageEnemie`))
  (`KismetSystemLibrary.DrawDebugSphere` (`self.K2_GetActorLocation`) (`SphereComponent.SphereRadius` (`self.Sphere`)) 12 (struct :`R` 1.0 :`G` 1.0 :`B` 1.0 :`A` 1.0) (`self.GetLifeSpan`) 2.0)
  (`PrimitiveComponent.SetCollisionEnabled` (`self.Sphere`) "QueryAndPhysics"))

(fn `UserConstructionScript`)