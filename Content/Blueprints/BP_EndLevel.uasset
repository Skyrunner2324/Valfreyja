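; BP_EndLevel is the finish-line trigger of a level, reacting when BP_PlayerCharacter overlaps its box.
; It reads the final time from the first WB_Chrono widget, prints it, and passes it to BP_ScoreBoard's RunFinished.
; It then asks GM_Skyrunner to toggle the win screen.
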(event `self.Box.OnComponentBeginOverlap`
  (params (OverlappedComponent :type "PrimitiveComponent Object Reference") (OtherActor :type "Actor Object Reference") (OtherComp :type "PrimitiveComponent Object Reference") (OtherBodyIndex :type Integer) (bFromSweep :type Boolean) (SweepResult :type "HitResult Structure (by ref)"))
  (cast `/Game/Blueprints/Characters/BP_PlayerCharacter` OtherActor)
  (`|ExecutionSequence`
    (:`then_0`
      (bind _foundwidgets (`WidgetBlueprintLibrary.GetAllWidgetsOfClass` "/Game/UI/HUD/WB_Chrono.WB_Chrono_C" false))
      (bind _returnvalue (`GameplayStatics.GetActorOfClass` "/Game/Blueprints/Scoring/BP_ScoreBoard.BP_ScoreBoard_C"))
      (bind _chronovalue (`/Game/UI/HUD/WB_Chrono.ChronoValue` (`|GetArrayItem` _foundwidgets)))
      (`KismetSystemLibrary.PrintString` (`KismetStringLibrary.Concat_StrStr` "Chrono value : " (`KismetStringLibrary.Conv_DoubleToString` _chronovalue)))
      (`/Game/Blueprints/Scoring/BP_ScoreBoard.RunFinished` _returnvalue _chronovalue false))
    (:`then_1`
      (bind _asgm_skyrunner (cast `/Game/Blueprints/GameMode/GM_Skyrunner` (`GameplayStatics.GetGameMode`)))
      (`/Game/Blueprints/GameMode/GM_Skyrunner.ToggleWinScreen` _asgm_skyrunner))))

(fn `UserConstructionScript`)