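; Burst-fire enemy that shoots volleys at the player and is shielded except while reloading.
; BurstShoot fires a set number of shots per burst, each pulling an aimed bullet from a pool, with a trail for gunner bullets and a Wwise sound.
; When its bursts run out, Reload swaps the shield material and sets Vulnerable until the timer refills them.
; Timeline updates act as tickers, counting down shot and reload timers with delta time stored on Tick.
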(event `self.ReceiveBeginPlay`
  (`parent.ReceiveBeginPlay`)
  (set `self.Vulnerable` false)
  (set `self.ShotsLeft` (`self.MaxShots`))
  (`PrimitiveComponent.SetMaterial` (`self.Mesh`) 0 (`self.ShieldMat`)))

(event `BurstShoot`
  (bind _shotsleft (`self.ShotsLeft`))
  ;[1 1 1] BurstShot
  (set `self.IsShooting` true)
  (set `self.BurstProgression` 0)
  (if (< (`self.BurstProgression`) (`self.ShotsPerBurst`)) :!label _label
    (`self.Shoot`)
    (set `self.ShotTimer` (`self.MaxShotDelay`))
    (`Timeline|Timeline` :!via `PlayFromStart` :!label _label_2
      (:`Update`
        (bind _output_get (set `self.ShotTimer` (- (`self.ShotTimer`) (`self.StoredDeltaTime`))))
        (if (<= _output_get 0.0)
          (`/Engine/EditorBlueprintResources/StandardMacros.IncrementInt` (`self.BurstProgression`)
            (:`  `
              (goto _label))))))
    (else
      (`/Engine/EditorBlueprintResources/StandardMacros.DecrementInt` _shotsleft
        (:`  `
          (if (<= _shotsleft 0)
            (`self.Reload`))
          (set `self.IsShooting` false)
          (goto _label_2 :!via `Stop`))))))

(event `self.ReceiveTick`
  (params (DeltaSeconds :type "Float (single-precision)"))
  (`parent.ReceiveTick` DeltaSeconds)
  (set `self.StoredDeltaTime` DeltaSeconds))

(event `Reload`
  ;[1 1 1] Reload Timeline
  (`PrimitiveComponent.SetMaterial` (`self.Mesh`) 0 (`self.RegulatMat`))
  (set `self.ReloadTimer` (`self.MaxReloadTime`))
  (set `self.Vulnerable` true)
  (`Timeline|Timeline_0` :!label _label_3
    (:`Update`
      (bind _output_get (set `self.ReloadTimer` (- (`self.ReloadTimer`) (`self.StoredDeltaTime`))))
      (if (< _output_get 0.0)
        (set `self.Vulnerable` false)
        (set `self.ShotsLeft` (`self.MaxShots`))
        (`PrimitiveComponent.SetMaterial` (`self.Mesh`) 0 (`self.ShieldMat`))
        (goto _label_3 :!via `Stop`)))))

(fn `Shoot`
  (bind _actorpooled (`/Game/Blueprints/Libraries/FunctionLibraries/BFL_GetActorPooled.GetActorPooled` (`self.BulletClass`) (`SceneComponent.K2_GetComponentLocation` (`self.CanonSocket`)) (`KismetMathLibrary.FindLookAtRotation` (`self.K2_GetActorLocation`) (`self.K2_GetActorLocation` (`self.playerCharacter`)))))
  (cast `/Game/Blueprints/Projectiles/Bullet/BP_EnemyBulletGuner` _actorpooled
    (:`then`
      (`|SpawnActorFromClass` "/Game/Blueprints/Projectiles/BP_BulletTrailEnemy.BP_BulletTrailEnemy_C" (`KismetMathLibrary.MakeTransform` (`SceneComponent.K2_GetComponentLocation` (`self.CanonSocket`)) (`KismetMathLibrary.FindLookAtRotation` (`self.K2_GetActorLocation`) (`self.K2_GetActorLocation` (`self.playerCharacter`)))) "Undefined" "MultiplyWithRoot" null null))
    (:`CastFailed`
      _))
  (bind _asbp_bullet_base (cast `/Game/Blueprints/Projectiles/Bullet/BP_BulletBase` _actorpooled))
  (`/Game/Blueprints/Projectiles/Bullet/BP_BulletBase.InitBullet` _asbp_bullet_base)
  ;[0.5535 1 0.2465] Bullet Sound
  (`AkGameplayStatics.SpawnAkComponentAtLocation` "/Game/WwiseAudio/Events/Enemy/SX_enemy_gunner_shot.SX_enemy_gunner_shot" (`self.K2_GetActorLocation`) (struct) true)
  (set `self.fireCooldown` (`self.fireRate`)))

(fn `TryShoot`
  (if (`self.CanShoot`)
    (`self.BurstShoot`)))

(fn `UserConstructionScript`
  (`parent.UserConstructionScript`))