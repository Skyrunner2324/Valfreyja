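; Rocket-firing enemy that turns to face a player inside its detection sphere and launches rockets that home on the player's head.
; Tick yaws the body, aims the weapon and calls TryShoot, gated by CanShoot.
; Projectile overlaps deal damage through AC_TakeDamage only while vulnerable, and each restarts a delay before timed invincibility, which swaps the material and drives a Wwise RTPC.
; Death destroys the actor and plays a sound.
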(event `self.ReceiveTick`
  (params (DeltaSeconds :type "Float (single-precision)"))
  (bind _returnvalue (`self.K2_GetActorLocation` (`self.playerCharacter`)))
  (bind (_returnvalue_roll _returnvalue_pitch _returnvalue_yaw) (`KismetMathLibrary.BreakRotator` (`KismetMathLibrary.FindLookAtRotation` (`self.K2_GetActorLocation`) _returnvalue)))
  (bind (_returnvalue_roll_2 _returnvalue_pitch_2 _returnvalue_yaw_2) (`KismetMathLibrary.BreakRotator` (`KismetMathLibrary.FindLookAtRotation` (`SceneComponent.K2_GetComponentLocation` (`self.Weapon`)) _returnvalue)))
  (if (not (<= (`self.InvincibilityTimer`) 0.0))
    (`self.CheckInvincibilityEnd` DeltaSeconds))
  (if (`self.PlayerInRange`)
    (`self.K2_SetActorRotation` (`KismetMathLibrary.MakeRotator` 0.0 0.0 _returnvalue_yaw))
    (`SceneComponent.K2_SetWorldRotation` (`self.Weapon`) (`KismetMathLibrary.MakeRotator` 0.0 _returnvalue_pitch_2 _returnvalue_yaw_2) false false)
    (`self.TryShoot`)))

(event `self.detectionSphere.OnComponentBeginOverlap`
  (params (OverlappedComponent :type "PrimitiveComponent Object Reference") (OtherActor :type "Actor Object Reference") (OtherComp :type "PrimitiveComponent Object Reference") (OtherBodyIndex :type Integer) (bFromSweep :type Boolean) (SweepResult :type "HitResult Structure (by ref)"))
  ;[1 1 1] Detection Sphere overlap
  (bind _asbp_player_character (cast `/Game/Blueprints/Characters/BP_PlayerCharacter` OtherActor))
  (set `self.PlayerInRange` true)
  (`KismetSystemLibrary.PrintString` "LookAt player")
  (set `self.playerCharacter` _asbp_player_character))

(event `self.detectionSphere.OnComponentEndOverlap`
  (params (OverlappedComponent :type "PrimitiveComponent Object Reference") (OtherActor :type "Actor Object Reference") (OtherComp :type "PrimitiveComponent Object Reference") (OtherBodyIndex :type Integer))
  ;[1 1 1] Detection Sphere overlap
  (cast `/Game/Blueprints/Characters/BP_PlayerCharacter` OtherActor)
  (set `self.PlayerInRange` false)
  (`KismetSystemLibrary.PrintString` "Stop LookAt player"))

(event `self.CollisionProjectile.OnComponentBeginOverlap`
  (params (OverlappedComponent :type "PrimitiveComponent Object Reference") (OtherActor :type "Actor Object Reference") (OtherComp :type "PrimitiveComponent Object Reference") (OtherBodyIndex :type Integer) (bFromSweep :type Boolean) (SweepResult :type "HitResult Structure (by ref)"))
  ;[1 1 1] Overlap w/ projectile
  (`AkGameplayStatics.PostEvent` "/Game/WwiseAudio/Events/Player/Feedback/SX_player_feedback_hitmarker.SX_player_feedback_hitmarker")
  (if (<= (`self.InvincibilityTimer`) 0.0)
    (`/Game/Blueprints/Component/ActorComponent/Damage/AC_TakeDamage.TakeDamage` (`self.AC_TakeDamage`) (`self.GetComponentByClass` OtherActor "/Game/Blueprints/Component/ActorComponent/Damage/AC_DoDamageEnemie.AC_DoDamageEnemie_C"))
    (`KismetSystemLibrary.K2_ClearAndInvalidateTimerHandle` (`self.OnDamageTimer`))
    (bind _returnvalue (`KismetSystemLibrary.K2_SetTimer` null "InvincibilityStart" (`self.TimeAfterDamage`)))
    (set `self.OnDamageTimer` _returnvalue)))

(event `self.AC_TakeDamage.Death`
  ;[1 1 1] Death
  (`self.Death`)
  (`AkGameplayStatics.SpawnAkComponentAtLocation` "/Game/WwiseAudio/Events/Player/Feedback/SX_player_death_notifier.SX_player_death_notifier" (`self.K2_GetActorLocation`) (struct) true))

(fn `Death`
  (`KismetSystemLibrary.PrintString` "Death Rocket")
  (`self.K2_DestroyActor`))

(fn `InvincibilityStart`
  (`KismetSystemLibrary.PrintString` "Start invincibility")
  (set `self.InvincibilityTimer` (`self.MaxInvincibilityTime`))
  (`PrimitiveComponent.SetMaterial` (`self.skMeshComponent`) 0 (`self.InvincibilityMaterial`)))

(fn `TryShoot`
  (if (`self.CanShoot`)
    (bind _returnvalue (`|SpawnActorFromClass` (`self.BulletClass`) (`SceneComponent.K2_GetComponentToWorld` (`self.CanonSocket`)) "Undefined" "MultiplyWithRoot" null self))
    (bind _asbp_enemy_rocket (cast `/Game/Blueprints/Projectiles/Bullet/BP_EnemyRocket` _returnvalue))
    (bind _asbp_player_character (cast `/Game/Blueprints/Characters/BP_PlayerCharacter` (`self.playerCharacter`)))
    (set `ProjectileMovementComponent.HomingTargetComponent` (`/Game/Blueprints/Characters/BP_PlayerCharacter.HeadPosition` _asbp_player_character) (`/Game/Blueprints/Projectiles/Bullet/BP_BulletBase.ProjectileMovement` _asbp_enemy_rocket))
    (set `self.fireCooldown` (`self.fireRate`))))

(fn `UserConstructionScript`
  (set `self.InvincibilityTimer` (`self.MaxInvincibilityTime`))
  (bind _returnvalue (`KismetSystemLibrary.K2_SetTimer` null "InvincibilityStart" (`self.TimeAfterDamage`)))
  (set `self.OnDamageTimer` _returnvalue)
  (set `self.DefaultMeshMat` (`PrimitiveComponent.GetMaterial` (`self.skMeshComponent`) 0)))