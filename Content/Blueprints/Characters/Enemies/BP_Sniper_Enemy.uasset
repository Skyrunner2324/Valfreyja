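; Sniper enemy that tracks the player with a laser and deals damage after an uninterrupted aim countdown.
; Tick rotates laser and model, lerping when the player is grounded off-rail or time is dilated, otherwise snapping, then line-traces to size the beam and gate targeting.
; HitZone overlap drives the TimeSlippage-scaled countdown, blinking before firing and entering cooldown.
; A player event cancels warned shots; game mode resets rebind the player.
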(event `self.ReceiveBeginPlay`
  (`parent.ReceiveBeginPlay`)
  (bind _asskyrunner_game_mode (cast `SkyrunnerGameMode` (`GameplayStatics.GetGameMode`)))
  (add `SkyrunnerGameMode.OnPlayerResetEvent` _asskyrunner_game_mode (delegate `OnReset`))
  (bind _asbp_player_character (cast `/Game/Blueprints/Characters/BP_PlayerCharacter` (`GameplayStatics.GetPlayerCharacter` 0) :!label _label))
  (bind _output_get (set `self.PlayerRef` _asbp_player_character))
  (add `/Game/Blueprints/Characters/BP_PlayerCharacter.CancelSnipersShots` _output_get (delegate `CancelShot`)))

(event `OnReset`
  (goto _label))

(event `CancelShot`
  (if (`self.Warning`)
    (set `self.Targetting` false)
    (set `self.Warning` false)
    (`self.StartShotCD`)))

(event `self.ReceiveTick`
  (params (DeltaSeconds :type "Float (single-precision)"))
  (bind _playerinrange (`self.PlayerInRange`))
  (bind _playerref (`self.PlayerRef`))
  (bind _lasersocket (`self.LaserSocket`))
  (bind _lasersocket_2 (`self.LaserSocket`))
  (bind _lasersocket_3 (`self.LaserSocket`))
  (bind _returnvalue (`SceneComponent.K2_GetComponentLocation` _lasersocket_2))
  (bind _returnvalue_2 (- (`self.K2_GetActorLocation` _playerref) (`SceneComponent.K2_GetComponentLocation` (`self.LaserSocket`))))
  (bind _returnvalue_3 (`KismetMathLibrary.MakeRotFromZ` _returnvalue_2))
  (bind _returnvalue_4 (`KismetMathLibrary.VSize` _returnvalue_2))
  (bind _returnvalue_5 (`KismetMathLibrary.RLerp` (`SceneComponent.K2_GetComponentRotation` _lasersocket_3) _returnvalue_3 (* (`TimeSlippage.GetGlobalTimeScale` (`TimeSlippageModifier.timeSlippage` (`self.TimeSlippageModifier`))) (`self.TargettingSpeed`)) true))
  (if (or (and (`NavMovementComponent.IsMovingOnGround` (`Character.CharacterMovement` _playerref)) (not (`/Game/Blueprints/Characters/BP_PlayerCharacter.IsOnRail` _playerref))) (`TimeSlippage.bIsDilated` (`TimeSlippageModifier.timeSlippage` (`self.TimeSlippageModifier`))))
    (`SceneComponent.K2_SetWorldRotation` _lasersocket_3 _returnvalue_5 false false)
    (`self.RotateModel` (`.Z (Yaw)` (`self.GetSplittedValues` _returnvalue_5)))
    (else
      (`SceneComponent.K2_SetWorldRotation` _lasersocket_3 _returnvalue_3 false false)
      (`self.RotateModel` (`.Z (Yaw)` (`self.GetSplittedValues` _returnvalue_3)))))
  (bind (_outhit _returnvalue_6) (`KismetSystemLibrary.LineTraceSingle` :`Start` _returnvalue :`End` (+ _returnvalue (* (`SceneComponent.GetUpVector` _lasersocket_2) _returnvalue_4)) :`TraceChannel` "TraceTypeQuery1" :`DrawDebugType` "ForOneFrame"))
  (`|ExecutionSequence`
    (:`then_0`
      (if (and (not _returnvalue_6) _playerinrange)
        (`self.TargetFunc`)))
    (:`then_1`
      (if (and _playerinrange (`self.Targetting`))
        (if _returnvalue_6
          (`SceneComponent.SetWorldScale3D` _lasersocket (`KismetMathLibrary.MakeVector` 1.0 1.0 (/ (`.Distance` (`GameplayStatics.BreakHitResult` _outhit)) 10.0)))
          (set `self.Targetting` false :!label _label_2)
          (else
            (`SceneComponent.SetWorldScale3D` _lasersocket (`KismetMathLibrary.MakeVector` 1.0 1.0 (/ _returnvalue_4 10.0)))))
        (else
          (`SceneComponent.SetWorldScale3D` _lasersocket (1.0 1.0 1.0))
          (goto _label_2))))))

(fn `Laser Blink`
  (bind _laser (`self.Laser`))
  (if (== (mod (`KismetMathLibrary.FCeil64` (* (`self.AimTimer`) 10.0)) 2) 0)
    (`SceneComponent.SetVisibility` _laser false true)
    (else
      (`SceneComponent.SetVisibility` _laser true true))))

(fn `RotateModel`
  (params (Angle :type "Float (double-precision)"))
  (`SceneComponent.K2_SetWorldRotation` (`self.WeaponSocket`) (`KismetMathLibrary.MakeRotator` 0.0 0.0 (- Angle 90.0)) false false)
  (`SceneComponent.K2_SetWorldRotation` (`self.skMeshComponent`) (`KismetMathLibrary.MakeRotator` 0.0 0.0 (+ Angle 180.0)) false false))

(fn `SniperShoot`
  (returns (PlayerHit :type Boolean))
  (return (`PrimitiveComponent.IsOverlappingActor` (`self.HitZone`) (`self.PlayerRef`))))

(fn `TargetFunc`
  (bind _shotcooldown (`self.ShotCooldown`))
  (bind _globalmanageddeltatime (`TimeSlippage.globalManagedDeltaTime` (`TimeSlippageModifier.timeSlippage` (`self.TimeSlippageModifier`))))
  (if (> _shotcooldown 0.0)
    (set `self.ShotCooldown` (- _shotcooldown _globalmanageddeltatime))
    (else
      (set `self.Targetting` true)
      (if (`PrimitiveComponent.IsOverlappingActor` (`self.HitZone`) (`self.PlayerRef`))
        (bind _output_get (set `self.AimTimer` (- (`self.AimTimer`) _globalmanageddeltatime)))
        (if (< _output_get 1.0)
          (set `self.Warning` true)
          (`self.Laser Blink`)
          (if (< (`self.AimTimer`) 0.0)
            (`/Game/Blueprints/Component/ActorComponent/Damage/AC_TakeDamage.TakeDamage` (`/Game/Blueprints/Characters/BP_PlayerCharacter.TakeDamage` (`self.PlayerRef`)) (`self.DoDamagePlayer`))
            (set `self.Warning` false)
            (set `self.Targetting` false)
            (`self.StartShotCD`)))
        (else
          (set `self.AimTimer` (`self.MaxAimTimer`))
          (`SceneComponent.SetVisibility` (`self.Laser`) true true))))))

(fn `UserConstructionScript`
  (`parent.UserConstructionScript`)
  (`self.SetTickGroup` "TG_PostUpdateWork"))