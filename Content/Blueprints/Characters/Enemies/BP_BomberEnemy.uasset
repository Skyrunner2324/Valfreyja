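; Bomber enemy that bombards the player with mortar-style fire, enabling its behavior tree on blackboard init.
; TryShoot traces down from above randomly offset points around the player, spawns a pooled bullet at the ground hit, then resets the cooldown.
; Each successful shot also launches a cosmetic bullet skyward from the cannon socket and scatters additional bullets within a separate radial imprecision range.
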(event `self.InitBB`
  (`parent.InitBB`)
  (`BlackboardComponent.SetValueAsBool` (`self.BlackBoard`) "bExecuteBT" true))

(event `self.OnTargetUpdate`
  (params (Target :type "/Game/Blueprints/Characters/BP_PlayerCharacter Object Reference"))
  (`parent.OnTargetUpdate` Target))

(fn `CreateSecondaryBullet`
  (bind (_returnvalue_x _returnvalue_y) (`KismetMathLibrary.BreakVector` (`KismetMathLibrary.RandomUnitVector`)))
  (bind (_secondaryimprecision_x _secondaryimprecision_y) (`KismetMathLibrary.BreakVector2D` (`self.secondaryImprecision`)))
  (bind (_returnvalue_x_2 _returnvalue_y_2) (`KismetMathLibrary.BreakVector2D` (* (`KismetMathLibrary.RandomFloatInRange` _secondaryimprecision_x _secondaryimprecision_y) (`KismetMathLibrary.Normal2D` (`KismetMathLibrary.MakeVector2D` _returnvalue_x _returnvalue_y)))))
  (bind _returnvalue (`KismetMathLibrary.MakeVector` (+ (.x (`self.K2_GetActorLocation` (`self.playerCharacter`))) _returnvalue_x_2) (+ (.y (`self.K2_GetActorLocation` (`self.playerCharacter`))) _returnvalue_y_2) (+ (.z (`self.K2_GetActorLocation` (`self.playerCharacter`))) (`self.RaycastTopHeight`))))
  (bind (_outhit _returnvalue_2) (`KismetSystemLibrary.LineTraceSingle` :`Start` _returnvalue :`End` (- _returnvalue (0.0 0.0 50000.0)) :`TraceChannel` "TraceTypeQuery1" :`DrawDebugType` "ForDuration" :`DrawTime` 0.5)) ; Trace from "almost" player towards ground
  (if _returnvalue_2
    (bind _actorpooled (`/Game/Blueprints/Libraries/FunctionLibraries/BFL_GetActorPooled.GetActorPooled` (`self.BulletClass`) (`.Location` (`GameplayStatics.BreakHitResult` _outhit))))
    (bind _asbp_bullet_base (cast `/Game/Blueprints/Projectiles/Bullet/BP_BulletBase` _actorpooled))
    (`/Game/Blueprints/Projectiles/Bullet/BP_BulletBase.InitBullet` _asbp_bullet_base)))

(fn `CreateVisualBullet`
  (bind _returnvalue (`self.K2_GetActorRotation`))
  (bind _actorpooled (`/Game/Blueprints/Libraries/FunctionLibraries/BFL_GetActorPooled.GetActorPooled` (`self.FakeBulletClass`) (`SceneComponent.K2_GetComponentLocation` (`self.CanonSocket`)) (`KismetMathLibrary.ComposeRotators` _returnvalue (`KismetMathLibrary.RotatorFromAxisAndAngle` (`KismetMathLibrary.GetRightVector` _returnvalue) -85.0))))
  (bind _asbp_bullet_base (cast `/Game/Blueprints/Projectiles/Bullet/BP_BulletBase` _actorpooled))
  (`/Game/Blueprints/Projectiles/Bullet/BP_BulletBase.InitBullet` _asbp_bullet_base))

(fn `TryShoot`
  (bind _maximprecision (`self.maxImprecision`))
  (bind _returnvalue (`KismetMathLibrary.MakeVector` (+ (.x (`self.K2_GetActorLocation` (`self.playerCharacter`))) (`KismetMathLibrary.RandomFloatInRange` (- 0.0 _maximprecision) _maximprecision)) (+ (.y (`self.K2_GetActorLocation` (`self.playerCharacter`))) (`KismetMathLibrary.RandomFloatInRange` (- 0.0 _maximprecision) _maximprecision)) (+ (.z (`self.K2_GetActorLocation` (`self.playerCharacter`))) (`self.RaycastTopHeight`))))
  (if (`self.CanShoot`)
    (bind (_outhit _returnvalue_2) (`KismetSystemLibrary.LineTraceSingle` :`Start` _returnvalue :`End` (- _returnvalue (0.0 0.0 10000.0)) :`TraceChannel` "TraceTypeQuery1" :`DrawDebugType` "ForDuration" :`DrawTime` 0.5)) ; Trace from "almost" player towards ground
    (if _returnvalue_2
      (bind _actorpooled (`/Game/Blueprints/Libraries/FunctionLibraries/BFL_GetActorPooled.GetActorPooled` (`self.BulletClass`) (`.Location` (`GameplayStatics.BreakHitResult` _outhit))))
      (bind _asbp_bullet_base (cast `/Game/Blueprints/Projectiles/Bullet/BP_BulletBase` _actorpooled))
      (`/Game/Blueprints/Projectiles/Bullet/BP_BulletBase.InitBullet` _asbp_bullet_base)
      (set `self.fireCooldown` (`self.fireRate`))
      (`self.CreateVisualBullet`)
      (for _ (range 1 (+ (`self.additionalBullets`) 1))
        (`self.CreateSecondaryBullet`)))))

(fn `UserConstructionScript`
  (`parent.UserConstructionScript`)
  (set `self.maxImprecision` (/ (`self.maxImprecision`) 2.0)) ; Halve imprecision because it is a radial value
)