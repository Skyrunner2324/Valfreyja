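; BP_DotMarker is an enemy marker Blueprint that shows a dot widget through its DotMarker widget component.
; Each tick it rotates the widget to face the player camera, acting as a billboard.
; A Hit event plays the hit animation on WB_DotMarker_, and ChangeTextureDotMarker passes a DilationType to the widget to swap its texture.
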(event `self.ReceiveTick`
  (params (DeltaSeconds :type "Float (single-precision)"))
  (`SceneComponent.K2_SetWorldRotation` (`self.DotMarker`) (`KismetMathLibrary.FindLookAtRotation` (`SceneComponent.K2_GetComponentLocation` (`self.DotMarker`)) (`PlayerCameraManager.GetCameraLocation` (`GameplayStatics.GetPlayerCameraManager` 0))) false false))

(event `Hit`
  (bind _aswb_dot_marker_ (cast `/Game/UI/WB_DotMarker_` (`WidgetComponent.GetWidget` (`self.DotMarker`))))
  (`/Game/UI/WB_DotMarker_.HitAnim` _aswb_dot_marker_))

(fn `ChangeTextureDotMarker`
  (params (dilationType :type "/Game/Blueprints/Enumerator/E_DilationType Enum" :default "NewEnumerator0"))
  (bind _aswb_dot_marker_ (cast `/Game/UI/WB_DotMarker_` (`WidgetComponent.GetUserWidgetObject` (`self.DotMarker`))))
  (`/Game/UI/WB_DotMarker_.ChangeTexture` _aswb_dot_marker_ (`local.dilationType`)))

(fn `UserConstructionScript`)