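; Sniper enemy that tracks the player with a laser and deals an unavoidable hit unless the shot is canceled.
; Tick aims and traces to the player, starting targeting when visible and in range, and stretching the laser to the trace distance.
; After an aim delay the laser blinks, then damages directly without rechecking sight; the player's cancel event works only during this warning.
; Shots and cancels trigger a cooldown; overlaps feed the damage component, whose death event destroys the sniper.
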(event `self.ReceiveBeginPlay`
  (add `/Game/Blueprints/Component/ActorComponent/Damage/AC_TakeDamage.Death` (`self.TakeDamage`) (`|CreateDelegate` :!event `Death`))
  (bind _asbp_player_character (cast `/Game/Blueprints/Characters/BP_PlayerCharacter` (`GameplayStatics.GetPlayerCharacter` 0)))
  (bind _output_get (set `self.PlayerRef` _asbp_player_character))
  (add `/Game/Blueprints/Characters/BP_PlayerCharacter.CancelSnipersShots` _output_get (delegate `CancelShot`)))

(event `CancelShot`
  (if (`self.Warning`)
    (set `self.Targetting` false)
    (set `self.ShotCanceled` true)
    (set `self.Warning` false)
    (`self.StartShotCooldown`)))

(event `self.ReceiveTick`
  (params (DeltaSeconds :type "Float (single-precision)"))
  (bind _lasersocket (`self.LaserSocket`))
  (bind _returnvalue (`self.K2_GetActorLocation` (`self.PlayerRef`)))
  (bind _returnvalue_2 (`SceneComponent.K2_GetComponentLocation` (`self.LaserSocket`)))
  (bind _returnvalue_3 (- _returnvalue _returnvalue_2))
  (bind _returnvalue_4 (`KismetMathLibrary.VSize` _returnvalue_3))
  (`SceneComponent.K2_SetWorldRotation` _lasersocket (`KismetMathLibrary.MakeRotFromZ` (`KismetMathLibrary.Normal` _returnvalue_3)) false false)
  (bind (_outhit _returnvalue_5) (`KismetSystemLibrary.LineTraceSingle` :`Start` _returnvalue_2 :`End` _returnvalue :`TraceChannel` "TraceTypeQuery1" :`DrawDebugType` "ForOneFrame"))
  (`|ExecutionSequence`
    (:`then_0`
      (if (and (not _returnvalue_5) (< _returnvalue_4 (`self.DetectionRange`)))
        (`self.StartTargetting`)))
    (:`then_1`
      (if (`self.Targetting`)
        (if _returnvalue_5
          (`SceneComponent.SetWorldScale3D` _lasersocket (`KismetMathLibrary.MakeVector` 1.0 1.0 (/ (`.Distance` (`GameplayStatics.BreakHitResult` _outhit)) 10.0)))
          (else
            (`SceneComponent.SetWorldScale3D` _lasersocket (`KismetMathLibrary.MakeVector` 1.0 1.0 (/ _returnvalue_4 10.0)))))
        (else
          (`SceneComponent.SetWorldScale3D` _lasersocket (1.0 1.0 1.0)))))))

(event `self.CollisionProjectile.OnComponentBeginOverlap`
  (params (OverlappedComponent :type "PrimitiveComponent Object Reference") (OtherActor :type "Actor Object Reference") (OtherComp :type "PrimitiveComponent Object Reference") (OtherBodyIndex :type Integer) (bFromSweep :type Boolean) (SweepResult :type "HitResult Structure (by ref)"))
  (`/Game/Blueprints/Component/ActorComponent/Damage/AC_TakeDamage.TakeDamage` (`self.TakeDamage`) (`self.GetComponentByClass` OtherActor "/Game/Blueprints/Component/ActorComponent/Damage/AC_DoDamageEnemie.AC_DoDamageEnemie_C")))

(fn `Death`
  (`KismetSystemLibrary.PrintString` "Death Enemi")
  (`self.K2_DestroyActor`))

(fn `UserConstructionScript`
  (`self.SetTickGroup` "TG_PostUpdateWork"))