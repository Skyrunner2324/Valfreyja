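; Gunner enemy that registers with BP_EnemyManager and fires pooled bullets aimed at the player through TryShoot.
; AI controller target updates feed the Blackboard and toggle a health bar, refreshed each tick from the shield ratio.
; Bullet overlaps on capsule or mesh remove the bullet, apply damage via ACTakeDamage and show a hitmarker.
; Death unregisters and destroys the enemy, plays a sound and adds time dilation through the player controller.
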(event `self.ReceiveBeginPlay`
  (`self.InitBB`)
  (`SceneComponent.SetVisibility` (`self.HealthBar`) false true)
  ;[1 1 1] Death
  (add `/Game/Blueprints/Component/ActorComponent/Damage/AC_TakeDamage.Death` (`self.AC_TakeDamage`) (`|CreateDelegate` :!event `Death`))
  (`|ExecutionSequence`
    (:`then_0`
      ;[1 1 1] manager
      (bind _returnvalue (`GameplayStatics.GetActorOfClass` "/Game/Blueprints/Managers/BP_EnemyManager.BP_EnemyManager_C"))
      (`/Engine/EditorBlueprintResources/StandardMacros.IsValid` _returnvalue
        (:`Is Valid`
          (bind _output_get (set `self.EnemyManager` _returnvalue))
          (`/Game/Blueprints/Managers/BP_EnemyManager.NewEnemy` _output_get self))
        (:`Is Not Valid`
          (`KismetSystemLibrary.PrintString` "--------------------------------------------------------------- \nNO ENEMY MANAGER FOUND, PLEASE ADD ONE IN THE SCENE \n---------------------------------------------------------------" true true (struct :`R` 1.0 :`A` 1.0) 60.0 "ManagerError"))))
    (:`then_1`
      ;[1 1 1] perception
      (bind _asaic_enemy_controller (cast `/Game/Blueprints/AI/Controller/AIC_EnemyController` (`AIBlueprintHelperLibrary.GetAIController` self)))
      (add `/Game/Blueprints/AI/Controller/AIC_EnemyController.OnTargetUpdate` _asaic_enemy_controller (delegate `OnTargetUpdate`)))))

(event `OnTargetUpdate`
  (params (Target :type "/Game/Blueprints/Characters/BP_PlayerCharacter Object Reference"))
  ;[1 1 1] perception
  (`/Engine/EditorBlueprintResources/StandardMacros.IsValid` Target
    (:`Is Valid`
      (set `self.PlayerInRange` true)
      (set `self.playerCharacter` Target)
      (`SceneComponent.SetVisibility` (`self.HealthBar`) true true)
      (`BlackboardComponent.SetValueAsObject` (`self.BlackBoard`) "Target" Target))
    (:`Is Not Valid`
      (set `self.PlayerInRange` false)
      (`SceneComponent.SetVisibility` (`self.HealthBar`) false true)
      (`BlackboardComponent.SetValueAsObject` (`self.BlackBoard`) "Target" null))))

(event `self.ReceiveTick`
  (params (DeltaSeconds :type "Float (single-precision)"))
  ;[1 1 1] tick
  (`self.UpdateHealthBar`))

(event `self.CapsuleComponent.OnComponentBeginOverlap`
  (params (OverlappedComponent :type "PrimitiveComponent Object Reference") (OtherActor :type "Actor Object Reference") (OtherComp :type "PrimitiveComponent Object Reference") (OtherBodyIndex :type Integer) (bFromSweep :type Boolean) (SweepResult :type "HitResult Structure (by ref)"))
  ;[1 1 1] Overlap w/ projectile
  ;;[1 1 1] capsule collision vs sk mesh collision
  (bind _asbp_bullet_base (cast `/Game/Blueprints/Projectiles/Bullet/BP_BulletBase` OtherActor :!label _label))
  (`/Game/Blueprints/Projectiles/Bullet/BP_BulletBase.RemoveBullet` _asbp_bullet_base)
  (`AkGameplayStatics.PostEvent` "/Game/WwiseAudio/Events/Player/Feedback/SX_player_feedback_hitmarker.SX_player_feedback_hitmarker")
  (`PrimitiveComponent.SetCollisionEnabled` (`/Game/Blueprints/Projectiles/Bullet/BP_BulletBase.CollisionComponent` _asbp_bullet_base) "NoCollision")
  (bind _takedamage (`/Game/Blueprints/Component/ActorComponent/Damage/AC_TakeDamage.TakeDamage` (`self.AC_TakeDamage`) (`self.GetComponentByClass` OtherActor "/Game/Blueprints/Component/ActorComponent/Damage/AC_DoDamageEnemie.AC_DoDamageEnemie_C") 0.0))
  (if _takedamage
    (`self.DisplayHitMarker`)))

(event `self.Mesh.OnComponentBeginOverlap`
  (params (OverlappedComponent :type "PrimitiveComponent Object Reference") (OtherActor :type "Actor Object Reference") (OtherComp :type "PrimitiveComponent Object Reference") (OtherBodyIndex :type Integer) (bFromSweep :type Boolean) (SweepResult :type "HitResult Structure (by ref)"))
  ;[1 1 1] Overlap w/ projectile
  ;;[1 1 1] capsule collision vs sk mesh collision
  (goto _label))

(event `DisplayHitMarker`
  ;[1 1 1] hitmarker
  (bind _returnvalue (`|CreateWidget` "/Game/UI/HUD/WB_HitMark.WB_HitMark_C"))
  (`UserWidget.AddToViewport` _returnvalue 0))

(fn `Death`
  (bind _enemymanager (`self.EnemyManager`))
  (`|ExecutionSequence`
    (:`then_0`
      (`KismetSystemLibrary.PrintString` "Death Gunner")
      (`/Engine/EditorBlueprintResources/StandardMacros.IsValid` _enemymanager
        (:`Is Valid`
          (`/Game/Blueprints/Managers/BP_EnemyManager.RemoveEnemy` _enemymanager self))
        (:`Is Not Valid`
          _))
      (`self.K2_DestroyActor`)
      ;[1 1 1] Add dilation to death
      (bind _asbp_player_controller (cast `/Game/Blueprints/Controller/BP_PlayerController` (`GameplayStatics.GetPlayerController` 0)))
      (`/Game/Blueprints/Controller/BP_PlayerController.AddDilation` _asbp_player_controller (`self.NumberOfDilationToAdd`)))
    (:`then_1`
      (`AkGameplayStatics.SpawnAkComponentAtLocation` "/Game/WwiseAudio/Events/Player/Feedback/SX_player_death_notifier.SX_player_death_notifier" (`self.K2_GetActorLocation`) (struct) true))))

(fn `InitBB`
  (`|ExecutionSequence`
    (:`then_0`
      (set `self.BlackBoard` (`AIBlueprintHelperLibrary.GetBlackboard` (`AIBlueprintHelperLibrary.GetAIController` self))))
    (:`then_1`
      (`BlackboardComponent.SetValueAsBool` (`self.BlackBoard`) "bExecuteBT" true))))

(fn `TryShoot`
  (if (`self.CanShoot`)
    (bind _actorpooled (`/Game/Blueprints/Libraries/FunctionLibraries/BFL_GetActorPooled.GetActorPooled` (`self.BulletClass`) (`SceneComponent.K2_GetComponentLocation` (`self.CanonSocket`)) (`KismetMathLibrary.FindLookAtRotation` (`self.K2_GetActorLocation`) (`self.K2_GetActorLocation` (`self.playerCharacter`)))))
    (bind _asbp_bullet_base (cast `/Game/Blueprints/Projectiles/Bullet/BP_BulletBase` _actorpooled))
    (`/Game/Blueprints/Projectiles/Bullet/BP_BulletBase.InitBullet` _asbp_bullet_base)
    (set `self.fireCooldown` (`self.fireRate`))))

(fn `UpdateHealthBar`
  (bind _aswb_enemy_health_bar (cast `/Game/UI/Enemy/WB_EnemyHealthBar` (`WidgetComponent.GetWidget` (`self.HealthBar`))))
  (`ProgressBar.SetPercent` (`/Game/UI/Enemy/WB_EnemyHealthBar.HealthBar` _aswb_enemy_health_bar) (`/Game/Blueprints/Component/ActorComponent/Damage/AC_TakeDamage.GetShieldRatio` (`self.AC_TakeDamage`))))

(fn `UserConstructionScript`)