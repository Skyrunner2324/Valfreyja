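; First-person player character with wall run, crouch/slide, rail grinding, switchable arm-mounted weapons, damage and death.
; Rail overlap starts a Tick-driven grind at clamped entry speed, and jumping dismounts with momentum.
; A detection sphere feeds nearby enemies to the controller's aiming system, while time-slippage changes set local time scale by dilation type.
; Also drives Wwise movement audio and dilation post-process; CanJumpInternal always returns true, leaving coyote-time checks unwired.
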(event `self.TimeSlippageModifier.OnTimeScaleChangedEvent`
  (params (newScale :type "Float (single-precision)"))
  (`self.ChangeTargetLocalTimeScale` newScale))

(event `self.ReceiveBeginPlay`
  ;[0 1 0.1956] Audio State - player is alive
  (`AkGameplayStatics.SetState` "/Game/WwiseAudio/States/Default_Work_Unit/PlayerState/PlayerState-Alive.PlayerState-Alive")
  (`|ExecutionSequence`
    (:`then_0`
      (`/Game/Blueprints/Component/ActorComponent/AC_WallRun.Initialize` (`self.WallRun`) self)
      (add `/Game/Blueprints/Component/ActorComponent/Damage/AC_TakeDamage.Death` (`self.TakeDamage`) (`|CreateDelegate` :!event `Death`))
      ;[1 1 1] Add Weapon
      (for _array_element (`self.allWeapon`)
        (`self.AddWeapon` _array_element))
      (`self.InitStartWeapon`)
      (set `self.controllerRef` (cast `/Game/Blueprints/Controller/BP_PlayerController` (`self.GetController`) :!pure true)))
    (:`then_1`
      (`self.InitPostProcessMaterials`))))

(event `self.OnLanded`
  (params (Hit :type "HitResult Structure (by ref)"))
  (`parent.OnLanded` Hit)
  (`KismetSystemLibrary.K2_ClearAndInvalidateTimerHandle` (`self.coyoteTimer`))
  (`/Game/Blueprints/Controller/BP_PlayerController.Land` (`self.controllerRef`))
  (`/Game/Blueprints/Component/ActorComponent/AC_WallRun.LandEvent` (`self.WallRun`))
  (`/Game/Blueprints/Component/ActorComponent/AC_CrouchAndSlide.LandEvent` (`self.CrouchAndSlide`))
  ;[0 1 0.2431] Land Sound
  (`AkGameplayStatics.PostEvent` "/Game/WwiseAudio/Events/Game/Player/SX_player_land.SX_player_land")
  (`AkGameplayStatics.SetRTPCValue` "/Game/WwiseAudio/Game_Parameters/Default_Work_Unit/RTPC_PlayerMovement.RTPC_PlayerMovement" 0.5))

(event `self.EnemyDetectionSphere.OnComponentBeginOverlap`
  (params (OverlappedComponent :type "PrimitiveComponent Object Reference") (OtherActor :type "Actor Object Reference") (OtherComp :type "PrimitiveComponent Object Reference") (OtherBodyIndex :type Integer) (bFromSweep :type Boolean) (SweepResult :type "HitResult Structure (by ref)"))
  (`self.isAnEnemy` OtherActor
    (:`True`
      (`KismetArrayLibrary.Array_AddUnique` (`/Game/Blueprints/Component/ActorComponent/AC_AimingSystem.nearEnemies` (`/Game/Blueprints/Controller/BP_PlayerController.AimingSystem` (`self.controllerRef`))) OtherActor))))

(event `self.EnemyDetectionSphere.OnComponentEndOverlap`
  (params (OverlappedComponent :type "PrimitiveComponent Object Reference") (OtherActor :type "Actor Object Reference") (OtherComp :type "PrimitiveComponent Object Reference") (OtherBodyIndex :type Integer))
  (bind _aimingsystem (`/Game/Blueprints/Controller/BP_PlayerController.AimingSystem` (`self.controllerRef`)))
  (`self.isAnEnemy` OtherActor
    (:`True`
      (`KismetArrayLibrary.Array_RemoveItem` (`/Game/Blueprints/Component/ActorComponent/AC_AimingSystem.nearEnemies` _aimingsystem) OtherActor)
      (if (== OtherActor (`/Game/Blueprints/Component/ActorComponent/AC_AimingSystem.enemyLocked` _aimingsystem))
        (`/Game/Blueprints/Component/ActorComponent/AC_AimingSystem.UnlockEnemy` _aimingsystem)))))

(event `self.K2_OnMovementModeChanged`
  (params (PrevMovementMode :type "EMovementMode Enum" :default "MOVE_None") (NewMovementMode :type "EMovementMode Enum" :default "MOVE_None") (PrevCustomMode :type Byte) (NewCustomMode :type Byte))
  ;[1 1 1] Coyote Time
  (if (`|EnumEquality` NewMovementMode "MOVE_Falling")
    (bind _returnvalue (`KismetSystemLibrary.K2_SetTimerDelegate` (delegate `CoyoteTimePassed`) (`self.coyoteTime`)))
    (set `self.coyoteTimer` _returnvalue)))

(event `CoyoteTimePassed`
  ;[1 1 1] Coyote Time
  (`KismetSystemLibrary.K2_ClearAndInvalidateTimerHandle` (`self.coyoteTimer`)))

(event `self.OnJumped`
  ;[1 1 1] Clear Coyote time
  (`KismetSystemLibrary.K2_ClearAndInvalidateTimerHandle` (`self.coyoteTimer`))
  ;[1 1 1] Dismount from rail
  (if (`self.IsOnRail`)
    (`self.CancelSnipersShots`)
    (set `self.IsOnRail` false)
    (bind _direction (`/Game/Blueprints/CustomRails.GetMovementDirection` (`self.AttachedRail`)))
    (set `MovementComponent.Velocity` (+ (* _direction (`self.GrindVelocity`)) (`self.GetVelocity`)) (`self.CharacterMovement`))
    (set `self.AttachedRail` null)))

(event `self.ReceiveTick`
  (params (DeltaSeconds :type "Float (single-precision)"))
  (`|ExecutionSequence`
    (:`then_0`
      ;[0 1 0.2431] get player speed RTPC
      (`AkGameplayStatics.SetRTPCValue` "/Game/WwiseAudio/Game_Parameters/Default_Work_Unit/RTPC_PlayerSpeed.RTPC_PlayerSpeed" (`KismetMathLibrary.VSize` (`CharacterMovementComponent.GetLastUpdateVelocity` (`self.CharacterMovement`))))
      ;[1 1 1] Update rail position
      (if (`self.IsOnRail`)
        (`AkGameplayStatics.SetRTPCValue` "/Game/WwiseAudio/Game_Parameters/Default_Work_Unit/RTPC_PlayerMovement.RTPC_PlayerMovement" 2.5)
        (bind (_endreached _worldposition) (`/Game/Blueprints/CustomRails.GetNextStepOnRail` (`self.AttachedRail`) (* DeltaSeconds (`self.GrindVelocity`))))
        (if _endreached
          (`self.Jump`)
          ;;[0 0.568 0.2536] Audio States - is player on air or on rail
          (`AkGameplayStatics.SetRTPCValue` "/Game/WwiseAudio/Game_Parameters/Default_Work_Unit/RTPC_PlayerMovement.RTPC_PlayerMovement" 4.5)
          (else
            (`self.K2_SetActorLocation` (`KismetMathLibrary.MakeVector` (.x _worldposition) (.y _worldposition) (+ (.z _worldposition) (`CapsuleComponent.CapsuleHalfHeight` (`self.CapsuleComponent`)))))
            (`AkGameplayStatics.SetRTPCValue` "/Game/WwiseAudio/Game_Parameters/Default_Work_Unit/RTPC_PlayerMovement.RTPC_PlayerMovement" 2.5)))))
    (:`then_1`
      (`self.GetDistanceFromGround` 999.0))))

(event `self.Sphere.OnComponentBeginOverlap`
  (params (OverlappedComponent :type "PrimitiveComponent Object Reference") (OtherActor :type "Actor Object Reference") (OtherComp :type "PrimitiveComponent Object Reference") (OtherBodyIndex :type Integer) (bFromSweep :type Boolean) (SweepResult :type "HitResult Structure (by ref)"))
  (bind (_returnvalue_x _returnvalue_y _returnvalue_z) (`KismetMathLibrary.BreakVector` (`self.K2_GetActorLocation`)))
  ;[1 1 1] Contact with rail
  (if (not (`self.IsOnRail`))
    (set `self.GrindVelocity` (`KismetMathLibrary.FClamp` (+ (`KismetMathLibrary.VSize` (`self.GetVelocity`)) 1.0) (`self.MinVelocity`) (`self.MaxVelocity`)))
    (if (and (`self.ActorHasTag` OtherActor "Rail") (not (`self.IsOnRail`)))
      (bind _ascustom_rails (cast `/Game/Blueprints/CustomRails` OtherActor))
      (bind _output_get (set `self.AttachedRail` _ascustom_rails))
      (`/Game/Blueprints/CustomRails.SetMovementDirection` _output_get (`KismetMathLibrary.MakeVector` _returnvalue_x _returnvalue_y (- _returnvalue_z (`CapsuleComponent.CapsuleHalfHeight` (`self.CapsuleComponent`)))) (`SceneComponent.GetForwardVector` (`self.CapsuleComponent`)))
      (`self.SnapToRail`)
      (set `self.IsOnRail` true)
      (`AkGameplayStatics.SetRTPCValue` "/Game/WwiseAudio/Game_Parameters/Default_Work_Unit/RTPC_PlayerMovement.RTPC_PlayerMovement" 2.5))))

(event `self.CapsuleComponent.OnComponentBeginOverlap`
  (params (OverlappedComponent :type "PrimitiveComponent Object Reference") (OtherActor :type "Actor Object Reference") (OtherComp :type "PrimitiveComponent Object Reference") (OtherBodyIndex :type Integer) (bFromSweep :type Boolean) (SweepResult :type "HitResult Structure (by ref)"))
  ;[1 1 1] Take Damage Player
  (`self.TakeDamage_` OtherActor))

(fn `AddPostProcessMaterial`
  (params (PostProcessMaterial :type "Array of MaterialInterface Object Reference"))
  (returns (MaterialInstanceDynamic :type "Array of MaterialInstanceDynamic Object Reference"))
  (locals (Array :type "Array of WeightedBlendable Structure") (MIDArray :type "Array of MaterialInstanceDynamic Object Reference"))
  (for _array_element PostProcessMaterial
    (bind _returnvalue (`KismetMaterialLibrary.CreateDynamicMaterialInstance` _array_element))
    (`KismetArrayLibrary.Array_Add` (`local.MIDArray`) _returnvalue)
    (`KismetArrayLibrary.Array_Add` (`local.Array`) (make `WeightedBlendable` 1.0 _returnvalue)))
  (set `CameraComponent.PostProcessSettings` (make `PostProcessSettings` :`WeightedBlendables` (make `WeightedBlendables` (`local.Array`))) (`self.FirstPersonCamera`))
  (return (`local.MIDArray`)))

(fn `AddWeapon`
  (params (weaponClass :type "ActorComponent Class Reference"))
  (bind _returnvalue (`|AddComponentByClass` (`local.weaponClass`)))
  (bind _asskc_weapon (cast `/Game/Blueprints/Component/SkeletalMeshComponent/Weapon/SKC_Weapon` _returnvalue))
  (`KismetArrayLibrary.Array_Add` (`self.weaponList`) _asskc_weapon)
  (`SceneComponent.K2_AttachToComponent` _asskc_weapon (`self.SK_Arm`) "GripPoint" "KeepRelative" "KeepRelative" "KeepRelative" true))

(fn `CanJumpInternal`
  (returns (ReturnValue :type Boolean))
  (return true))

(fn `ChangeChromaticAberratioin`
  (params (AberrationScale :type "Float (single-precision)") (AberrationStrength :type "Float (double-precision)" :default 5.0))
  (bind _weightedblendables (`self.RecreatePPSettingsWithExistingPPMID` (`self.DilationPPArray`)))
  (set `CameraComponent.PostProcessSettings` (make `PostProcessSettings` :`SceneFringeIntensity` (* AberrationScale AberrationStrength) :`WeightedBlendables` _weightedblendables) (`self.FirstPersonCamera`)))

(fn `ChangeTargetLocalTimeScale`
  (params (newScale :type "Float (double-precision)"))
  (`/Game/Blueprints/MacroLibraries/BPML_TimeManagementActor.DilationTypeDo` (`self.controllerRef`)
    (:`NoDilation`
      (set `TimeSlippageModifier.localTimeScaleTarget` 1.0 (`self.TimeSlippageModifier`)))
    (:`WeakDilation`
      (set `TimeSlippageModifier.localTimeScaleTarget` (`self.WeakDilationTargetLocalTimeScale`) (`self.TimeSlippageModifier`)))
    (:`StrongDilation`
      (set `TimeSlippageModifier.localTimeScaleTarget` (`self.StrongDilationTargetLocalTimeScale`) (`self.TimeSlippageModifier`)))))

(fn `Death`
  (`KismetSystemLibrary.PrintString` "DeathPlayer")
  ;[0 1 0.5182] Audio State - player is dead
  (`AkGameplayStatics.SetState` "/Game/WwiseAudio/States/Default_Work_Unit/PlayerState/PlayerState-Dead.PlayerState-Dead"))

(fn `Get WeaponInArray`
  (params (index :type Integer))
  (returns (Output :type "/Game/Blueprints/Component/SkeletalMeshComponent/Weapon/SKC_Weapon Object Reference"))
  (return (`|GetArrayItem` (`self.weaponList`) index)))

(fn `GetDistanceFromGround`
  (params (MaxDistance :type "Float (double-precision)" :default 999.0))
  (bind _returnvalue (`self.K2_GetActorLocation`))
  (if (`NavMovementComponent.IsFalling` (`self.CharacterMovement`))
    (bind (_outhit _returnvalue_2) (`KismetSystemLibrary.LineTraceSingle` :`Start` _returnvalue :`End` (+ _returnvalue (* (`KismetMathLibrary.NegateVector` (`self.GetActorUpVector`)) MaxDistance)) :`TraceChannel` "TraceTypeQuery1" :`DrawTime` MaxDistance))
    (if _returnvalue_2
      (set `self.height_above_ground` (- (`.Distance` (`GameplayStatics.BreakHitResult` _outhit)) (`CapsuleComponent.GetScaledCapsuleHalfHeight` (`self.CapsuleComponent`))))
      (else
        (set `self.height_above_ground` MaxDistance)))
    (else
      (set `self.height_above_ground` 0.0))))

(fn `InitPostProcessMaterials`
  (`|ExecutionSequence`
    (:`then_0`
      (bind _materialinstancedynamic (`self.AddPostProcessMaterial` (`|MakeArray` (`self.PPMIDilation`) :!type "MaterialInterface Object Reference")))
      (set `self.DilationPPArray` _materialinstancedynamic))
    (:`then_1`
      (`MaterialInstanceDynamic.SetScalarParameterValue` (`|GetArrayItem` (`self.DilationPPArray`)) "Opacity" 0.0))))

(fn `InitStartWeapon`
  (set `self.actualWeapon` (`|GetArrayItem` (`self.weaponList`)))
  (for _index (range 1 (`KismetArrayLibrary.Array_Length` (`self.weaponList`)))
    (`/Game/Blueprints/Component/SkeletalMeshComponent/Weapon/SKC_Weapon.Hide` (`|GetArrayItem` (`self.weaponList`) _index))
    (`/Game/Blueprints/HUD/BP_PlayerHUD.ChangeWeapon` (`self.HUD`) (`self.indexWeapon`))))

(fn `RecreatePPSettingsWithExistingPPMID`
  (params (MIDArray :type "Array of MaterialInstanceDynamic Object Reference"))
  (returns (WeightedBlendables :type "WeightedBlendables Structure"))
  (locals (Array :type "Array of WeightedBlendable Structure"))
  (for _array_element MIDArray
    (`KismetArrayLibrary.Array_Add` (`local.Array`) (make `WeightedBlendable` 1.0 _array_element)))
  (return (make `WeightedBlendables` (`local.Array`))))

(fn `SetDilationPPScalarParameter`
  (params (ParameterName :type Name) (Value :type "Float (single-precision)"))
  (`MaterialInstanceDynamic.SetScalarParameterValue` (`|GetArrayItem` (`self.DilationPPArray`)) ParameterName Value))

(fn `SnapToRail`)

(fn `SwitchWeapon`
  (params (addIndexWeapon :type Integer))
  (locals (localActualWeapon :type "/Game/Blueprints/Component/SkeletalMeshComponent/Weapon/SKC_Weapon Object Reference"))
  (bind _controllerref (`self.controllerRef`))
  (bind _localactualweapon (`local.localActualWeapon`))
  (set `self.indexWeapon` (+ addIndexWeapon (`self.indexWeapon`)))
  (`/Game/Blueprints/Component/SkeletalMeshComponent/Weapon/SKC_Weapon.Hide` (`self.actualWeapon`))
  (if (not (`KismetArrayLibrary.Array_IsValidIndex` (`self.weaponList`) (`self.indexWeapon`)))
    (set `self.indexWeapon` (`KismetMathLibrary.SelectInt` (`KismetArrayLibrary.Array_LastIndex` (`self.weaponList`)) 0 (== (`KismetMathLibrary.SignOfInteger` (`self.indexWeapon`)) -1))))
  (set `local.localActualWeapon` (`self.Get WeaponInArray` (`self.indexWeapon`)))
  (`/Game/Blueprints/Component/SkeletalMeshComponent/Weapon/SKC_Weapon.Show` (`local.localActualWeapon`))
  (set `self.actualWeapon` _localactualweapon)
  (`PlayerController.ClientStopForceFeedback` _controllerref null "WeaponTrigger")
  (`PlayerController.K2_ClientPlayForceFeedback` _controllerref (`/Game/Blueprints/Component/SkeletalMeshComponent/Weapon/SKC_Weapon.TriggerFeedback` _localactualweapon) "WeaponTrigger" true false false)
  (`KismetSystemLibrary.PrintString` "Playing trigger FFB")
  (`/Game/Blueprints/HUD/BP_PlayerHUD.ChangeWeapon` (`self.HUD`) (`self.indexWeapon`))
  (`/Game/Blueprints/Component/SkeletalMeshComponent/Weapon/SKC_Weapon.UpdateOverheatingProgressBar` (`self.actualWeapon`)))

(fn `TakeDamage_`
  (params (targetActor :type "Actor Object Reference"))
  (`/Game/Blueprints/Component/ActorComponent/Damage/AC_TakeDamage.TakeDamage` (`self.TakeDamage`) (`self.GetComponentByClass` targetActor "/Game/Blueprints/Component/ActorComponent/Damage/AC_DoDamagePlayer.AC_DoDamagePlayer_C")))

(fn `UserConstructionScript`)