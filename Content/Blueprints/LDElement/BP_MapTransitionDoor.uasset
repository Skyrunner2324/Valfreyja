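; BP_MapTransitionDoor is a level element that stays locked until the wave manager reports that all waves are finished.
; On BeginPlay it caches the Target's collision mode, then hides it and disables its collision.
; The WavesFinished event from WaveManagerRef prints a debug message and reveals Target with its original collision restored.
; The map transition itself is not handled in this Blueprint's graphs.
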(event `self.ReceiveBeginPlay`
  (set `self.BaseCollisionMode` (`PrimitiveComponent.GetCollisionEnabled` (`self.Target`)))
  (`self.SetTargetVisibility` false))

(event `self.WaveManagerRef.WavesFinished`
  (`KismetSystemLibrary.PrintString` "Waves finished : door unlocked" true true (struct :`R` 1.0 :`A` 1.0))
  (`self.SetTargetVisibility` true))

(fn `SetTargetVisibility`
  (params (bVisible :type Boolean))
  (`PrimitiveComponent.SetCollisionEnabled` (`self.Target`) (select `bool` bVisible :`false` "NoCollision" :`true` (`self.BaseCollisionMode`)))
  (`SceneComponent.SetVisibility` (`self.Target`) (`local.bVisible`) true))

(fn `UserConstructionScript`
  (`parent.UserConstructionScript`))