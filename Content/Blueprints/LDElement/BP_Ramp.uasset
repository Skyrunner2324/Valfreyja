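; BP_Ramp is a level design element that propels the player character forward and upward when it enters the ramp's box collision.
; At BeginPlay it derives the launch direction by rotating the actor's forward vector a quarter turn.
; On overlap it raises the character's max walk speed by ForcePropulsion, then launches it with ForcePropulsion along that direction and ForceHeight vertically.
; The speed boost is not reset here.
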(event `self.ReceiveBeginPlay`
  (set `self.direction` (`KismetMathLibrary.GreaterGreater_VectorRotator` (`self.GetActorForwardVector`) (struct :`Yaw` -90.0))))

(event `self.BoxColision.OnComponentBeginOverlap`
  (params (OverlappedComponent :type "PrimitiveComponent Object Reference") (OtherActor :type "Actor Object Reference") (OtherComp :type "PrimitiveComponent Object Reference") (OtherBodyIndex :type Integer) (bFromSweep :type Boolean) (SweepResult :type "HitResult Structure (by ref)"))
  (bind _asbp_player_character (cast `/Game/Blueprints/Characters/BP_PlayerCharacter` OtherActor))
  (set `self.playerCharacter` _asbp_player_character)
  (`self.LaunchPlayer`))

(fn `LaunchPlayer`
  (bind (_direction_x _direction_y) (`KismetMathLibrary.BreakVector` (`self.direction`)))
  (set `CharacterMovementComponent.MaxWalkSpeed` (+ (`/Game/Blueprints/Characters/BP_PlayerCharacter.maxWalkSpeed` (`self.playerCharacter`)) (`self.forcePropulsion`)) (`Character.CharacterMovement` (`self.playerCharacter`)))
  (`Character.LaunchCharacter` (`self.playerCharacter`) (`KismetMathLibrary.MakeVector` (* (`self.forcePropulsion`) _direction_x) (* _direction_y (`self.forcePropulsion`)) (`self.forceHeight`)) false false))

(fn `UserConstructionScript`)