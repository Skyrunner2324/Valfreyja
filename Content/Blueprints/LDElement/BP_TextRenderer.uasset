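; BP_TextRenderer is a level-design actor that shows localized text in the world through a TextRender component.
; On BeginPlay it binds to GI_Global's localization culture change event and applies the current culture, then unbinds when destroyed.
; SetLocalizedText looks up the string from the actor's localization key and category for the given culture and writes it to the component.
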(event `self.ReceiveBeginPlay`
  (bind _asgi_global (cast `/Game/Blueprints/GameInstance/GI_Global` (`GameplayStatics.GetGameInstance`) :!pure true))
  (add `/Game/Blueprints/GameInstance/GI_Global.OnLocalizationCultureChange` _asgi_global (`|CreateDelegate` :!event `SetLocalizedText`))
  (`self.SetLocalizedText` (`/Game/Blueprints/GameInstance/GI_Global.currentCulture` _asgi_global)))

(event `self.ReceiveDestroyed`
  (remove `/Game/Blueprints/GameInstance/GI_Global.OnLocalizationCultureChange` (cast `/Game/Blueprints/GameInstance/GI_Global` (`GameplayStatics.GetGameInstance`) :!pure true) (`|CreateDelegate` :!event `SetLocalizedText`)))

(fn `SetLocalizedText`
  (params (culture :type "/Game/Enumerations/E_LocalizationCulture Enum" :default "NewEnumerator0"))
  (bind _value (`/Game/Blueprints/Libraries/FunctionLibraries/BFL_Localization.GetLocalizedText` (`self.localizationKey`) (`self.localizationCategory`) culture))
  (`TextRenderComponent.K2_SetText` (`self.TextRender`) _value))

(fn `UserConstructionScript`)