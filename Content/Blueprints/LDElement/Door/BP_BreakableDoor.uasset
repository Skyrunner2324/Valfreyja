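; Breakable door that shatters as a Chaos geometry collection when a player damage bullet hits its target component.
; Init passes a direction override to the child field actor, builds dynamic materials and applies the starting lock state.
; Locking shows the lock mesh, disables target collision and recolors materials.
; A hit enables physics, triggers the field, posts Wwise sound and state, and enables anchor box collision.
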(event `Init`
  (params (directionVectorOverrideField :type "Vector Structure") (startLocked :type Boolean) (akState :type "AkStateValue Object Reference"))
  (set `self.Direction Vector Override Field` directionVectorOverrideField)
  (set `self.startLocked` startLocked)
  (set `self.AkState` akState)
  (bind _asfs_field (cast `/Game/Blueprints/LDElement/Door/FS_Field` (`ChildActorComponent.ChildActor` (`self.Field`))))
  (set `self.field_` _asfs_field)
  (set `/Engine/EditorResources/FieldNodes/FS_MasterField.DIrectionalVectorOveride` (`self.Direction Vector Override Field`) (`self.field_`))
  (`self.SetMaterialDynamic`)
  (`self.Lock` (`self.startLocked`)))

(event `self.Target.OnComponentHit`
  (params (HitComponent :type "PrimitiveComponent Object Reference") (OtherActor :type "Actor Object Reference") (OtherComp :type "PrimitiveComponent Object Reference") (NormalImpulse :type "Vector Structure") (Hit :type "HitResult Structure (by ref)"))
  (cast `/Game/Blueprints/Projectiles/Bullet/PlayerBullet/BP_BulletPlayerDoDamage` OtherActor)
  (`self.OnHitTarget`)
  (`self.hitTarget`))

(fn `DestroyDoor`
  (`/Engine/EditorResources/FieldNodes/FS_MasterField.CE_Trigger` (`self.field_`))
  (set `self.destroy?` true))

(fn `Lock`
  (params (lock :type Boolean))
  (`SceneComponent.SetVisibility` (`self.SM_Door_Lock`) (`local.lock`) false)
  (`SceneComponent.SetHiddenInGame` (`self.SM_Door_Lock`) (not (`local.lock`)) false)
  (`PrimitiveComponent.SetCollisionEnabled` (`self.Target`) (select `bool` (`local.lock`) :`false` "QueryAndPhysics" :`true` "NoCollision" :!type "ECollisionEnabled Enum"))
  (`self.SetColorMaterial` (select `bool` (`local.lock`) :`false` (`self.unLockColor`) :`true` (`self.lockColor`))))

(fn `OnHitTarget`
  (`PrimitiveComponent.SetCollisionEnabled` (`self.Target`) "NoCollision")
  (`self.SetActorTickEnabled` false)
  (`PrimitiveComponent.SetSimulatePhysics` (`self.instanceGeometryComponent`) true)
  (`AkGameplayStatics.PostEvent` "/Game/WwiseAudio/Events/Environment/Door_Destroy.Door_Destroy" self)
  (`AkGameplayStatics.SetState` (`self.AkState`))
  (`self.DestroyDoor`)
  (for _array_element (`self.anchorFields`)
    (bind _asanchor (cast `/Game/Blueprints/LDElement/Door/Anchor` _array_element))
    (`PrimitiveComponent.SetCollisionEnabled` (`/Engine/EditorResources/FieldNodes/FS_AnchorField_Generic.Box` _asanchor) "QueryAndPhysics")))

(fn `SetColorMaterial`
  (params (newColor :type "LinearColor Structure"))
  (for _array_element (`self.dynamicMaterials`)
    (`MaterialInstanceDynamic.SetVectorParameterValue` _array_element "Color" newColor)))

(fn `SetMaterialDynamic`
  (locals (localActualMesh :type "StaticMeshComponent Object Reference") (localActualIndex :type Integer))
  (bind _output_get (set `self.staticMeshsComponents` (`|MakeArray` (`self.SM_Door_pillars`) (`self.SM_Door_Lock`))))
  (for (_array_element _array_index) _output_get
    (set `local.localActualMesh` _array_element)
    (set `local.localActualIndex` _array_index)
    (for _array_element_2 (`MeshComponent.GetMaterials` (`local.localActualMesh`))
      (bind _returnvalue (`KismetMaterialLibrary.CreateDynamicMaterialInstance` _array_element_2))
      (`KismetArrayLibrary.Array_Add` (`self.dynamicMaterials`) _returnvalue)
      (`PrimitiveComponent.SetMaterial` (`local.localActualMesh`) (`local.localActualIndex`) _returnvalue))
    (for (_array_element_3 _array_index_2) (`MeshComponent.GetMaterials` (`self.instanceGeometryComponent`))
      (if (not (>= _array_index_2 2))
        (bind _returnvalue_2 (`KismetMaterialLibrary.CreateDynamicMaterialInstance` _array_element_3))
        (`KismetArrayLibrary.Array_Add` (`self.dynamicMaterials`) _returnvalue_2)
        (`PrimitiveComponent.SetMaterial` (`self.instanceGeometryComponent`) (`local.localActualIndex`) _returnvalue_2)))))

(fn `UserConstructionScript`
  (`parent.UserConstructionScript`)
  (set `/Game/Blueprints/Component/ActorComponent/AC_AimTarget.targetToAim` (`self.Target`) (`self.AC_AimTarget`))
  (`GeometryCollectionComponent.SetRestCollection` (`self.instanceGeometryComponent`) (`self.Rest Collection In`))
  (set `GeometryCollectionComponent.ObjectType` "Chaos_Object_Sleeping" (`self.instanceGeometryComponent`))
  (`SceneComponent.K2_SetRelativeLocationAndRotation` (`self.instanceGeometryComponent`) (0.0 0.0 -350.0) (struct :`Yaw` -90.0) false false))