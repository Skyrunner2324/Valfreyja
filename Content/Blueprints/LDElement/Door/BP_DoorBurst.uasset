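; BP_DoorBurst is a door element that counts hits toward a target within a limited time window.
; GetDamaged enables Tick, increments the hit count and compares it to HitTarget, though that branch and DisableActor are empty here.
; Tick accumulates TimeSlippageModifier's local delta time, so the window follows managed time, then clears the count and disables itself when time runs out.
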(event `self.ReceiveBeginPlay`
  (set `self.playerController` (cast `/Game/Blueprints/Controller/BP_PlayerController` (`GameplayStatics.GetPlayerController` 0) :!pure true)))

(event `self.ReceiveTick`
  (params (DeltaSeconds :type "Float (single-precision)"))
  (bind _output_get (set `self.elapsedCompletionTime` (+ (`TimeSlippageModifier.localManagedDeltaTime` (`self.TimeSlippageModifier`)) (`self.elapsedCompletionTime`))))
  (if (>= _output_get (`self.timeToComplete`))
    (set `self.hitCount` 0)
    (set `self.elapsedCompletionTime` 0.0)
    (`self.SetActorTickEnabled` false)))

(fn `GetDamaged`
  (`self.SetActorTickEnabled` true)
  (bind _result (`/Engine/EditorBlueprintResources/StandardMacros.IncrementInt` (`self.hitCount`))
    (:`  `
      (if (>= _result (`self.hitTarget`))
        _))))

(fn `UserConstructionScript`
  (`parent.UserConstructionScript`))