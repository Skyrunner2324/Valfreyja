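; Shootable door level element that breaks when a player damage bullet hits its Target component, which is registered with the aim-target component.
; A hit disables the target's collision and actor tick, posts Wwise destroy audio and triggers the child-actor field system.
; BeginPlay overrides that field's direction vector, with debug prints, and sets lock-mesh visibility from StartLocked.
; OnReset restores collision, visibility and tick; older breakable-wall setup is left unwired.
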(event `self.ReceiveBeginPlay`
  (`self.Lock` (`self.startLocked?`))
  (bind _asfs_field (cast `/Game/Blueprints/LDElement/Door/FS_Field` (`ChildActorComponent.ChildActor` (`self.FS_Field2`))))
  (`KismetSystemLibrary.PrintString` (`KismetStringLibrary.Conv_VectorToString` (`/Engine/EditorResources/FieldNodes/FS_MasterField.DIrectionalVectorOveride` _asfs_field)) true true (struct :`G` 0.66 :`B` 1.0 :`A` 1.0) 200.0)
  (set `/Engine/EditorResources/FieldNodes/FS_MasterField.DIrectionalVectorOveride` (`self.directionVectorOverrideField`) _asfs_field)
  (`KismetSystemLibrary.PrintString` (`KismetStringLibrary.Concat_StrStr` "After: " (`KismetStringLibrary.Conv_VectorToString` (`/Engine/EditorResources/FieldNodes/FS_MasterField.DIrectionalVectorOveride` _asfs_field))) true true (struct :`R` 1.0 :`A` 1.0) 200.0))

(event `self.Target.OnComponentHit`
  (params (HitComponent :type "PrimitiveComponent Object Reference") (OtherActor :type "Actor Object Reference") (OtherComp :type "PrimitiveComponent Object Reference") (NormalImpulse :type "Vector Structure") (Hit :type "HitResult Structure (by ref)"))
  (cast `/Game/Blueprints/Projectiles/Bullet/PlayerBullet/BP_BulletPlayerDoDamage` OtherActor)
  (`self.OnHitTarget`))

(event `self.K2_OnReset`
  (`PrimitiveComponent.SetCollisionEnabled` (`self.Target`) "QueryAndPhysics")
  (`self.SetActorHiddenInGame` false)
  (`self.SetActorEnableCollision` true)
  (`self.SetActorTickEnabled` true))

(fn `DisableActor`
  (`PrimitiveComponent.SetCollisionEnabled` (`self.Target`) "NoCollision")
  (`self.SetActorTickEnabled` false))

(fn `Lock`
  (params (lock :type Boolean))
  (`SceneComponent.SetVisibility` (`self.SM_Door_Lock`) (`local.lock`) false)
  (`SceneComponent.SetHiddenInGame` (`self.SM_Door_Lock`) (not (`local.lock`)) false))

(fn `OnHitTarget`
  (`self.DisableActor`)
  (`AkGameplayStatics.PostEvent` "/Game/WwiseAudio/Events/Environment/Door_Destroy.Door_Destroy" self)
  (`AkGameplayStatics.SetState` (`self.AkState`))
  (bind _asfs_master_field (cast `/Engine/EditorResources/FieldNodes/FS_MasterField` (`ChildActorComponent.ChildActor` (`self.FS_Field2`))))
  (`/Engine/EditorResources/FieldNodes/FS_MasterField.CE_Trigger` _asfs_master_field))

(fn `SetUnLockParameterShader`
  (params (Value :type Boolean))
  (`/Game/Blueprints/Enviro/BP_Breakable_wall.SetUnLockParameterShader` (`self.breakableWall`) (`local.Value`)))

(fn `UserConstructionScript`
  (set `/Game/Blueprints/Component/ActorComponent/AC_AimTarget.targetToAim` (`self.Target`) (`self.AC_AimTarget`)))