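; Checkpoint actor that sets the player's respawn location and facing the first time they overlap its trigger, until OnReset re-arms it.
; It derives both from a local SpawnPoint and an angle offset from actor forward, previewed by a construction-script debug arrow.
; On activation it notifies the player's HUD and, if RegenHealth is set and health isn't full, spawns an instant BP_RegenShield power-up to heal.
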(event `self.Trigger Area.OnComponentBeginOverlap`
  (params (OverlappedComponent :type "PrimitiveComponent Object Reference") (OtherActor :type "Actor Object Reference") (OtherComp :type "PrimitiveComponent Object Reference") (OtherBodyIndex :type Integer) (bFromSweep :type Boolean) (SweepResult :type "HitResult Structure (by ref)"))
  (bind _respawn (`/Game/Blueprints/Characters/BP_PlayerCharacter.Respawn` (`self.playerCharacter`)))
  (bind _returnvalue (not (`/Game/Blueprints/Component/ActorComponent/Damage/AC_TakeDamage.IsHealthFull` (`/Game/Blueprints/Characters/BP_PlayerCharacter.TakeDamage` (`self.playerCharacter`)))))
  (if (not (`self.takeCheckpoint`))
    (bind _asbp_player_character (cast `/Game/Blueprints/Characters/BP_PlayerCharacter` OtherActor))
    (set `self.playerCharacter` _asbp_player_character)
    (`/Game/Blueprints/Component/ActorComponent/Player/AC_Respawn.SetExactSpawnLocation` _respawn (`KismetMathLibrary.TransformLocation` (`self.GetTransform`) (`self.spawnPoint`)))
    (set `/Game/Blueprints/Component/ActorComponent/Player/AC_Respawn.currentSpawnRotation` (`self.GetLookAtRotation`) _respawn)
    (set `self.takeCheckpoint` true)
    ;[1 1 1] Event Hud Checkpoint registered
    (`/Game/Blueprints/HUD/BP_PlayerHUD.CheckpointRegistered` (`/Game/Blueprints/Characters/BP_PlayerCharacter.HUD` (`self.playerCharacter`)) _returnvalue)
    (if (and (`self.regenHealth`) _returnvalue)
      ;[1 1 1] Regen health
      (`|SpawnActorFromClass` "/Game/Blueprints/PowerUps/BP_RegenShield.BP_RegenShield_C" (`KismetMathLibrary.MakeTransform` (0.0 0.0 0.0)) "Undefined" "MultiplyWithRoot" null 0.1 0.5 100.0 true false true false 5.0 true false 50.0 null))))

(event `self.K2_OnReset`
  (set `self.takeCheckpoint` false))

(fn `GetLookAtRotation`
  (returns (rotation :type "Rotator Structure"))
  (bind _returnvalue (`KismetMathLibrary.TransformLocation` (`self.GetTransform`) (`self.spawnPoint`)))
  (return (`KismetMathLibrary.FindLookAtRotation` _returnvalue (+ _returnvalue (`KismetMathLibrary.RotateAngleAxis` (`self.GetActorForwardVector`) (`self.spawnDirectionAngle`) (0.0 0.0 1.0))))))

(fn `GetSpawnLocation`)

(fn `UserConstructionScript`
  (bind _returnvalue (`KismetMathLibrary.TransformLocation` (`self.GetTransform`) (`self.spawnPoint`)))
  (`KismetSystemLibrary.DrawDebugArrow` _returnvalue (+ _returnvalue (* (`self.GetLookAtRotation`) 150)) 50.0 (struct :`R` 1.0 :`A` 1.0) 3.0 2.0))