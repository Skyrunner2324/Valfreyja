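; BP_TriggerOpenPortal is a trigger volume that animates a portal opening the first time its box is overlapped.
; The OpenPortal timeline, scaled to TimeToOpen, grows Niagara float parameters on the separate Portal and RunePortal effects from their start sizes by configurable amounts.
; An AlreadyPassed flag blocks retriggering until OnReset clears it and restores the start sizes.
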(event `self.ReceiveBeginPlay`
  (`self.SetPortalVariable` (`self.startSizePortal`) (`self.startSizeRunePortal`))
  (`TimelineComponent.SetPlayRate` (`self.OpenPortal`) (/ 1.0 (`self.timeToOpen`))))

(event `self.Box.OnComponentBeginOverlap`
  (params (OverlappedComponent :type "PrimitiveComponent Object Reference") (OtherActor :type "Actor Object Reference") (OtherComp :type "PrimitiveComponent Object Reference") (OtherBodyIndex :type Integer) (bFromSweep :type Boolean) (SweepResult :type "HitResult Structure (by ref)"))
  (if (not (`self.alreadyPassed`))
    (`TimelineComponent.PlayFromStart` (`self.OpenPortal`))
    (set `self.alreadyPassed` true)))

(event `self.K2_OnReset`
  (set `self.alreadyPassed` false)
  (`self.SetPortalVariable` (`self.startSizePortal`) (`self.startSizeRunePortal`)))

(fn `SetPortalVariable`
  (params (InValue :type "Float (single-precision)") (InValue1 :type "Float (single-precision)"))
  (`NiagaraComponent.SetVariableFloat` (`NiagaraActor.NiagaraComponent` (`self.portal`)) "sizePortal" InValue)
  (`NiagaraComponent.SetVariableFloat` (`NiagaraActor.NiagaraComponent` (`self.runePortal`)) "largeRadius" InValue1))

(fn `UserConstructionScript`)