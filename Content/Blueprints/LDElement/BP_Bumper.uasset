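; BP_Bumper is a level element that launches the player along its mesh's up vector on overlap and awards score through BP_ScoreBoard.
; The bump stops Slide and Dash and resets Dash before the launch overrides the player's velocity.
; It then drives Wwise bump and wind sounds, adds dilation and starts a point-sequence counter on the player controller, and plays controller rumble and a wing animation.
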(event `self.ReceiveBeginPlay`
  (bind _returnvalue (`GameplayStatics.GetActorOfClass` "/Game/Blueprints/Scoring/BP_ScoreBoard.BP_ScoreBoard_C"))
  (set `self.ScoreRef` _returnvalue))

(event `self.Colision.OnComponentBeginOverlap`
  (params (OverlappedComponent :type "PrimitiveComponent Object Reference") (OtherActor :type "Actor Object Reference") (OtherComp :type "PrimitiveComponent Object Reference") (OtherBodyIndex :type Integer) (bFromSweep :type Boolean) (SweepResult :type "HitResult Structure (by ref)"))
  (bind _dash (`/Game/Blueprints/Characters/BP_PlayerCharacter.Dash` (`self.playerCharacter`)))
  (bind _asbp_player_character (cast `/Game/Blueprints/Characters/BP_PlayerCharacter` OtherActor))
  (set `self.playerCharacter` _asbp_player_character)
  (`/Game/Blueprints/Scoring/BP_ScoreBoard.AddScore` (`self.ScoreRef`) 100)
  (`/Game/Blueprints/Component/ActorComponent/Player/AC_Ability.StopAbility` (`/Game/Blueprints/Characters/BP_PlayerCharacter.Slide` (`self.playerCharacter`)))
  (`/Game/Blueprints/Component/ActorComponent/Player/AC_Ability.StopAbility` _dash)
  (`/Game/Blueprints/Component/ActorComponent/Player/AC_Dash.ResetDash` _dash)
  (`Character.LaunchCharacter` (`self.playerCharacter`) (* (`SceneComponent.GetUpVector` (`self.SM_Bumper_3x1`)) (`self.LaunchForce`)) true true)
  (`AkGameplayStatics.PostEvent` "/Game/WwiseAudio/Events/Player/Movement/SX_player_bumper.SX_player_bumper")
  ;[0.03957 1 0.1456] Sound State
  (`AkGameplayStatics.SetRTPCValue` "/Game/WwiseAudio/Game_Parameters/Default_Work_Unit/RTPC_PlayerMovement.RTPC_PlayerMovement" 4.5)
  (`AkGameplayStatics.PostEvent` "/Game/WwiseAudio/Events/Hoverboots/Hoverboots/Stop_wind_blast.Stop_wind_blast")
  (`AkGameplayStatics.PostEvent` "/Game/WwiseAudio/Events/Hoverboots/Hoverboots/Play_wind_blast.Play_wind_blast")
  ;[1 1 1] Add dilation
  (bind _asbp_player_controller (cast `/Game/Blueprints/Controller/BP_PlayerController` (`GameplayStatics.GetPlayerController` 0)))
  (`/Game/Blueprints/Controller/BP_PlayerController.AddDilation` _asbp_player_controller (`self.numberToAddDilation`))
  (`/Game/Blueprints/Controller/BP_PlayerController.StartCounterSequencePoint` _asbp_player_controller (`self.numberToAddPointSequence`))
  (`PlayerController.K2_ClientPlayForceFeedback` _asbp_player_controller "/Game/Feedbacks/LD_Elements/FFB_BumperVibration.FFB_BumperVibration" "None" false true false)
  (bind _asbp_player_character_2 (cast `/Game/Blueprints/Characters/BP_PlayerCharacter` (`GameplayStatics.GetPlayerCharacter` 0)))
  (`/Game/Blueprints/Characters/BP_PlayerCharacter.PlayAnimOnWings` _asbp_player_character_2 "/Game/Animations/Character/Wings/AM_Wings_Bump.AM_Wings_Bump" true true))

(fn `UserConstructionScript`)