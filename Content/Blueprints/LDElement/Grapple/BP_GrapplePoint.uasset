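; Grapple point actor that the player's grapple system can target, with a widget indicator for its locked state.
; The detection sphere toggles the indicator and Tick, which hides it while unlocked if out of line of sight or off screen.
; The can-use sphere broadcasts overlap begin and end, while the stop collision ends the player's grapple ability when the point is in use.
; Lock changes trigger a grapple animation call; the texture-swap code is disconnected.
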(event `self.ReceiveBeginPlay`
  (set `self.lock` false)
  (`self.SetActorTickEnabled` false)
  (bind _aswg_grapple_lock (cast `/Game/UI/Grapple/WG_GrappleLock` (`WidgetComponent.GetUserWidgetObject` (`self.WG_Indicator`))))
  (set `self.WG_GrappleLock` _aswg_grapple_lock))

(event `self.SphereCanUseGrapple.OnComponentBeginOverlap`
  (params (OverlappedComponent :type "PrimitiveComponent Object Reference") (OtherActor :type "Actor Object Reference") (OtherComp :type "PrimitiveComponent Object Reference") (OtherBodyIndex :type Integer) (bFromSweep :type Boolean) (SweepResult :type "HitResult Structure (by ref)"))
  ;[1 1 1] Overlap Can Use Grapple
  (`self.OverlapEvent` self))

(event `self.SphereCanUseGrapple.OnComponentEndOverlap`
  (params (OverlappedComponent :type "PrimitiveComponent Object Reference") (OtherActor :type "Actor Object Reference") (OtherComp :type "PrimitiveComponent Object Reference") (OtherBodyIndex :type Integer))
  ;[1 1 1] Overlap Can Use Grapple
  (`self.EndOverlapEvent` self))

(event `self.CollisionStopAbility.OnComponentBeginOverlap`
  (params (OverlappedComponent :type "PrimitiveComponent Object Reference") (OtherActor :type "Actor Object Reference") (OtherComp :type "PrimitiveComponent Object Reference") (OtherBodyIndex :type Integer) (bFromSweep :type Boolean) (SweepResult :type "HitResult Structure (by ref)"))
  ;[1 1 1] CheckColision With GrapplePoint
  (if (`self.isUsed`)
    (bind _asbp_player_character (cast `/Game/Blueprints/Characters/BP_PlayerCharacter` OtherActor))
    (`/Game/Blueprints/Component/ActorComponent/Player/AC_Ability.StopAbility` (`/Game/Blueprints/Characters/BP_PlayerCharacter.GrappleSystem` _asbp_player_character))))

(event `self.DetectionSphere.OnComponentBeginOverlap`
  (params (OverlappedComponent :type "PrimitiveComponent Object Reference") (OtherActor :type "Actor Object Reference") (OtherComp :type "PrimitiveComponent Object Reference") (OtherBodyIndex :type Integer) (bFromSweep :type Boolean) (SweepResult :type "HitResult Structure (by ref)"))
  ;[1 1 1] Overlap detection sphere
  (`self.ChangeLockWidget` false)
  (`self.SetActorTickEnabled` true))

(event `self.DetectionSphere.OnComponentEndOverlap`
  (params (OverlappedComponent :type "PrimitiveComponent Object Reference") (OtherActor :type "Actor Object Reference") (OtherComp :type "PrimitiveComponent Object Reference") (OtherBodyIndex :type Integer))
  ;[1 1 1] Overlap detection sphere
  (`self.ChangeLockWidget` false true)
  (`self.SetActorTickEnabled` false))

(event `self.ReceiveTick`
  (params (DeltaSeconds :type "Float (single-precision)"))
  ;[1 1 1] Detect if grapple is behind object
  (`self.DetectBehindObject`))

(fn `ChangeLockWidget`
  (params (localLock :type Boolean) (hiddenInGame :type Boolean))
  (`SceneComponent.SetHiddenInGame` (`self.WG_Indicator`) hiddenInGame false)
  (set `self.lock` (`local.localLock`))
  (`self.GrappleAnim`))

(fn `ChangeMaterial`
  (params (Material :type "MaterialInterface Object Reference"))
  (`PrimitiveComponent.SetMaterial` (`self.StaticMesh`) 0 Material))

(fn `DetectBehindObject`
  (if (not (`self.lock`))
    (bind _asbp_player_character (cast `/Game/Blueprints/Characters/BP_PlayerCharacter` (`GameplayStatics.GetPlayerCharacter` 0)))
    (`SceneComponent.SetHiddenInGame` (`self.WG_Indicator`) (not (and (`Controller.LineOfSightTo` (`GameplayStatics.GetPlayerController` 0) self (0.0 0.0 0.0) false) (`.bIsOnScreen` (`HUDBlueprintLibrary.FindScreenEdgeLocationForWorldLocation` (`self.K2_GetActorLocation`) (`/Game/Blueprints/Component/ActorComponent/Player/AC_GrappleSystem.edgePercentRenderAtScreen` (`/Game/Blueprints/Characters/BP_PlayerCharacter.GrappleSystem` _asbp_player_character)) (0.5 0.5))))) false)))

(fn `GetOpacityTextureGrapplePoint`
  (params (localLock :type Boolean))
  (returns (ReturnValue :type "Float (double-precision)"))
  (return (select `bool` localLock :`false` (`self.opacityNotLock`) :`true` (`self.opacityIsLock`))))

(fn `GetTextureGrapplePoint`
  (params (localLock :type Boolean))
  (returns (ReturnValue :type "Texture2D Object Reference"))
  (return (select `bool` localLock :`false` (`self.textureClose`) :`true` (`self.textureLock`))))

(fn `Lock_`
  (`self.ChangeLockWidget` true))

(fn `SetTextureWIdgetIndicator`
  (params (Texture :type "Texture2D Object Reference") (newOpacity :type "Float (single-precision)")))

(fn `UserConstructionScript`)