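; Grapple point, apparently for enemies, that tracks the player's grapple system and broadcasts when a grapple starts and ends.
; Overlapping the stop collision during a grapple stops the ability and clears the tracked system.
; Enable and Disable toggle query collision on its three collision components; Disable skips an active grapple unless forced, in which case it stops the ability without broadcasting the end event.
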(event `GrappleStart`
  (params (grappleSystem :type "/Game/Blueprints/Component/ActorComponent/Player/AC_GrappleSystem Object Reference"))
  (`/Engine/EditorBlueprintResources/StandardMacros.IsValid` grappleSystem
    (:`Is Valid`
      (set `self.playerGrappling` grappleSystem)
      (`self.OnGrappleStart`))))

(event `self.CollisionStopAbility.OnComponentBeginOverlap`
  (params (OverlappedComponent :type "PrimitiveComponent Object Reference") (OtherActor :type "Actor Object Reference") (OtherComp :type "PrimitiveComponent Object Reference") (OtherBodyIndex :type Integer) (bFromSweep :type Boolean) (SweepResult :type "HitResult Structure (by ref)"))
  (bind _playergrappling (`self.playerGrappling`))
  (`/Engine/EditorBlueprintResources/StandardMacros.IsValid` _playergrappling ; If player isn't grappling, do nothing
    (:`Is Valid`
      (`/Game/Blueprints/Component/ActorComponent/Player/AC_Ability.StopAbility` _playergrappling)
      (set `self.playerGrappling` null)
      (`self.OnGrappleEnd`))))

(fn `Disable`
  (params (forceDisable :type Boolean))
  (bind _playergrappling (`self.playerGrappling`))
  (if (or forceDisable (not (`KismetSystemLibrary.IsValid` _playergrappling)))
    (`PrimitiveComponent.SetCollisionEnabled` (`self.SphereCanUseGrapple`) "NoCollision")
    (`PrimitiveComponent.SetCollisionEnabled` (`self.CollisionStopAbility`) "NoCollision")
    (`PrimitiveComponent.SetCollisionEnabled` (`self.Sphere`) "NoCollision")
    (`/Engine/EditorBlueprintResources/StandardMacros.IsValid` _playergrappling
      (:`Is Valid`
        (`/Game/Blueprints/Component/ActorComponent/Player/AC_Ability.StopAbility` _playergrappling)))))

(fn `Enable`
  (`PrimitiveComponent.SetCollisionEnabled` (`self.SphereCanUseGrapple`) "QueryOnly")
  (`PrimitiveComponent.SetCollisionEnabled` (`self.CollisionStopAbility`) "QueryOnly")
  (`PrimitiveComponent.SetCollisionEnabled` (`self.Sphere`) "QueryOnly"))

(fn `UserConstructionScript`
  (`parent.UserConstructionScript`))