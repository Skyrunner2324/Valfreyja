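; Laser trap spawner that places moving, rotating or cycling laser actors in the level.
; It pulls lasers from an actor pool, once at BeginPlay if enabled and then repeatedly at the emission rate, and initializes each with its motion, scale and activation settings.
; The emission timer uses the player's time-slippage delta time rather than Tick's.
; ActivateTrap toggles every tracked laser and the manager's own tick.
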(event `self.ReceiveBeginPlay`
  (if (`self.spawnTrapAtStart`)
    (`self.SpawnTrap`)))

(event `self.ReceiveTick`
  (params (DeltaSeconds :type "Float (single-precision)"))
  (if (> (`self.emissionRate`) 0.0)
    (set `self.counterEmissionRate` (+ (`self.counterEmissionRate`) (`TimeSlippageModifier.localManagedDeltaTime` (`/Game/Blueprints/Characters/BP_PlayerCharacter.TimeSlippageModifier` (cast `/Game/Blueprints/Characters/BP_PlayerCharacter` (`GameplayStatics.GetPlayerCharacter` 0) :!pure true)))))
    (if (>= (`self.counterEmissionRate`) (`self.emissionRate`))
      (set `self.counterEmissionRate` 0.0)
      (`self.SpawnTrap`))))

(fn `ActivateTrap`
  (params (ActivateTrap :type Boolean) (colision :type "ECollisionEnabled Enum" :default "NoCollision"))
  (for _array_element (`self.trap`)
    (`/Game/Blueprints/LDElement/Trap/BP_Trap.ActivateTrap` _array_element (`local.ActivateTrap`) (`local.colision`)))
  (`self.SetActorTickEnabled` (`local.ActivateTrap`)))

(fn `SpawnTrap`
  (locals (localCurrentLaserActor :type "/Game/Blueprints/LDElement/Trap/BP_LaserActor_ Object Reference"))
  (bind _actorpooled (`/Game/Blueprints/Libraries/FunctionLibraries/BFL_GetActorPooled.GetActorPooled` (`self.trapClass`) (`self.K2_GetActorLocation`) (`SceneComponent.K2_GetComponentRotation` (`self.arrowStartRotation`))))
  (bind _asbp_non_destructible_laser_actor (cast `/Game/Blueprints/LDElement/Trap/BP_LaserActor_` _actorpooled))
  (set `local.localCurrentLaserActor` _asbp_non_destructible_laser_actor)
  (`KismetArrayLibrary.Array_Add` (`self.trap`) (`local.localCurrentLaserActor`))
  (`/Game/Blueprints/LDElement/Trap/BP_LaserActor_.Init` (`local.localCurrentLaserActor`) (`self.speed`) (`self.trapMoving`) (`self.trapGoBack?`) (`self.scaleTrap`) (`KismetMathLibrary.TransformLocation` (`self.GetTransform`) (`self.targetLocation`)) (`self.speedRotation`) (`self.cyclicRotation`) (`self.doActivation`) (`self.activationTime`) (`self.deactivationTime`)))

(fn `UserConstructionScript`
  (`parent.UserConstructionScript`))