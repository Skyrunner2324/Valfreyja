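; BP_LaserActor is a laser trap element that can travel along its forward axis and spins as it goes.
; Init sets scale, speed, spin and movement flags, and derives the target from distance and forward vector.
; Tick sweeps it toward the target using the time-slippage-managed delta time, then reverses or calls Death on arrival.
; Spin accumulates as quaternions over the start rotation each frame, independent of delta time.
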(event `self.ReceiveTick`
  (params (DeltaSeconds :type "Float (single-precision)"))
  (`|ExecutionSequence`
    (:`then_0`
      (if (`self.isMoving`)
        (set `self.currentLocation` (`KismetMathLibrary.VInterpTo_Constant` (`self.currentLocation`) (`self.targetLocation`) (`TimeSlippageModifier.localManagedDeltaTime` (`self.Time Slippage Modifier`)) (`self.speed`)))
        (`self.K2_SetActorLocation` (`self.currentLocation`) true)
        (if (== (`self.currentLocation`) (`self.targetLocation`) :`ErrorTolerance` 0.001)
          (if (`self.goBack`)
            (set `self.targetLocation` (`self.startLocation`))
            (set `self.startLocation` (`self.currentLocation`))
            (else
              (`self.Death`))))))
    (:`then_1`
      (set `self.currentRotation` (`KismetMathLibrary.Quat_Rotator` (* (`self.currentRotation`) (`self.rotationVisse`))))
      (`self.K2_SetActorRotation` (`KismetMathLibrary.Quat_Rotator` (* (`self.currentRotation`) (`self.startRotation`)))))))

(fn `Init`
  (params (distanceToTravel :type "Float (double-precision)") (speed :type "Float (double-precision)") (isMoving :type Boolean) (goBack :type Boolean) (scale :type "Vector Structure") (rotationVisse :type "Rotator Structure"))
  (set `self.rotationVisse` rotationVisse)
  (`self.SetActorScale3D` (`local.scale`))
  (set `self.goBack` (`local.goBack`))
  (set `self.isMoving` (`local.isMoving`))
  (set `self.distance` (`local.distanceToTravel`))
  (set `self.speed` (`local.speed`))
  (set `self.currentLocation` (`self.K2_GetActorLocation`))
  (set `self.startLocation` (`self.currentLocation`))
  (`self.SetTargetLocation`)
  (set `self.startRotation` (`KismetMathLibrary.Conv_RotatorToQuaternion` (`self.K2_GetActorRotation`))))

(fn `SetTargetLocation`
  (set `self.targetLocation` (+ (`self.currentLocation`) (* (`self.GetActorForwardVector`) (`self.distance`)))))

(fn `UserConstructionScript`)