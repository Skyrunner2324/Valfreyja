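; BP_DestructibleTrap is a level-design trap that takes damage from actors able to damage traps.
; Overlaps on its TrigerTakeDamage component check the other actor for an AC_DoDamageTrap component and, if found, pass it to ACTakeDamage as the damage source.
; On BeginPlay it runs the parent logic and binds an event to ACTakeDamage's death, though the bound handler is not shown.
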(event `self.ReceiveBeginPlay`
  (`parent.ReceiveBeginPlay`)
  (add `/Game/Blueprints/Component/ActorComponent/Damage/AC_TakeDamage.Death` (`self.AC_TakeDamage`) (`|CreateDelegate` :!event `Death`)))

(event `self.TrigerTakeDamage.OnComponentBeginOverlap`
  (params (OverlappedComponent :type "PrimitiveComponent Object Reference") (OtherActor :type "Actor Object Reference") (OtherComp :type "PrimitiveComponent Object Reference") (OtherBodyIndex :type Integer) (bFromSweep :type Boolean) (SweepResult :type "HitResult Structure (by ref)"))
  (`self.TakeDamage` OtherActor))

(fn `TakeDamage`
  (params (actor :type "Actor Object Reference"))
  (bind _returnvalue (`self.GetComponentByClass` actor "/Game/Blueprints/Component/ActorComponent/Damage/AC_DoDamageTrap.AC_DoDamageTrap_C"))
  (`/Engine/EditorBlueprintResources/StandardMacros.IsValid` _returnvalue
    (:`Is Valid`
      (`/Game/Blueprints/Component/ActorComponent/Damage/AC_TakeDamage.TakeDamage` (`self.AC_TakeDamage`) _returnvalue 0.0 false))))

(fn `UserConstructionScript`
  (`parent.UserConstructionScript`))