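; Laser trap actor that can rotate, travel to a target point and cycle on and off.
; Init supplies its settings; while active, Tick rotates it and optionally moves it at constant speed, then reverses or calls Death on arrival.
; Optional timers toggle the trap and its collision through ActivateTrap.
; Motion and timers use the TimeSlippageModifier's local delta time, so they follow its managed time.
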(event `self.ReceiveTick`
  (params (DeltaSeconds :type "Float (single-precision)"))
  (set `self.deltaTime` (`TimeSlippageModifier.localManagedDeltaTime` (`self.Time Slippage Modifier`)))
  (`|ExecutionSequence`
    (:`then_0`
      (if (`self.isActive`)
        ;[1 1 1] Set Rotation and Location
        (`self.SetRotation`)
        (if (`self.isMoving`)
          (set `self.currentLocation` (`KismetMathLibrary.VInterpTo_Constant` (`self.currentLocation`) (`self.targetLocation`) (`self.deltaTime`) (`self.speed`)))
          (`self.K2_SetActorLocation` (`self.currentLocation`) true)
          (if (== (`self.currentLocation`) (`self.targetLocation`) :`ErrorTolerance` 0.001)
            (if (`self.goBack`)
              (set `self.targetLocation` (`self.startLocation`))
              (set `self.startLocation` (`self.currentLocation`))
              (else
                (`self.Death`)))))))
    (:`then_1`
      ;[1 1 1] Manage Activation
      (if (`self.doActivation`)
        (if (`self.isActive`)
          (`self.DoActivation_` (`self.counterActivation`) (`self.activationTime`))
          (else
            (`self.DoActivation_` (`self.counterDeactivation`) (`self.deactivationTime`) true "QueryAndPhysics")))))))

(fn `DoActivation_`
  (params (counter :type "Float (double-precision) (by ref)") (timeToActivation :type "Float (double-precision)") (isActive :type Boolean) (colision :type "ECollisionEnabled Enum" :default "NoCollision"))
  (`|VariableSetRef` (`local.counter`) (+ (`local.counter`) (`self.deltaTime`)))
  (if (>= (`local.counter`) (`local.timeToActivation`))
    (`self.ActivateTrap` (`local.isActive`) (`local.colision`))
    (`|VariableSetRef` (`local.counter`))
    (set `self.isActive` (`local.isActive`))))

(fn `Init`
  (params (speed :type "Float (double-precision)") (isMoving :type Boolean) (goBack :type Boolean) (scale :type "Vector Structure") (targetLocation :type "Vector Structure") (speedRotation :type "Float (double-precision)") (cyclicRotation :type "IntVector Structure") (doActivation :type Boolean) (activationTime :type "Float (double-precision)") (deactivationTime :type "Float (double-precision)"))
  (set `self.activationTime` (`local.activationTime`))
  (set `self.deactivationTime` (`local.deactivationTime`))
  (set `self.doActivation` (`local.doActivation`))
  (set `self.cyclicRotation` (`local.cyclicRotation`))
  (set `self.speedRotation` (`local.speedRotation`))
  (set `self.targetLocation` (`local.targetLocation`))
  (`self.SetActorScale3D` (`local.scale`))
  (set `self.goBack` (`local.goBack`))
  (set `self.isMoving` (`local.isMoving`))
  (set `self.speed` (`local.speed`))
  (set `self.currentLocation` (`self.K2_GetActorLocation`))
  (set `self.startLocation` (`self.currentLocation`))
  (set `self.currentRotation` (`self.K2_GetActorRotation`)))

(fn `SetRotation`
  (bind (_currentrotation_roll _currentrotation_pitch _currentrotation_yaw) (`KismetMathLibrary.BreakRotator` (`self.currentRotation`)))
  (bind (_returnvalue_x _returnvalue_y _returnvalue_z) (`KismetMathLibrary.BreakVector` (* (`KismetMathLibrary.Conv_IntVectorToVector` (`self.cyclicRotation`)) (* (`self.speedRotation`) (`self.deltaTime`)))))
  (set `self.currentRotation` (`KismetMathLibrary.MakeRotator` (+ _currentrotation_roll _returnvalue_x) (+ _currentrotation_pitch _returnvalue_y) (+ _currentrotation_yaw _returnvalue_z)))
  (`self.K2_SetActorRotation` (`self.currentRotation`)))

(fn `SetTargetLocation`
  (set `self.targetLocation` (+ (`self.currentLocation`) (* (`self.GetActorForwardVector`) (0.0 0.0 0.0)))))

(fn `UserConstructionScript`)