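; BP_GrapplePoint is a level element that the player's grapple ability can target.
; Overlapping BoxCanUseGrapple notifies BP_PlayerController when the player enters or leaves range.
; CollisionStopAbility stops the player's GrappleSystem ability on contact.
; BoxIndicator shows or hides the WG_GrappleLock widget, with helper functions to swap its lock texture and the mesh material.
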(event `self.ReceiveBeginPlay`
  (bind _aswg_grapple_lock (cast `/Game/UI/Grapple/WG_GrappleLock` (`WidgetComponent.GetUserWidgetObject` (`self.WG_Indicator`))))
  (set `self.WG_GrappleLock` _aswg_grapple_lock))

(event `self.BoxCanUseGrapple.OnComponentBeginOverlap`
  (params (OverlappedComponent :type "PrimitiveComponent Object Reference") (OtherActor :type "Actor Object Reference") (OtherComp :type "PrimitiveComponent Object Reference") (OtherBodyIndex :type Integer) (bFromSweep :type Boolean) (SweepResult :type "HitResult Structure (by ref)"))
  (cast `/Game/Blueprints/Characters/BP_PlayerCharacter` OtherActor)
  (bind _asbp_player_controller (cast `/Game/Blueprints/Controller/BP_PlayerController` (`GameplayStatics.GetPlayerController` 0)))
  (`/Game/Blueprints/Controller/BP_PlayerController.OverlapEvent` _asbp_player_controller self))

(event `self.BoxCanUseGrapple.OnComponentEndOverlap`
  (params (OverlappedComponent :type "PrimitiveComponent Object Reference") (OtherActor :type "Actor Object Reference") (OtherComp :type "PrimitiveComponent Object Reference") (OtherBodyIndex :type Integer))
  (cast `/Game/Blueprints/Characters/BP_PlayerCharacter` OtherActor)
  (bind _asbp_player_controller (cast `/Game/Blueprints/Controller/BP_PlayerController` (`GameplayStatics.GetPlayerController` 0)))
  (`/Game/Blueprints/Controller/BP_PlayerController.EndOverlapEvent` _asbp_player_controller self))

(event `self.CollisionStopAbility.OnComponentBeginOverlap`
  (params (OverlappedComponent :type "PrimitiveComponent Object Reference") (OtherActor :type "Actor Object Reference") (OtherComp :type "PrimitiveComponent Object Reference") (OtherBodyIndex :type Integer) (bFromSweep :type Boolean) (SweepResult :type "HitResult Structure (by ref)"))
  ;[1 1 1] CheckColision With GrapplePoint
  (bind _asbp_player_character (cast `/Game/Blueprints/Characters/BP_PlayerCharacter` OtherActor))
  (`/Game/Blueprints/Component/ActorComponent/Player/AC_Ability.StopAbility` (`/Game/Blueprints/Characters/BP_PlayerCharacter.GrappleSystem` _asbp_player_character)))

(event `self.BoxIndicator.OnComponentBeginOverlap`
  (params (OverlappedComponent :type "PrimitiveComponent Object Reference") (OtherActor :type "Actor Object Reference") (OtherComp :type "PrimitiveComponent Object Reference") (OtherBodyIndex :type Integer) (bFromSweep :type Boolean) (SweepResult :type "HitResult Structure (by ref)"))
  (`self.ChangeLockWidget` false))

(event `self.BoxIndicator.OnComponentEndOverlap`
  (params (OverlappedComponent :type "PrimitiveComponent Object Reference") (OtherActor :type "Actor Object Reference") (OtherComp :type "PrimitiveComponent Object Reference") (OtherBodyIndex :type Integer))
  (`SceneComponent.SetHiddenInGame` (`self.WG_Indicator`) true false))

(fn `ChangeLockWidget`
  (params (lock :type Boolean) (hiddenInGame :type Boolean))
  (`SceneComponent.SetHiddenInGame` (`self.WG_Indicator`) hiddenInGame false)
  (if lock
    (`self.SetTextureWIdgetIndicator` (`self.textureLock`))
    (else
      (`self.SetTextureWIdgetIndicator` (`self.textureClose`)))))

(fn `ChangeMaterial`
  (params (Material :type "MaterialInterface Object Reference"))
  (`PrimitiveComponent.SetMaterial` (`self.StaticMesh`) 0 Material))

(fn `SetTextureWIdgetIndicator`
  (params (Texture :type "Texture2D Object Reference"))
  (`Image.SetBrushFromTexture` (`/Game/UI/Grapple/WG_GrappleLock.ImageLock` (`self.WG_GrappleLock`)) Texture false))

(fn `UserConstructionScript`)