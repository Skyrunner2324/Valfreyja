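; Trigger volume that moves the player into a new map, by either a hard level open or async streaming.
; Open-level mode stops the main music first.
; Streaming mode places the map relative to the actor using a rotated player-start offset, registers it with GI_Global and disables the trigger.
; Once shown, it requests optional unload of the replaced map, or has SkyrunnerGameMode unload the oldest if none is valid.
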(event `self.trigger.OnComponentBeginOverlap`
  (params (OverlappedComponent :type "PrimitiveComponent Object Reference") (OtherActor :type "Actor Object Reference") (OtherComp :type "PrimitiveComponent Object Reference") (OtherBodyIndex :type Integer) (bFromSweep :type Boolean) (SweepResult :type "HitResult Structure (by ref)"))
  (bind _newmapplayerstartposition (`self.NewMapPlayerStartPosition`))
  (cast `/Game/Blueprints/Characters/BP_PlayerCharacter` OtherActor)
  (if (`KismetSystemLibrary.IsValidSoftObjectReference` (`self.NewMap`))
    ;[1 1 1] OpenLevel
    (if (`self.bUseOpenLevel`)
      (`AkGameplayStatics.PostEvent` "/Game/WwiseAudio/Events/Music/MUS_Stop_MainMusic.MUS_Stop_MainMusic")
      (`GameplayStatics.OpenLevelBySoftObjectPtr` (`self.NewMap`))
      (else
        (`|ExecutionSequence`
          (:`then_0`
            ;[1 1 1] Load level instance
            ;;[1 1 1] loading
            (bind _returnvalue (`MapLoader.LoadMapAsync` :`level` (`self.NewMap`) :`levelTransform` (`KismetMathLibrary.MakeTransform` (+ (`self.K2_GetActorLocation`) (`self.MapPosition`) (`KismetMathLibrary.GreaterGreater_VectorRotator` (select `bool` (`self.bNegatePlayerStartPosition`) :`false` _newmapplayerstartposition :`true` (`KismetMathLibrary.NegateVector` _newmapplayerstartposition)) (`self.NewMapPlayerStartOrientation`))) (`self.NewMapPlayerStartOrientation`)) :`OnLevelShown` (delegate `OnShown`) :`bResetUponCompletion` false))
            ;;[1 1 1] game instance
            (bind _asgi_global (cast `/Game/Blueprints/GameInstance/GI_Global` (`GameplayStatics.GetGameInstance`)))
            (bind _oldmap (`/Game/Blueprints/GameInstance/GI_Global.ChangeCurrentLoadedMap` _asgi_global _returnvalue))
            (set `self.MapToUnload` _oldmap))
          (:`then_1`
            (`PrimitiveComponent.SetCollisionEnabled` (`self.trigger`) "NoCollision")))))
    (else
      (`KismetSystemLibrary.PrintString` "Please, specify a new map to transition to"))))

(event `OnShown`
  ;[1 1 1] Load level instance
  (`/Engine/EditorBlueprintResources/StandardMacros.IsValid` (`self.MapToUnload`)
    (:`Is Valid`
      (`LevelStreaming.SetIsRequestingUnloadAndRemoval` (`self.MapToUnload`) (`self.bShouldUnloadReplacedMap`)))
    (:`Is Not Valid`
      (bind _asskyrunner_game_mode (cast `SkyrunnerGameMode` (`GameplayStatics.GetGameMode`)))
      ;;[1 0 0.6578] TODO
      (`SkyrunnerGameMode.UnloadOldestMap` _asskyrunner_game_mode))))

(fn `UserConstructionScript`
  (`BoxComponent.SetBoxExtent` (`self.trigger`) (`self.TriggerExtent`) true))