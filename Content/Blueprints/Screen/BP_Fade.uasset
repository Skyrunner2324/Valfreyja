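; BP_Fade is an actor that fades the screen in and out through a WB_Fade widget, optionally created at BeginPlay.
; One timeline drives the Screen brush's alpha, played forward by FadeIn and reversed by FadeOut, calling OnFading and OnFadeFinished.
; With a new widget, StartBlack sets initial content opacity and triggers FadeOut.
; The timeline copies the actor's tickable-when-paused setting, so fades can run during pause.
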(event `self.ReceiveBeginPlay`
  (bind _returnvalue (`self.GetTickableWhenPaused`))
  (`ActorComponent.SetTickableWhenPaused` (`self.FadeInTimeline`) _returnvalue)
  (if (`self.bInstanciateNewWidget`)
    (`|ExecutionSequence`
      (:`then_0`
        (bind _returnvalue_2 (`|CreateWidget` "/Game/UI/Screen/WB_Fade.WB_Fade_C"))
        (`UserWidget.AddToViewport` _returnvalue_2 1)
        (set `self.FadeWidget` _returnvalue_2))
      (:`then_1`
        (`Border.SetContentColorAndOpacity` (`/Game/UI/Screen/WB_Fade.Screen` (`self.FadeWidget`)) (make `LinearColor` 0.0 0.0 0.0 (select `bool` (`self.bStartBlack`) :`true` 1.0 :!type "Float (single-precision)")))
        (if (`self.bStartBlack`)
          (`self.FadeOut`))))))

(event `FadeIn`
  (bind (_direction _opacity) (`Timeline|FadeInTimeline` :!via `PlayFromStart` :!label _label)
    (:`Update`
      (`Border.SetBrushColor` (`/Game/UI/Screen/WB_Fade.Screen` (`self.FadeWidget`)) (make `LinearColor` 0.0 0.0 0.0 _opacity))
      (`self.OnFading` _opacity))
    (:`Finished`
      (`self.OnFadeFinished`))))

(event `FadeOut`
  (goto _label :!via `ReverseFromEnd`))

(fn `UserConstructionScript`)