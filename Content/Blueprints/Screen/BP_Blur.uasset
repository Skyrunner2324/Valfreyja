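; BP_Blur is an actor that fades a full-screen blur in and out.
; If InstanciateNewWidget is set, BeginPlay adds a WB_Blur widget to the viewport and, with StartBlack, starts at maximum blur and fades out.
; Fadein and FadeOut play one timeline forward or in reverse, scaling blur by MaxBlurStrength and broadcasting OnFading progress and OnFadeFinished.
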(event `self.ReceiveBeginPlay`
  (if (`self.bInstanciateNewWidget`)
    (`|ExecutionSequence`
      (:`then_0`
        (bind _returnvalue (`|CreateWidget` "/Game/UI/Screen/WB_Blur.WB_Blur_C"))
        (`UserWidget.AddToViewport` _returnvalue 1)
        (set `self.BlurWidget` _returnvalue))
      (:`then_1`
        (`self.SetBlurStrength` (select `bool` (`self.bStartBlack`) :`true` (`self.MaxBlurStrength`)))
        (if (`self.bStartBlack`)
          (`self.FadeOut`))))))

(event `self.FadeIn`
  (bind (_direction _blurvalue) (`Timeline|BlurInTimeline` :!via `PlayFromStart` :!label _label)
    (:`Update`
      (`self.SetBlurStrength` (* _blurvalue (`self.MaxBlurStrength`)))
      (`self.OnFading` _blurvalue))
    (:`Finished`
      (`self.OnFadeFinished`))))

(event `self.FadeOut`
  (goto _label :!via `ReverseFromEnd`))

(fn `SetBlurStrength`
  (params (InStrength :type "Float (single-precision)"))
  (`BackgroundBlur.SetBlurStrength` (`/Game/UI/Screen/WB_Blur.Screen` (`self.BlurWidget`)) InStrength))

(fn `UserConstructionScript`)