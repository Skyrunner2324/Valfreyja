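; BP_CreditsGP is a credits Blueprint that displays a localized title.
; It overrides SetLocalizedText, calling the parent implementation first, then looking up its second localization key for the given culture and applying the result to the Title text.
; All other behavior comes from the parent class, as BeginPlay, overlap and Tick are disabled stubs and construction only calls the parent.
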(event `self.SetLocalizedText`
  (params (culture :type "/Game/Enumerations/E_LocalizationCulture Enum" :default "NewEnumerator0"))
  (`parent.SetLocalizedText` culture)
  (bind _value (`/Game/Blueprints/Libraries/FunctionLibraries/BFL_Localization.GetLocalizedText` (`self.LocalizationKey2`) "NewEnumerator0" culture))
  (`TextRenderComponent.K2_SetText` (`self.Title`) _value))

(fn `UserConstructionScript`
  (`parent.UserConstructionScript`))