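; BP_Credits is a credits actor that shows a localized title through its Title component.
; On BeginPlay it sets the text for the current culture in GI_Global and binds to that game instance's culture change event, so the title follows language switches.
; SetLocalizedText looks up LocalizationKey in a fixed category for the given culture, and the binding is removed when the actor is destroyed.
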(event `self.ReceiveBeginPlay`
  (bind _asgi_global (cast `/Game/Blueprints/GameInstance/GI_Global` (`GameplayStatics.GetGameInstance`) :!pure true))
  (add `/Game/Blueprints/GameInstance/GI_Global.OnLocalizationCultureChange` _asgi_global (delegate `SetLocalizedText`))
  (`self.SetLocalizedText` (`/Game/Blueprints/GameInstance/GI_Global.currentCulture` _asgi_global)))

(event `self.ReceiveDestroyed`
  (remove `/Game/Blueprints/GameInstance/GI_Global.OnLocalizationCultureChange` (cast `/Game/Blueprints/GameInstance/GI_Global` (`GameplayStatics.GetGameInstance`) :!pure true) (delegate `SetLocalizedText`)))

(event `SetLocalizedText`
  (params (culture :type "/Game/Enumerations/E_LocalizationCulture Enum" :default "NewEnumerator0"))
  (bind _value (`/Game/Blueprints/Libraries/FunctionLibraries/BFL_Localization.GetLocalizedText` (`self.localizationKey`) "NewEnumerator0" culture))
  (`TextRenderComponent.K2_SetText` (`self.Title`) _value))

(fn `UserConstructionScript`)