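; Breakable wall Blueprint with a toggleable door-lock mesh and a triggered destruction.
; Destroy sets a flag, spawns an FS_OldField actor at DestructionPoint and fires its trigger, apparently a field system to fracture the wall.
; Lock shows or hides the lock mesh, while SetUnLockParameterShader switches emissive intensity on stored dynamic materials.
; Init and Reset are empty; the material setup and physics-enabling nodes are disconnected, so that material array is never filled here.
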(fn `CreateDynamicMaterial`
  (params (mesh :type "PrimitiveComponent Object Reference"))
  (bind _returnvalue (`KismetMaterialLibrary.CreateDynamicMaterialInstance` (`PrimitiveComponent.GetMaterial` mesh 0)))
  (`KismetArrayLibrary.Array_Add` (`self.materialDynamic`) _returnvalue)
  (`PrimitiveComponent.SetMaterial` (`local.mesh`) 0 _returnvalue))

(fn `Destroy_`
  (set `self.destroy` true)
  (bind _returnvalue (`|SpawnActorFromClass` "/Game/Blueprints/LDElement/Door/FS_OldField.FS_OldField_C" (`KismetMathLibrary.MakeTransform` (`SceneComponent.K2_GetComponentLocation` (`self.DestructionPoint`))) "Undefined" "MultiplyWithRoot" null null))
  (`/Engine/EditorResources/FieldNodes/FS_MasterField.CE_Trigger` _returnvalue))

(fn `Init`)

(fn `Lock`
  (params (lock :type Boolean))
  (`SceneComponent.SetVisibility` (`self.SM_Door_Lock`) (`local.lock`) false)
  (`SceneComponent.SetHiddenInGame` (`self.SM_Door_Lock`) (not (`local.lock`)) false))

(fn `Reset`)

(fn `SetUnLockParameterShader`
  (params (value :type Boolean))
  (for _array_element (`self.materialDynamic`)
    (`MaterialInstanceDynamic.SetScalarParameterValue` _array_element "E_Intentisty" (`KismetMathLibrary.SelectFloat` (`self.intensityEmissive`) 0.0 value))))

(fn `UserConstructionScript`)