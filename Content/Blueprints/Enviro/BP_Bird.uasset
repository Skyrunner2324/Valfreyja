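; BP_Bird is an environment actor that scatters a flock of bird meshes around its origin as instances of the Birds component.
; The construction script assigns the mesh and material, then adds instances according to Amount.
; Each instance takes a random direction from one of three cycling cones, with distance growing by Spread every three birds and randomized per-axis scale.
; The event graph holds no active logic.
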(fn `UserConstructionScript`
  (locals (ThisDirection :type "Vector Structure"))
  (bind _returnvalue (`KismetMathLibrary.RandomFloatInRange` 0.75 1.25))
  (bind _amount (`self.Amount`))
  (`/Engine/EditorBlueprintResources/StandardMacros.IsValid` null
    (:`Is Valid`
      (`StaticMeshComponent.SetStaticMesh` (`self.Birds`) null)
      (`/Engine/EditorBlueprintResources/StandardMacros.IsValid` (`self.Mesh`)
        (:`Is Valid`
          (`PrimitiveComponent.SetMaterial` (`self.Birds`) 0 (`self.Material`))
          (if (> _amount 0)
            (for _index (range (+ _amount 1))
              (`|ExecutionSequence`
                (:`then_0`
                  (switch `int` (mod _index 3)
                    (:`0`
                      (set `local.ThisDirection` (`KismetMathLibrary.RandomUnitVectorInConeInDegrees` (1.0 0.0 0.0) 120.0)))
                    (:`1`
                      (set `local.ThisDirection` (`KismetMathLibrary.RandomUnitVectorInConeInDegrees` (`KismetMathLibrary.GreaterGreater_VectorRotator` (1.0 0.0 0.0) (`KismetMathLibrary.MakeRotator` 0.0 0.0 120.0)) 120.0)))
                    (:`2`
                      (set `local.ThisDirection` (`KismetMathLibrary.RandomUnitVectorInConeInDegrees` (`KismetMathLibrary.GreaterGreater_VectorRotator` (0.0 0.0 0.0) (`KismetMathLibrary.MakeRotator` 0.0 0.0 240.0)) 120.0)))))
                (:`then_1`
                  (`InstancedStaticMeshComponent.AddInstance` (`self.Birds`) (`KismetMathLibrary.MakeTransform` (* (`local.ThisDirection`) (`KismetMathLibrary.Conv_IntToDouble` (* (+ (/ _index 3) 1) (`self.Spread`)))) (struct) (`KismetMathLibrary.MakeVector` _returnvalue _returnvalue _returnvalue)) false))))))))))