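; Tutorial (FTUE) trigger box that freezes the player on overlap and shows a text prompt until the taught action is done.
; Its Type selects Grapple, Dash or Door, binding completion to that player ability's trigger or the FTUE door's OnOpen.
; Tick holds the player by zeroing movement velocity.
; Completion unfreezes, hides the text, restores in-game status and blocks retriggering; Grapple also toggles Dash's UseAbility flag around the lesson.
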(event `self.ReceiveBeginPlay`
  (`SceneComponent.SetHiddenInGame` (`self.TextToDisplay`) true false))

(event `GrappleFTUEComplete`
  ;[1 1 1] Bind grapple FTUE
  (if (not (`self.Completed`))
    (set `self.PlayerFrozen` false)
    (set `self.Completed` true)
    (`AkGameplayStatics.SetState` "/Game/WwiseAudio/States/Default_Work_Unit/GameStatus/GameStatus-InGame.GameStatus-InGame")
    (set `/Game/Blueprints/Component/ActorComponent/Player/AC_Ability.useAbility` false (`/Game/Blueprints/Characters/BP_PlayerCharacter.Dash` (`self.PlayerRef`)))
    ;[1 1 1] Hide FTUE text when completed
    (`SceneComponent.SetHiddenInGame` (`self.TextToDisplay`) true false :!label _label)
    (set `/Game/Blueprints/Characters/BP_PlayerCharacter.InFTUE` false (`self.PlayerRef`))))

(event `self.ReceiveActorBeginOverlap`
  (params (OtherActor :type "Actor Object Reference"))
  (bind _playerref (`self.PlayerRef`))
  (bind _playerref_2 (`self.PlayerRef`))
  (if (not (`self.Completed`))
    (bind _asbp_player_character (cast `/Game/Blueprints/Characters/BP_PlayerCharacter` OtherActor))
    (`/Engine/EditorBlueprintResources/StandardMacros.IsValid` (`self.PlayerRef`)
      (:`Is Not Valid`
        (set `self.PlayerRef` _asbp_player_character)
        (switch `/Game/Blueprints/Enumerator/E_FTUEType` (`self.Type`)
          (:`NewEnumerator0`
            ;[1 1 1] Bind grapple FTUE
            (set `/Game/Blueprints/Component/ActorComponent/Player/AC_Ability.useAbility` true (`/Game/Blueprints/Characters/BP_PlayerCharacter.Dash` _playerref))
            (add `/Game/Blueprints/Component/ActorComponent/Player/AC_Ability.TriggerAbility_` (`/Game/Blueprints/Characters/BP_PlayerCharacter.GrappleSystem` _playerref) (delegate `GrappleFTUEComplete`))
            (`AkGameplayStatics.SetState` "/Game/WwiseAudio/States/Default_Work_Unit/GameStatus/GameStatus-InFTUE.GameStatus-InFTUE")
            (`self.SetInFTUE`))
          (:`NewEnumerator1`
            ;[1 1 1] Bind dash FTUE
            (bind _out (`/Game/Blueprints/Component/ActorComponent/Player/AC_Dash.DashUsed` (`/Game/Blueprints/Characters/BP_PlayerCharacter.Dash` _playerref_2)))
            (if _out
              (add `/Game/Blueprints/Component/ActorComponent/Player/AC_Ability.TriggerAbility_` (`/Game/Blueprints/Characters/BP_PlayerCharacter.Dash` _playerref_2) (delegate `DashFTUEComplete`))
              (`AkGameplayStatics.SetState` "/Game/WwiseAudio/States/Default_Work_Unit/GameStatus/GameStatus-InFTUE.GameStatus-InFTUE")
              (`self.SetInFTUE`)))
          (:`NewEnumerator2`
            ;[1 1 1] FTUE door
            (bind _returnvalue (`GameplayStatics.GetActorOfClass` "/Game/Blueprints/FTUE/BP_Door_FTUE.BP_Door_FTUE_C"))
            (`/Engine/EditorBlueprintResources/StandardMacros.IsValid` _returnvalue
              (:`Is Valid`
                (add `/Game/Blueprints/FTUE/BP_Door_FTUE.OnOpen_` _returnvalue (delegate `DoorFTUEComplete`))
                (`AkGameplayStatics.SetState` "/Game/WwiseAudio/States/Default_Work_Unit/GameStatus/GameStatus-InFTUE.GameStatus-InFTUE")
                (`self.SetInFTUE`)))))))))

(event `self.ReceiveTick`
  (params (DeltaSeconds :type "Float (single-precision)"))
  (if (`self.PlayerFrozen`)
    (set `MovementComponent.Velocity` (0.0 0.0 0.0) (`Character.CharacterMovement` (`self.PlayerRef`)))))

(event `DashFTUEComplete`
  ;[1 1 1] Bind dash FTUE
  (if (not (`self.Completed`))
    (set `self.PlayerFrozen` false)
    (set `self.Completed` true)
    (`AkGameplayStatics.SetState` "/Game/WwiseAudio/States/Default_Work_Unit/GameStatus/GameStatus-InGame.GameStatus-InGame")
    (goto _label)))

(event `DoorFTUEComplete`
  ;[1 1 1] FTUE door
  (if (not (`self.Completed`))
    (set `self.PlayerFrozen` false)
    (set `self.Completed` true)
    (`AkGameplayStatics.SetState` "/Game/WwiseAudio/States/Default_Work_Unit/GameStatus/GameStatus-InGame.GameStatus-InGame")
    (goto _label)))

(fn `SetInFTUE`
  (`SceneComponent.SetHiddenInGame` (`self.TextToDisplay`) false false)
  (set `self.PlayerFrozen` true)
  (set `/Game/Blueprints/Characters/BP_PlayerCharacter.InFTUE` true (`self.PlayerRef`)))

(fn `UserConstructionScript`)