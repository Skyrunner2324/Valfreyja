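; One-shot FTUE trigger that shows a tutorial pop-up on the HUD when the player character overlaps its box while it is not hidden.
; It sets the pop-up text from its LocalizationKey in the game instance's current culture.
; The pop-up icon comes from looking up the key mapped to its InputAction in the game instance's controller key table.
; It then plays the HUD pop-up animation and destroys itself.
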(event `self.Box.OnComponentBeginOverlap`
  (params (OverlappedComponent :type "PrimitiveComponent Object Reference") (OtherActor :type "Actor Object Reference") (OtherComp :type "PrimitiveComponent Object Reference") (OtherBodyIndex :type Integer) (bFromSweep :type Boolean) (SweepResult :type "HitResult Structure (by ref)"))
  (if (not (`self.bHidden`))
    (bind _asbp_player_character (cast `/Game/Blueprints/Characters/BP_PlayerCharacter` OtherActor))
    (`|ExecutionSequence`
      (:`then_0`
        (bind _tx_tutorial (`/Game/UI/HUD/WB_FTUEPopUp.TX_Tutorial` (`/Game/UI/HUD/WB_HUD.WB_FTUEPopUp` (`/Game/Blueprints/HUD/BP_PlayerHUD.hudWidget` (`/Game/Blueprints/Characters/BP_PlayerCharacter.HUD` _asbp_player_character)))))
        ;[1 1 1] change text
        (set `/Game/UI/WB_LocalizedText.localizationKey` (`self.Localization Key`) _tx_tutorial)
        (bind _asgi_global (cast `/Game/Blueprints/GameInstance/GI_Global` (`GameplayStatics.GetGameInstance`)))
        (`/Game/UI/WB_LocalizedText.SetLocalizedText` _tx_tutorial (`/Game/Blueprints/GameInstance/GI_Global.currentCulture` _asgi_global)))
      (:`then_1`
        (bind _asbp_player_controller (cast `/Game/Blueprints/Controller/BP_PlayerController` (`GameplayStatics.GetPlayerController` 0)))
        (bind _mappedkey (`/Game/Blueprints/Controller/BP_PlayerController.GetMappedKey` _asbp_player_controller (`self.InputAction`)))
        (`KismetSystemLibrary.PrintString` (`KismetTextLibrary.Conv_TextToString` _mappedkey) true true (struct :`G` 1.0 :`A` 1.0) 0.0)
        (bind _hudwidget (`/Game/Blueprints/HUD/BP_PlayerHUD.hudWidget` (`/Game/Blueprints/Characters/BP_PlayerCharacter.HUD` _asbp_player_character)))
        (`Image.SetBrushFromTexture` (`/Game/UI/HUD/WB_FTUEPopUp.InputImage` (`/Game/UI/HUD/WB_HUD.WB_FTUEPopUp` _hudwidget)) (`BlueprintMapLibrary.Map_Find` (`/Game/Blueprints/GameInstance/GI_Global.GetControllerKeyTable` (cast `/Game/Blueprints/GameInstance/GI_Global` (`GameplayStatics.GetGameInstance`) :!pure true)) (`KismetTextLibrary.Conv_TextToString` _mappedkey)) false))
      (:`then_2`
        (`UserWidget.PlayAnimation` _hudwidget (`/Game/UI/HUD/WB_HUD.ANIM_PopUp` _hudwidget) 0.0 1 "Forward" 1.0 false)
        (`self.K2_DestroyActor`)))))

(fn `UserConstructionScript`)