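; BP_MobilePlatform is a moving platform that slides its Cube component either vertically or horizontally once play begins.
; On BeginPlay, the IsVertical flag picks one of two timelines: Move drives the Cube's relative Z, and Timeline drives its relative X.
; Each update sets that axis to the track value scaled by MovementValue, keeping the other two axes at their current values.
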(event `self.ReceiveBeginPlay`
  (bind _cube (`self.Cube`))
  (bind _movementvalue (`self.MovementValue`))
  (bind (_relativelocation_x _relativelocation_y _relativelocation_z) (`KismetMathLibrary.BreakVector` (`SceneComponent.RelativeLocation` _cube)))
  (bind (_relativelocation_x_2 _relativelocation_y_2) (`KismetMathLibrary.BreakVector` (`SceneComponent.RelativeLocation` _cube)))
  (if (`self.IsVertical`)
    (bind (_direction _newtrack_0) (`Timeline|Move` :!via `PlayFromStart`)
      (:`Update`
        (`SceneComponent.K2_SetRelativeLocation` _cube (`KismetMathLibrary.MakeVector` _relativelocation_x_2 _relativelocation_y_2 (* _newtrack_0 _movementvalue)) false false)))
    (else
      (bind (_direction_2 _newtrack_0_2) (`Timeline|Timeline` :!via `PlayFromStart`)
        (:`Update`
          (`SceneComponent.K2_SetRelativeLocation` _cube (`KismetMathLibrary.MakeVector` (* _newtrack_0_2 _movementvalue) _relativelocation_y _relativelocation_z) false false))))))

(fn `UserConstructionScript`)