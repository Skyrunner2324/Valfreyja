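; Laser launcher actor for the LD_3C folder that repeatedly sends its Cube component along a local axis.
; After an initial delay, one of two timelines scales its curve by Distance to drive relative Z when vertical, otherwise X.
; Speed sets both timelines' length rather than a velocity.
; On finish, the actor hides by scaling to zero, waits, restores unit scale and restarts the move.
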(event `self.ReceiveBeginPlay`
  (bind _cube (`self.Cube`))
  (bind _distance (`self.Distance`))
  (bind (_relativelocation_x _relativelocation_y _relativelocation_z) (`KismetMathLibrary.BreakVector` (`SceneComponent.RelativeLocation` _cube)))
  (bind (_relativelocation_x_2 _relativelocation_y_2) (`KismetMathLibrary.BreakVector` (`SceneComponent.RelativeLocation` _cube)))
  (`KismetSystemLibrary.Delay` (`self.DelayInitial`))
  (`TimelineComponent.SetTimelineLength` (`self.Timeline`) (`self.Speed`))
  (`TimelineComponent.SetTimelineLength` (`self.Move`) (`self.Speed`))
  (if (`self.IsVertical`) :!label _label
    (bind (_direction _newtrack_0) (`Timeline|Move` :!via `PlayFromStart`)
      (:`Update`
        (`SceneComponent.K2_SetRelativeLocation` _cube (`KismetMathLibrary.MakeVector` _relativelocation_x_2 _relativelocation_y_2 (* _newtrack_0 _distance)) false false))
      (:`Finished`
        (`self.SetActorScale3D` (0.0 0.0 0.0) :!label _label_2)
        (`KismetSystemLibrary.Delay` (`self.Delay`))
        (`self.SetActorScale3D` (1.0 1.0 1.0))
        (goto _label)))
    (else
      (bind (_direction_2 _newtrack_0_2) (`Timeline|Timeline` :!via `PlayFromStart`)
        (:`Update`
          (`SceneComponent.K2_SetRelativeLocation` _cube (`KismetMathLibrary.MakeVector` (* _newtrack_0_2 _distance) _relativelocation_y _relativelocation_z) false false))
        (:`Finished`
          (goto _label_2))))))

(fn `UserConstructionScript`)